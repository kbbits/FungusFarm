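; ModSlot is a placement target that holds one piece of modifier equipment, optionally restricted to accepted classes and their children, and exposes that equipment's attribute modifiers.
; Placing equipment attaches it at ModSpot, records its ID on the parent ModSlot_CAC_BP component and fires a placed event; removal reverses this.
; RemoveModEquipment hands the slotted item to the player controller for pickup.
; The construction script applies the slot image through a dynamic material.
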(event OnClicked(SlotImagePlane)
  (params (TouchedComponent :type Primitive%20Component%20Object%20Reference) (ButtonPressed :type Key%20Structure)))

(event Custom|RemoveModEquipment
  (Utilities|IsValid (Variables|Default|GetMyModEquipment)
    (:Is%20Valid
      (bind _asff_player_controller (Utilities|Casting|CastToFF_PlayerController (Game|GetPlayerController 0)))
      (Default|PickupEquipment _asff_player_controller (Variables|Default|GetMyModEquipment) false))))

(event EventOnEquipmentPlaced
  (params (Placed%20Equipment :type I%20Placeable%20Equipment%20Interface))
  (bind _asmod_equipment_base (Utilities|Casting|CastToModEquipment_Base Placed%20Equipment))
  (bind _output_get (Variables|Default|SetMyModEquipment _asmod_equipment_base))
  (bind _asmod_slot_cac_bp (Utilities|Casting|CastToModSlot_CAC_BP (Transformation|GetAttachParent (Variables|Default|GetScene))))
  (Variables|/Script/FungusFarm.ModSlot_CAC|SetSlottedEquipmentID _asmod_slot_cac_bp (Variables|/Game/FungusFarm/Blueprints/Equipment/Equipment_Base.Equipment_Base_C|GetMyID _output_get))
  (Variables|/Game/FungusFarm/Blueprints/Equipment/PlaceableEquipment_Base.PlaceableEquipment_Base_C|SetCurrentPlaceableTarget (Variables|Default|GetMyModEquipment) self)
  (Transformation|AttachActorToActor _output_get self "None" "SnapToTarget" "KeepRelative" "KeepRelative" true)
  (Transformation|SetRelativeLocation (Variables|/Script/Engine.Actor|GetRootComponent _output_get) (.Location (Math|Transform|BreakTransform (Transformation|GetRelativeTransform (Variables|Default|GetModSpot)))) false true)
  (Default|CallOnModifierEquipmentPlaced self (Variables|Default|GetMyModEquipment)))

(event EventOnEquipmentRemoved
  (params (Removed%20Equipment :type I%20Placeable%20Equipment%20Interface))
  (bind _asmod_equipment_base (Utilities|Casting|CastToModEquipment_Base Removed%20Equipment))
  (if (== _asmod_equipment_base (Variables|Default|GetMyModEquipment))
    (Transformation|DetachFromActor _asmod_equipment_base "KeepWorld" "KeepWorld" "KeepWorld")
    (Variables|Default|SetMyModEquipment 0)
    (bind _asmod_slot_cac_bp (Utilities|Casting|CastToModSlot_CAC_BP (Transformation|GetAttachParent (Variables|Default|GetScene))))
    (Guid|InvalidateGuid (Variables|/Script/FungusFarm.ModSlot_CAC|GetSlottedEquipmentID _asmod_slot_cac_bp))
    (Default|CallOnModifierEquipmentRemoved self)))

(fn ConstructionScript
  (bind _returnvalue (Rendering|Material|CreateDynamicMaterialInstance (Variables|Default|GetSlotImagePlane) 0 (Rendering|Material|GetMaterial (Variables|Default|GetSlotImagePlane) 0) "None" :!class /Script/Engine.PrimitiveComponent))
  (bind _output_get (Variables|Default|SetSlotMaterial _returnvalue))
  (Rendering|Material|SetTextureParameterValue _output_get "MaterialTexture" (Variables|Default|GetSlotImage))
  (Rendering|Material|SetMaterial (Variables|Default|GetSlotImagePlane) 0 (Variables|Default|GetSlotMaterial)))

(fn GetAllModifiers
  (Utilities|IsValid (Variables|Default|GetMyModEquipment)
    (:Is%20Valid
      (for _array_element (.Modifiers (Utilities|Struct|BreakNamedModifierSet (Default|GetModifierData (Variables|Default|GetMyModEquipment))))
        (Utilities|Array|Add (LocalVariables|GettmpAttributeModifiers) _array_element)))
    (:Is%20Not%20Valid
      _))
  (return (LocalVariables|GettmpAttributeModifiers)))

(fn CanAcceptEquipment?
  (params (Equipment :type Equipment%20Base%20Object%20Reference))
  (bind _asmod_equipment_base (Utilities|Casting|CastToModEquipment_Base Equipment)
    (:then
      (if (> (Utilities|Array|Length (Variables|Default|GetAcceptsClasses)) 0)
        (bind _array_element (Utilities|Array|ForEachLoopwithBreak (Variables|Default|GetAcceptsClasses) :!label _label)
          (:LoopBody
            (if (Utilities|ClassIsChildOf (Utilities|GetClass _asmod_equipment_base) _array_element)
              (LocalVariables|SettmpCanAccept true)
              (goto _label Break)))
          (:Completed
            (return (LocalVariables|GettmpCanAccept))))
        (else
          (return true))))
    (:CastFailed
      (return false))))