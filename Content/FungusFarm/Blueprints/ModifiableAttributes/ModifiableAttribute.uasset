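; ModifiableAttribute represents a single attribute, identified by a code, whose base value is altered by a list of added modifiers.
; UpdateCalculatedValue scans each modifier's entries for a matching AttributeCode, summing Scalar and Multiplier values separately.
; Multipliers stack additively, scaling the base by one plus their total before scalars are added.
; GetValue returns the cached result; adding or clearing modifiers does not recalculate it.
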(fn AddModifier
  (params (Modifier :type Modifier%20Effect%20Info%20Struct%20Structure))
  (Utilities|Array|Add (Variables|Default|GetModifiers) Modifier))

(fn ClearModifiers
  (Utilities|Array|Clear (Variables|Default|GetModifiers)))

(fn GetValue
  (return (Variables|Default|GetModifiedValue)))

(fn UpdateCalculatedValue
  (for _array_element (Variables|Default|GetModifiers)
    (for _array_element_2 (.Modifier (Utilities|Struct|BreakModifierEffectInfo_Struct _array_element))
      (if (Utilities|Enum|Equal(Enum) (Variables|Default|GetAttribute%20Code) (.AttributeCode (Utilities|Struct|BreakAttributeModifierInfo_Struct _array_element_2)))
        (switch Utilities|FlowControl|Switch|SwitchonModifier_Types (.Type (Utilities|Struct|BreakModifier_Struct (.Modifier (Utilities|Struct|BreakAttributeModifierInfo_Struct _array_element_2))))
          (:NewEnumerator0
            (LocalVariables|SettmpScalarTotal (+ (.Value (Utilities|Struct|BreakModifier_Struct (.Modifier (Utilities|Struct|BreakAttributeModifierInfo_Struct _array_element_2)))) (LocalVariables|GettmpScalarTotal))))
          (:NewEnumerator1
            (LocalVariables|SettmpMultiplierTotal (+ (.Value (Utilities|Struct|BreakModifier_Struct (.Modifier (Utilities|Struct|BreakAttributeModifierInfo_Struct _array_element_2)))) (LocalVariables|GettmpMultiplierTotal))))))))
  (Variables|Default|SetModifiedValue (+ (* (Variables|Default|GetBaseValue) (+ (LocalVariables|GettmpMultiplierTotal) 1.0)) (LocalVariables|GettmpScalarTotal))))