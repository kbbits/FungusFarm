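; RecipeMapDev_BP is a development Blueprint in FungusFarm that sketches a recipe map for resource goods, with no working logic yet.
; The construction script and RecipeMap graph are empty apart from unconnected G1 nodes.
; G and ResourceGoods are empty stub graphs, while Recipe_2_1 merges two inputs, G1 and G2, into one path without processing them.
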(fn ConstructionScript)

(fn RecipeMap)