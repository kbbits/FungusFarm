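; Minion actor that ferries a configured good from a source lab equipment to the equipment modified by its parent mod.
; Tick starts trips when the parent's stock is below target, sliding the minion in the XZ plane until within either equipment's bounds.
; Reusable looping timers transfer goods in batches, pausing and flipping travel state when done.
; A thumbnail and quantity display the cargo, and clicking the sprite opens the mod's config menu.
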(event OnClicked(MinionSprite)
  (params (TouchedComponent :type Primitive%20Component%20Object%20Reference) (ButtonPressed :type Key%20Structure :default "None"))
  (bind _myparentmod (Variables|Default|GetMyParentMod))
  (Utilities|IsValid _myparentmod
    (:Is%20Valid
      (Default|ShowMinionConfigMenu _myparentmod))))

(event EventBeginPlay
  (Variables|Default|SetbTransferring false)
  (Utilities|FlowControl|Delay 0.5)
  (Utilities|Casting|CastToFF_GameState (Game|GetGameState))
  (CallFunction|UpdateGoodsThumb)
  (Variables|Default|SetbReturningToHome (not (Default|IsEmpty? (Variables|Default|GetGoodsInventory)))))

(event EventTick
  (params (DeltaSeconds :type Float%20%28single-precision%29))
  (bind _returnvalue (Transformation|GetActorLocation))
  (bind _myparentmod (Variables|Default|GetMyParentMod))
  (bind _pullfromequipment (Variables|Default|GetPullFromEquipment))
  (bind (_origin _boxextent) (Collision|GetActorBounds _pullfromequipment false false))
  (bind _pulluntilquantity (Variables|/Game/FungusFarm/Blueprints/Equipment/EquipmentMods/LabEquipmentMod_GoodsMoverMinion.LabEquipmentMod_GoodsMoverMinion_C|GetPullUntilQuantity _myparentmod))
  (bind _returnvalue_2 (- _origin _returnvalue))
  (bind _returnvalue_3 (* _returnvalue_2 "1.000000, 0,1.000000"))
  (Utilities|IsValid (Variables|Default|GetMyParentMod)
    (:Is%20Valid
      (if (not (Variables|Default|GetbTransferring))
        (if (Variables|Default|GetbTravelIsActive)
          (if (Variables|Default|GetbReturningToHome)
            (bind _aslab_equipment_base_bp (Utilities|Casting|CastToLabEquipmentBase_BP (Default|GetModifiedParent (Variables|Default|GetMyParentMod))))
            (if (<= (Math|Vector|VectorLength (* (- (.Origin (Collision|GetActorBounds _aslab_equipment_base_bp false false)) (Transformation|GetActorLocation)) "1.000000, 0,1.000000")) (.X (Math|Vector|BreakVector (.BoxExtent (Collision|GetActorBounds _aslab_equipment_base_bp false false)))))
              (Variables|Default|SetbTransferring true)
              (if (Class|KismetSystemLibrary|IsTimerPausedHandle (Variables|Default|GetDropToParentTimer))
                (Utilities|Time|UnpauseTimerbyHandle (Variables|Default|GetDropToParentTimer))
                (elif (not (Class|KismetSystemLibrary|TimerExistsHandle (Variables|Default|GetDropToParentTimer)))
                  (bind _returnvalue_4 (Utilities|Time|SetTimerbyFunctionName self "TryDropGoodsToParent" 1.0 true))
                  (Variables|Default|SetDropToParentTimer _returnvalue_4)))
              (else
                (Transformation|AddActorWorldOffset (* (Math|Vector|Normalize (* (- (.Origin (Collision|GetActorBounds _aslab_equipment_base_bp false false)) (Transformation|GetActorLocation)) "1.000000, 0,1.000000")) (* DeltaSeconds (Variables|Default|GetMaxSpeed))) false true)))
            (else
              (Utilities|IsValid (Variables|Default|GetPullFromEquipment)
                (:Is%20Valid
                  (if (<= (Math|Vector|VectorLength _returnvalue_3) (.X (Math|Vector|BreakVector _boxextent)))
                    (Variables|Default|SetbTransferring true)
                    (if (Class|KismetSystemLibrary|IsTimerPausedHandle (Variables|Default|GetPickupFromTargetTimer))
                      (Utilities|Time|UnpauseTimerbyHandle (Variables|Default|GetPickupFromTargetTimer))
                      (elif (not (Class|KismetSystemLibrary|TimerExistsHandle (Variables|Default|GetPickupFromTargetTimer)))
                        (bind _returnvalue_5 (Utilities|Time|SetTimerbyFunctionName self "TryPickupGoodsFromTarget" 1.0 true))
                        (Variables|Default|SetPickupFromTargetTimer _returnvalue_5)))
                    (else
                      (Transformation|AddActorWorldOffset (* (Math|Vector|Normalize _returnvalue_3) (* DeltaSeconds (Variables|Default|GetMaxSpeed))) false true)))))))
          (else
            (Utilities|IsValid (Variables|Default|GetPullFromEquipment)
              (:Is%20Valid
                (bind _aslab_equipment_base_bp_2 (Utilities|Casting|CastToLabEquipmentBase_BP (Default|GetModifiedParent (Variables|Default|GetMyParentMod))))
                (if (and (< (Default|GetGoodsInventoryQuantity (Variables|/Game/FungusFarm/Blueprints/Equipment/LabEquipment/LabEquipmentBase_BP.LabEquipmentBase_BP_C|GetFF_GoodsInventory_Component _aslab_equipment_base_bp_2) (Variables|/Game/FungusFarm/Blueprints/Equipment/EquipmentMods/LabEquipmentMod_GoodsMoverMinion.LabEquipmentMod_GoodsMoverMinion_C|GetPullGoodsName (Variables|Default|GetMyParentMod))) _pulluntilquantity) (> _pulluntilquantity 0.0))
                  (Variables|Default|SetbTravelIsActive true))))))))))

(event EventDestroyed
  (Utilities|Time|ClearandInvalidateTimerbyHandle (Variables|Default|GetDropToParentTimer))
  (Utilities|Time|ClearandInvalidateTimerbyHandle (Variables|Default|GetPickupFromTargetTimer)))

(fn ConstructionScript
  (CallFunction|UpdateGoodsThumb))

(fn UpdateGoodsThumb
  (bind _goodsinventory (Variables|Default|GetGoodsInventory))
  (bind _myparentmod (Variables|Default|GetMyParentMod))
  (bind _goodsinventory_2 (Variables|/Game/FungusFarm/Blueprints/Inventory/FF_GoodsInventory_Component.FF_GoodsInventory_Component_C|GetGoodsInventory _goodsinventory))
  (if (not (Default|IsEmpty? (Variables|Default|GetGoodsInventory)))
    (Variables|Default|SetGoodsQuantity (Utilities|Struct|MakeGoodsQuantity "None" 0.0))
    (bind _keys (Utilities|Map|Keys _goodsinventory_2))
    (bind _array_element (Utilities|Array|ForEachLoopwithBreak _keys :!label _label)
      (:LoopBody
        (if (> (.Value (Utilities|Map|Find _goodsinventory_2 _array_element)) 0.0)
          (Variables|Default|SetGoodsQuantity (Utilities|Struct|MakeGoodsQuantity _array_element (.Value (Utilities|Map|Find _goodsinventory_2 _array_element))))
          (goto _label Break)))
      (:Completed
        (if (Utilities|Name|NotEqual(Name) (.Name (Utilities|Struct|BreakGoodsQuantity (Variables|Default|GetGoodsQuantity))) "None") :!label _label_2
          (Rendering|SetVisibility (Variables|Default|GetGoodsPlane) true true)
          (Rendering|SetVisibility (Variables|Default|GetGoodQuantity) true true)
          (Utilities|FlowControl|Sequence
            (:then_0
              (bind _asff_game_state (Utilities|Casting|CastToFF_GameState (Game|GetGameState)))
              (LocalVariables|SettmpGoodsData (.GoodsData (Default|GetGoodsData _asff_game_state (.Name (Utilities|Struct|BreakGoodsQuantity (Variables|Default|GetGoodsQuantity))))))
              (Rendering|Components|TextRender|SetText (Variables|Default|GetGoodQuantity) (Utilities|Text|ToText(Float) (.Quantity (Utilities|Struct|BreakGoodsQuantity (Variables|Default|GetGoodsQuantity))) "HalfToEven" false true 1 324 0 0)))
            (:then_1
              (Utilities|IsValid (Variables|Default|GetGoodsMaterial)
                (:Is%20Valid
                  _)
                (:Is%20Not%20Valid
                  (bind _returnvalue (Rendering|Material|CreateDynamicMaterialInstance (Variables|Default|GetGoodsPlane) 0 (Rendering|Material|GetMaterial (Variables|Default|GetGoodsPlane) 0) "None" :!class /Script/Engine.PrimitiveComponent))
                  (Variables|Default|SetGoodsMaterial _returnvalue)))
              (Rendering|Material|SetTextureParameterValue (Variables|Default|GetGoodsMaterial) "MaterialTexture" (Utilities|ResolveSoftReference (.Thumbnail (Utilities|Struct|BreakGoodsType (LocalVariables|GettmpGoodsData)))))
              (Rendering|Material|SetMaterial (Variables|Default|GetGoodsPlane) 0 (Variables|Default|GetGoodsMaterial))))
          (else
            (Rendering|SetVisibility (Variables|Default|GetGoodsPlane) false true)
            (Rendering|SetVisibility (Variables|Default|GetGoodQuantity) false true)))))
    (else
      (Utilities|IsValid _myparentmod
        (:Is%20Valid
          (Variables|Default|SetGoodsQuantity (Utilities|Struct|MakeGoodsQuantity (Variables|/Game/FungusFarm/Blueprints/Equipment/EquipmentMods/LabEquipmentMod_GoodsMoverMinion.LabEquipmentMod_GoodsMoverMinion_C|GetPullGoodsName _myparentmod) 0.0))
          (goto _label_2))
        (:Is%20Not%20Valid
          (goto _label_2))))))

(fn DropGoodstoParentMod
  (if (Default|IsEmpty? (Variables|Default|GetGoodsInventory))
    (return true)
    (else
      (Utilities|IsValid (Variables|Default|GetMyParentMod)
        (:Is%20Valid
          (bind _inventorymap (Default|GetAllInventoryasMap (Variables|Default|GetGoodsInventory)))
          (bind _output_get (LocalVariables|SettmpInventoryMap _inventorymap))
          (bind _keys (Utilities|Map|Keys _output_get))
          (bind _array_element (Utilities|Array|ForEachLoopwithBreak _keys :!label _label)
            (:LoopBody
              (LocalVariables|SettmpGoodsName _array_element)
              (if (> (.Value (Utilities|Map|Find (LocalVariables|GettmpInventoryMap) (LocalVariables|GettmpGoodsName))) 0.0)
                (LocalVariables|SettmpGoodsQuantity (Utilities|Struct|MakeGoodsQuantity (LocalVariables|GettmpGoodsName) (Math|Float|Min(Float) (.Value (Utilities|Map|Find (LocalVariables|GettmpInventoryMap) (LocalVariables|GettmpGoodsName))) (Variables|/Game/FungusFarm/Blueprints/Equipment/EquipmentMods/LabEquipmentMod_GoodsMoverMinion.LabEquipmentMod_GoodsMoverMinion_C|GetPullQuantityPerBatch (Variables|Default|GetMyParentMod)))))
                (goto _label Break)))
            (:Completed
              (if (> (.Quantity (Utilities|Struct|BreakGoodsQuantity (LocalVariables|GettmpGoodsQuantity))) 0.0)
                (bind _aslab_equipment_base_bp (Utilities|Casting|CastToLabEquipmentBase_BP (Default|GetModifiedParent (Variables|Default|GetMyParentMod))))
                (Default|TransferGoodstoOther (Variables|Default|GetGoodsInventory) (Variables|/Game/FungusFarm/Blueprints/Equipment/LabEquipment/LabEquipmentBase_BP.LabEquipmentBase_BP_C|GetFF_GoodsInventory_Component _aslab_equipment_base_bp) (LocalVariables|GettmpGoodsQuantity))
                (CallFunction|UpdateGoodsThumb)
                (return (Default|IsEmpty? (Variables|Default|GetGoodsInventory)))
                (else
                  (return true))))))
        (:Is%20Not%20Valid
          (return false))))))

(fn PickupGoodsfromTarget
  (Utilities|IsValid (Variables|Default|GetPullFromEquipment)
    (:Is%20Valid
      (LocalVariables|SettmpSupplyQuantity (Default|GetGoodsInventoryQuantity (Variables|/Game/FungusFarm/Blueprints/Equipment/LabEquipment/LabEquipmentBase_BP.LabEquipmentBase_BP_C|GetFF_GoodsInventory_Component (Variables|Default|GetPullFromEquipment)) (Variables|/Game/FungusFarm/Blueprints/Equipment/EquipmentMods/LabEquipmentMod_GoodsMoverMinion.LabEquipmentMod_GoodsMoverMinion_C|GetPullGoodsName (Variables|Default|GetMyParentMod))))
      (LocalVariables|SettmpCurrentInvQuantity (Default|GetGoodsInventoryQuantity (Variables|Default|GetGoodsInventory) (Variables|/Game/FungusFarm/Blueprints/Equipment/EquipmentMods/LabEquipmentMod_GoodsMoverMinion.LabEquipmentMod_GoodsMoverMinion_C|GetPullGoodsName (Variables|Default|GetMyParentMod))))
      (LocalVariables|SettmpTransferQuantity (Math|Float|Clamp(Float) (- (Variables|/Game/FungusFarm/Blueprints/Equipment/EquipmentMods/LabEquipmentMod_GoodsMoverMinion.LabEquipmentMod_GoodsMoverMinion_C|GetMaxPullQuantity (Variables|Default|GetMyParentMod)) (LocalVariables|GettmpCurrentInvQuantity)) 0.0 (Math|Float|Min(Float) (Variables|/Game/FungusFarm/Blueprints/Equipment/EquipmentMods/LabEquipmentMod_GoodsMoverMinion.LabEquipmentMod_GoodsMoverMinion_C|GetPullQuantityPerBatch (Variables|Default|GetMyParentMod)) (LocalVariables|GettmpSupplyQuantity))))
      (if (and (> (LocalVariables|GettmpSupplyQuantity) 0.0) (> (LocalVariables|GettmpTransferQuantity) 0.0))
        (bind _output_get (LocalVariables|SettmpTransferGoods (Utilities|Struct|MakeGoodsQuantity (Variables|/Game/FungusFarm/Blueprints/Equipment/EquipmentMods/LabEquipmentMod_GoodsMoverMinion.LabEquipmentMod_GoodsMoverMinion_C|GetPullGoodsName (Variables|Default|GetMyParentMod)) (LocalVariables|GettmpTransferQuantity))))
        (bind _successful (Default|TransferGoodstoOther (Variables|/Game/FungusFarm/Blueprints/Equipment/LabEquipment/LabEquipmentBase_BP.LabEquipmentBase_BP_C|GetFF_GoodsInventory_Component (Variables|Default|GetPullFromEquipment)) (Variables|Default|GetGoodsInventory) _output_get))
        (CallFunction|UpdateGoodsThumb)
        (if _successful
          (return (select (>= (+ (LocalVariables|GettmpCurrentInvQuantity) (LocalVariables|GettmpTransferQuantity)) (Variables|/Game/FungusFarm/Blueprints/Equipment/EquipmentMods/LabEquipmentMod_GoodsMoverMinion.LabEquipmentMod_GoodsMoverMinion_C|GetMaxPullQuantity (Variables|Default|GetMyParentMod))) true (not (> (- (LocalVariables|GettmpSupplyQuantity) (LocalVariables|GettmpTransferQuantity)) 0.0))))
          (else
            (Development|PrintString "Inventory pull unsuccessful" true true "(R=1.000000,G=0.010362,B=0.020309,A=1.000000)" 1e+01)
            (return true)))
        (else
          (return (>= (LocalVariables|GettmpCurrentInvQuantity) (Variables|/Game/FungusFarm/Blueprints/Equipment/EquipmentMods/LabEquipmentMod_GoodsMoverMinion.LabEquipmentMod_GoodsMoverMinion_C|GetMinPullQuantity (Variables|Default|GetMyParentMod)))))))
    (:Is%20Not%20Valid
      (return false))))

(fn TryDropGoodstoParent
  (bind _ballgoodstransferred (CallFunction|DropGoodstoParentMod))
  (if _ballgoodstransferred
    (Utilities|Time|PauseTimerbyHandle (Variables|Default|GetDropToParentTimer))
    (Variables|Default|SetbTransferring false)
    (Variables|Default|SetbReturningToHome false)
    (Variables|Default|SetbTravelIsActive false)))

(fn TryPickupGoodsfromTarget
  (bind _bcompletedpickup (CallFunction|PickupGoodsfromTarget))
  (if _bcompletedpickup
    (Utilities|Time|PauseTimerbyHandle (Variables|Default|GetPickupFromTargetTimer))
    (Variables|Default|SetbTransferring false)
    (Variables|Default|SetbReturningToHome true)
    (Variables|Default|SetbTravelIsActive true)))