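; Base Blueprint for tools in FungusFarm that carry a global gameplay modifier.
; ApplyEffects registers the tool's GlobalModifiers entry with the supplied GlobalManager, and RemoveEffects removes it again by its UniqueName.
; Both functions do nothing when that UniqueName is None, so a tool without a named modifier has no global effect.
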(fn ApplyEffects
  (params (GlobalManager :type Global%20Manager%20Object%20Reference))
  (if (Utilities|Name|NotEqual(Name) (.UniqueName (Utilities|Struct|BreakGlobalEffect (Variables|Default|GetGlobalModifiers))) "None")
    (Class|GlobalManager|AddGlobalEffects GlobalManager (Utilities|Array|MakeArray (Variables|Default|GetGlobalModifiers)))))

(fn RemoveEffects
  (params (GlobalManager :type Global%20Manager%20Object%20Reference))
  (bind _globalmodifiers (Variables|Default|GetGlobalModifiers))
  (bind _uniquename (Utilities|Struct|BreakGlobalEffect _globalmodifiers))
  (if (Utilities|Name|NotEqual(Name) _uniquename "None")
    (Class|GlobalManager|RemoveGlobalEffect GlobalManager _uniquename)))