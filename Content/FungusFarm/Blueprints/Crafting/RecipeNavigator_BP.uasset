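; RecipeNavigator_BP indexes crafting recipes and works out the base goods and gold values behind crafted goods.
; On BeginPlay it gets FF_GameState, retrying if needed, and caches maps from goods to producing and consuming recipes.
; Mutual recursion reduces recipes to Resource, Spores and Caps, using each good's last producing recipe and average yield.
; Gold value recurses through all producing recipes, scales input costs by recipe tier and keeps the cheapest.
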(event EventBeginPlay
  (bind _asff_game_state (Utilities|Casting|CastToFF_GameState (Game|GetGameState) :!label _label)
    (:then
      (Variables|Default|SetGameState _asff_game_state)
      (CallFunction|RefreshRecipeDataCache))
    (:CastFailed
      (Utilities|FlowControl|DoN 30
        (:Exit
          (Utilities|FlowControl|Delay 0.15)
          (goto _label))))))

(fn BaseGoodsforRecipe
  (params (RecipeName :type Name))
  (bind _gamestate (Variables|Default|GetGameState))
  (bind (_found _recipe) (Default|GetRecipeData _gamestate RecipeName))
  (if _found
    (for _array_element (.CraftingInputs (Utilities|Struct|BreakCraftingRecipe _recipe))
      (if (Math|Boolean|ORBoolean (Utilities|Array|ContainsItem (.GoodsCategories (Utilities|Struct|BreakGoodsType (.GoodsData (Default|GetGoodsData (Variables|Default|GetGameState) (.Name (Utilities|Struct|BreakGoodsQuantity _array_element)))))) "Resource") (Utilities|Array|ContainsItem (.GoodsCategories (Utilities|Struct|BreakGoodsType (.GoodsData (Default|GetGoodsData (Variables|Default|GetGameState) (.Name (Utilities|Struct|BreakGoodsQuantity _array_element)))))) "Spores") (Utilities|Array|ContainsItem (.GoodsCategories (Utilities|Struct|BreakGoodsType (.GoodsData (Default|GetGoodsData (Variables|Default|GetGameState) (.Name (Utilities|Struct|BreakGoodsQuantity _array_element)))))) "Caps"))
        (Utilities|Array|Add (LocalVariables|GettmpBaseGoods) _array_element)
        (else
          (bind _basegoods (CallFunction|BaseGoodsforGood (.Name (Utilities|Struct|BreakGoodsType (.GoodsData (Default|GetGoodsData (Variables|Default|GetGameState) (.Name (Utilities|Struct|BreakGoodsQuantity _array_element)))))) (.Quantity (Utilities|Struct|BreakGoodsQuantity _array_element))))
          (Utilities|Array|AppendArray (LocalVariables|GettmpBaseGoods) _basegoods)))))
  (bind _summed_goods (CallFunction|SumGoodsArray (LocalVariables|GettmpBaseGoods)))
  (return _summed_goods))

(fn RefreshRecipeDataCache
  (bind _all_recipes (Default|GetAllRecipes (Variables|Default|GetGameState)))
  (for _array_element _all_recipes
    (LocalVariables|SettmpRecipeName (.Name (Utilities|Struct|BreakCraftingRecipe _array_element)))
    (Utilities|FlowControl|Sequence
      (:then_0
        ;[1 1 1] Recipes by what they produce
        (for _array_element_2 (.CraftingResults (Utilities|Struct|BreakCraftingRecipe _array_element))
          (if (> (.PercentChance (Utilities|Struct|BreakGoodsDropChance _array_element_2)) 0.0)
            (for _array_element_3 (.GoodsOdds (Utilities|Struct|BreakGoodsDropChance _array_element_2))
              (if (> (.QuantityMin (Utilities|Struct|BreakGoodsQuantityRange _array_element_3)) 0.0)
                (LocalVariables|SettmpNameArray (.Value (Utilities|Map|Find (Variables|Default|GetGoodsToProducingRecipes) (.Name (Utilities|Struct|BreakGoodsQuantityRange _array_element_3)))))
                (if (.ReturnValue (Utilities|Map|Find (Variables|Default|GetGoodsToProducingRecipes) (.Name (Utilities|Struct|BreakGoodsQuantityRange _array_element_3))))
                  (Utilities|Array|AddUnique (Utilities|Struct|BreakNameArray (LocalVariables|GettmpNameArray)) (LocalVariables|GettmpRecipeName))
                  (Utilities|Map|Add (Variables|Default|GetGoodsToProducingRecipes) (.Name (Utilities|Struct|BreakGoodsQuantityRange _array_element_3)) (LocalVariables|GettmpNameArray))
                  (else
                    (Utilities|Map|Add (Variables|Default|GetGoodsToProducingRecipes) (.Name (Utilities|Struct|BreakGoodsQuantityRange _array_element_3)) (Utilities|Struct|MakeNameArray (Utilities|Array|MakeArray (LocalVariables|GettmpRecipeName)))))))))))
      (:then_1
        ;[1 1 1] Recipes by what they consume
        (for _array_element_4 (.CraftingInputs (Utilities|Struct|BreakCraftingRecipe _array_element))
          (LocalVariables|SettmpNameArray (.Value (Utilities|Map|Find (Variables|Default|GetGoodsToConsumingRecipes) (.Name (Utilities|Struct|BreakGoodsQuantity _array_element_4)))))
          (if (.ReturnValue (Utilities|Map|Find (Variables|Default|GetGoodsToConsumingRecipes) (.Name (Utilities|Struct|BreakGoodsQuantity _array_element_4))))
            (Utilities|Array|AddUnique (Utilities|Struct|BreakNameArray (LocalVariables|GettmpNameArray)) (LocalVariables|GettmpRecipeName))
            (Utilities|Map|Add (Variables|Default|GetGoodsToConsumingRecipes) (.Name (Utilities|Struct|BreakGoodsQuantity _array_element_4)) (LocalVariables|GettmpNameArray))
            (else
              (Utilities|Map|Add (Variables|Default|GetGoodsToConsumingRecipes) (.Name (Utilities|Struct|BreakGoodsQuantity _array_element_4)) (Utilities|Struct|MakeNameArray (Utilities|Array|MakeArray (LocalVariables|GettmpRecipeName)))))))))))

(fn BaseGoodsforRecipeRaw
  (params (Recipe%20Name :type Name))
  (bind _gamestate (Variables|Default|GetGameState))
  (bind (_found _recipe) (Default|GetRecipeData _gamestate Recipe%20Name))
  (if _found
    (for _array_element (.CraftingInputs (Utilities|Struct|BreakCraftingRecipe _recipe))
      (if (Math|Boolean|ORBoolean (Utilities|Array|ContainsItem (.GoodsCategories (Utilities|Struct|BreakGoodsType (.GoodsData (Default|GetGoodsData (Variables|Default|GetGameState) (.Name (Utilities|Struct|BreakGoodsQuantity _array_element)))))) "Resource") (Utilities|Array|ContainsItem (.GoodsCategories (Utilities|Struct|BreakGoodsType (.GoodsData (Default|GetGoodsData (Variables|Default|GetGameState) (.Name (Utilities|Struct|BreakGoodsQuantity _array_element)))))) "Spores") (Utilities|Array|ContainsItem (.GoodsCategories (Utilities|Struct|BreakGoodsType (.GoodsData (Default|GetGoodsData (Variables|Default|GetGameState) (.Name (Utilities|Struct|BreakGoodsQuantity _array_element)))))) "Caps"))
        (Utilities|Array|Add (LocalVariables|GettmpBaseGoods) _array_element)
        (else
          (bind _basegoods (CallFunction|BaseGoodsforGood (.Name (Utilities|Struct|BreakGoodsType (.GoodsData (Default|GetGoodsData (Variables|Default|GetGameState) (.Name (Utilities|Struct|BreakGoodsQuantity _array_element)))))) (.Quantity (Utilities|Struct|BreakGoodsQuantity _array_element))))
          (Utilities|Array|AppendArray (LocalVariables|GettmpBaseGoods) _basegoods)))))
  (return (LocalVariables|GettmpBaseGoods)))

(fn GetRecipesThatProduceGood
  (params (Goods%20Name :type Name))
  (bind _goodstoproducingrecipes (Variables|Default|GetGoodsToProducingRecipes))
  (bind (_value _returnvalue) (Utilities|Map|Find _goodstoproducingrecipes Goods%20Name))
  (if _returnvalue
    (return (Utilities|Struct|BreakNameArray _value))
    (else
      (return (Utilities|Array|MakeArray)))))

(fn GetRecipesThatConsumeGood
  (params (Goods%20Name :type Name))
  (bind _goodstoconsumingrecipes (Variables|Default|GetGoodsToConsumingRecipes))
  (bind (_value _returnvalue) (Utilities|Map|Find _goodstoconsumingrecipes Goods%20Name))
  (if _returnvalue
    (return (Utilities|Struct|BreakNameArray _value))
    (else
      (return (Utilities|Array|MakeArray)))))

(fn GoldValueforGood
  (params (GoodsName :type Name) (Quantity :type Float%20%28single-precision%29))
  (bind _gamestate (Variables|Default|GetGameState))
  (bind _tmprecipegoldvalues (LocalVariables|GettmpRecipeGoldValues))
  (bind _goodsdata (Default|GetGoodsData _gamestate GoodsName))
  (bind _minvalue (Math|Float|MinOfFloatArray _tmprecipegoldvalues))
  (bind (_name _displayname _thumbnail _equipmentname _goodsparenttype _sellvalue _buycost _goodscategories) (Utilities|Struct|BreakGoodsType _goodsdata))
  (bind _returnvalue (>= _minvalue 1e+01))
  (bind _returnvalue_2 (Math|Float|Truncate _minvalue))
  (bind _returnvalue_3 (* _minvalue 1e+03))
  (bind _returnvalue_4 (Math|Conversions|ToFloat(Integer) _returnvalue_2))
  (bind _returnvalue_5 (Math|Float|Truncate _returnvalue_3))
  (bind _returnvalue_6 (* Quantity _sellvalue))
  (bind _returnvalue_7 (Math|Conversions|ToFloat(Integer) _returnvalue_5))
  (bind _returnvalue_8 (/ _returnvalue_7 1e+03))
  (bind _returnvalue_9 (select _returnvalue _returnvalue_4 _returnvalue_8))
  (Math|Integer|IncrementInt (Variables|Default|GettmpRecursionLevel)
    (:%20%20
      (if (Math|Boolean|ORBoolean (Utilities|Array|ContainsItem _goodscategories "Resource") (Utilities|Array|ContainsItem _goodscategories "Spores") (Utilities|Array|ContainsItem _goodscategories "Caps"))
        (CallFunction|PrintGoodsValueDebug GoodsName Quantity _returnvalue_6)
        (Math|Integer|DecrementInt (Variables|Default|GettmpRecursionLevel)
          (:%20%20
            (return _returnvalue_6)))
        (else
          (bind _recipe_names (CallFunction|GetRecipesThatProduceGood GoodsName))
          (for _array_element _recipe_names
            (LocalVariables|SettmpProducedGoods 0.0)
            (LocalVariables|SettmpGoldSum 0.0)
            (LocalVariables|SettmpRecipeData (.Recipe (Default|GetRecipeData (Variables|Default|GetGameState) _array_element)))
            (bind _array_element_2 (Utilities|Array|ForEachLoopwithBreak (.CraftingResults (Utilities|Struct|BreakCraftingRecipe (LocalVariables|GettmpRecipeData))))
              (:LoopBody
                (if (> (.PercentChance (Utilities|Struct|BreakGoodsDropChance _array_element_2)) 0.0)
                  (bind _array_element_3 (Utilities|Array|ForEachLoopwithBreak (.GoodsOdds (Utilities|Struct|BreakGoodsDropChance _array_element_2)) :!label _label)
                    (:LoopBody
                      (if (Utilities|Name|Equal(Name) GoodsName (.Name (Utilities|Struct|BreakGoodsQuantityRange _array_element_3)))
                        (LocalVariables|SettmpProducedGoods (+ (LocalVariables|GettmpProducedGoods) (/ (+ (.QuantityMin (Utilities|Struct|BreakGoodsQuantityRange _array_element_3)) (.QuantityMax (Utilities|Struct|BreakGoodsQuantityRange _array_element_3))) 2.0)))
                        (goto _label Break))))))
              (:Completed
                (for _array_element_4 (.CraftingInputs (Utilities|Struct|BreakCraftingRecipe (LocalVariables|GettmpRecipeData)))
                  (bind _sell_value (CallFunction|GoldValueforGood (.Name (Utilities|Struct|BreakGoodsQuantity _array_element_4)) (* (.Quantity (Utilities|Struct|BreakGoodsQuantity _array_element_4)) (/ Quantity (LocalVariables|GettmpProducedGoods)))))
                  (LocalVariables|SettmpGoldSum (+ (* _sell_value (+ (LocalVariables|GettmpBaseTierValueMultiplier) (* (LocalVariables|GettmpTierIncrement) (Math|Conversions|ToFloat(Integer) (.Tier (Utilities|Struct|BreakCraftingRecipe (LocalVariables|GettmpRecipeData))))))) (LocalVariables|GettmpGoldSum))))
                (Utilities|Array|Add (LocalVariables|GettmpRecipeGoldValues) (LocalVariables|GettmpGoldSum)))))
          (CallFunction|PrintGoodsValueDebug GoodsName Quantity _returnvalue_9)
          (Math|Integer|DecrementInt (Variables|Default|GettmpRecursionLevel)
            (:%20%20
              (return _returnvalue_9))))))))

(fn GoldValueforGoods
  (params (Goods :type Array%20of%20Goods%20Quantity%20Structures))
  (for _array_element Goods
    (bind _sell_value (CallFunction|GoldValueforGood (.Name (Utilities|Struct|BreakGoodsQuantity _array_element)) (.Quantity (Utilities|Struct|BreakGoodsQuantity _array_element))))
    (LocalVariables|SettmpTotalVal (+ _sell_value (LocalVariables|GettmpTotalVal))))
  (return (LocalVariables|GettmpTotalVal)))

(fn BaseGoodsforGood
  (params (GoodsName :type Name) (Quantity :type Float%20%28single-precision%29))
  (bind _recipe_names (CallFunction|GetRecipesThatProduceGood GoodsName))
  (if (> (Utilities|Array|Length _recipe_names) 0)
    (for _array_element (.CraftingResults (Utilities|Struct|BreakCraftingRecipe (.Recipe (Default|GetRecipeData (Variables|Default|GetGameState) (Utilities|Array|Get(acopy) _recipe_names (Utilities|Array|LastIndex _recipe_names))))))
      (if (> (.PercentChance (Utilities|Struct|BreakGoodsDropChance _array_element)) 0.0)
        (bind _array_element_2 (Utilities|Array|ForEachLoopwithBreak (.GoodsOdds (Utilities|Struct|BreakGoodsDropChance _array_element)) :!label _label)
          (:LoopBody
            (if (Utilities|Name|Equal(Name) GoodsName (.Name (Utilities|Struct|BreakGoodsQuantityRange _array_element_2)))
              (LocalVariables|SettmpProducedGoods (+ (LocalVariables|GettmpProducedGoods) (/ (+ (.QuantityMin (Utilities|Struct|BreakGoodsQuantityRange _array_element_2)) (.QuantityMax (Utilities|Struct|BreakGoodsQuantityRange _array_element_2))) 2.0)))
              (goto _label Break))))))
    (bind _basegoods (CallFunction|BaseGoodsforRecipe (Utilities|Array|Get(acopy) _recipe_names (Utilities|Array|LastIndex _recipe_names))))
    (return (CallFunction|MultiplyInventory _basegoods (/ Quantity (LocalVariables|GettmpProducedGoods)) false))
    (else
      (return (Utilities|Array|MakeArray (Utilities|Struct|MakeGoodsQuantity GoodsName Quantity))))))

(fn PrintGoodsValueDebug
  (params (GoodsName :type Name) (Quantity :type Float%20%28single-precision%29) (Value :type Float%20%28single-precision%29))
  (for _index (range 1 (Variables|Default|GettmpRecursionLevel))
    (LocalVariables|SettmpString (Utilities|String|Append (LocalVariables|GettmpString) " - ")))
  (Development|PrintString (Utilities|String|Append (LocalVariables|GettmpString) (Utilities|String|ToString(Name) GoodsName) "(" (Utilities|String|ToString(Float) Quantity) ")=" (Utilities|String|ToString(Float) Value)) false))