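; FF_CraftQueueSlot is a crafting queue slot that tracks a Quantity for Fungus Farm's crafting system.
; AddSubtractQuantity applies a signed delta, clamps the result to a hard-coded range of zero to one hundred, and stores it.
; It returns the new quantity plus any overflow or underflow the slot could not absorb, and a zero delta returns early without changes.
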(fn AddSubtractQuantity
  (params (QuantityDelta :type Integer))
  (if (== QuantityDelta 0)
    (return (Variables|Default|GetQuantity) 0)
    (else
      (LocalVariables|SettmpRemaining (- (+ QuantityDelta (Variables|Default|GetQuantity)) (Math|Integer|Clamp(Integer) (+ QuantityDelta (Variables|Default|GetQuantity)) 0 100)))
      (bind _output_get (Variables|Default|SetQuantity (Math|Integer|Clamp(Integer) (+ QuantityDelta (Variables|Default|GetQuantity)) 0 100)))
      (return _output_get (LocalVariables|GettmpRemaining)))))