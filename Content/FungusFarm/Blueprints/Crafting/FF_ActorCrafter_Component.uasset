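; Actor component for Fungus Farm that crafts queued recipes from a linked inventory, registering with the game state and following game pause.
; A looping timer takes the first queued recipe with available inputs, consumes them, advances progress, and deposits rolled drops, carrying leftover time into further recipes.
; The queue uses capped, stackable slot objects, broadcasts changes through dispatchers, and is saved as name/quantity pairs rebuilt via game state recipe lookup.
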(event Custom|RefreshFromSerialized
  ;[1 1 1] Serialize
  (Utilities|FlowControl|Sequence
    (:then_0
      (Variables|Default|SettmpCraftingState (Variables|Default|GetCraftingState))
      (CallFunction|PauseCrafting)
      (CallFunction|EmptytheCraftingQueue))
    (:then_1
      (for _array_element (Variables|Default|GetserializedCrafting%20Queue)
        (bind _ffgamestate (Utilities|GetGameState))
        (if (.Found (Default|GetRecipeData _ffgamestate (.Name (Utilities|Struct|BreakCraftingSlot _array_element))))
          (CallFunction|AddtoCraftingQueue (.Recipe (Default|GetRecipeData _ffgamestate (.Name (Utilities|Struct|BreakCraftingSlot _array_element)))) (.Value (Utilities|Struct|BreakCraftingSlot _array_element))))))
    (:then_2
      (if (Utilities|Enum|NotEqual(Enum) (Variables|Default|GettmpCraftingState) "NewEnumerator3")
        (CallFunction|UnpauseCrafting)))))

(event Custom|SaveToSerialized
  ;[1 1 1] Serialize
  (Utilities|FlowControl|Sequence
    (:then_0
      (Variables|Default|SettmpCraftingState (Variables|Default|GetCraftingState))
      (CallFunction|PauseCrafting)
      (Utilities|Array|Clear (Variables|Default|GetserializedCrafting%20Queue)))
    (:then_1
      (for _array_element (Variables|Default|GetRecipeQueue)
        (Utilities|Array|Add (Variables|Default|GetserializedCrafting%20Queue) (Utilities|Struct|MakeCraftingSlot (.Name (Utilities|Struct|BreakCraftingRecipe (Variables|/Game/FungusFarm/Blueprints/Crafting/FF_CraftQueueSlot.FF_CraftQueueSlot_C|GetRecipe _array_element))) (Variables|/Game/FungusFarm/Blueprints/Crafting/FF_CraftQueueSlot.FF_CraftQueueSlot_C|GetQuantity _array_element)))))
    (:then_2
      (if (Utilities|Enum|NotEqual(Enum) (Variables|Default|GettmpCraftingState) "NewEnumerator3")
        (CallFunction|UnpauseCrafting)))))

(event Custom|OnGamePaused
  (CallFunction|PauseCrafting))

(event Custom|OnGameUnpaused
  (CallFunction|UnpauseCrafting))

(event EventBeginPlay
  (Utilities|FlowControl|Sequence
    (:then_0
      (bind _ffgamestate (Utilities|GetGameState))
      (Default|BindtoMonitoredCrafter _ffgamestate self)
      (EventDispatchers|BindEventtoOnGamePaused _ffgamestate (delegate Custom|OnGamePaused))
      (EventDispatchers|BindEventtoOnGameUnPaused _ffgamestate (delegate Custom|OnGameUnpaused)))
    (:then_1
      (bind _returnvalue (Utilities|Time|SetTimerbyFunctionName 0 "CraftingTick" 0.2 true))
      (Variables|Default|SetCraftingTimer _returnvalue))))

(event EventEndPlay
  (params (EndPlayReason :type EEndPlayReason%20Enum :default "Destroyed"))
  (Utilities|Time|ClearandInvalidateTimerbyHandle (Variables|Default|GetCraftingTimer))
  (bind _ffgamestate (Utilities|GetGameState))
  (Default|UnbindMonitoredCrafter _ffgamestate self)
  (EventDispatchers|UnbindEventfromOnGamePaused _ffgamestate (delegate Custom|OnGamePaused))
  (EventDispatchers|UnbindEventfromOnGameUnPaused _ffgamestate (delegate Custom|OnGameUnpaused)))

(fn CraftingTick
  (LocalVariables|SettmpCraftedGoods (Utilities|Array|MakeArray))
  (LocalVariables|SettmpDeltaTime (Class|KismetSystemLibrary|GetTimerElapsedTimeHandle (Variables|Default|GetCraftingTimer)))
  (switch Utilities|FlowControl|Switch|SwitchonFF_CraftingState (Variables|Default|GetCraftingState)
    (:NewEnumerator0
      ;[1 1 1] Idle - Go to crafting if we can pop a queued recipe
      (if (Utilities|CurrentRecipeIsNothing?) :!label _label
        (if (CallFunction|AnythingtoCraft?)
          (bind _recipe_returned (CallFunction|PopNextCraftableinQueue))
          (if _recipe_returned
            (CallFunction|SetCraftingState "NewEnumerator1" :!label _label_2)
            (while (Math|Boolean|ANDBoolean (Utilities|Enum|Equal(Enum) (Variables|Default|GetCraftingState) "NewEnumerator1") (> (LocalVariables|GettmpDeltaTime) 0.0) (CallFunction|AnythingtoCraft?)) :!label _label_3
              (Utilities|FlowControl|Sequence
                (:then_0
                  ;[1 1 1] Pop the next recipe (than can be built) from the queue if we don't have a current one
                  (if (Utilities|CurrentRecipeIsNothing?)
                    (bind _recipe_returned_2 (CallFunction|PopNextCraftableinQueue))
                    (if (not _recipe_returned_2)
                      ;[1 1 1] Nothing we have inputs to craft for
                      (CallFunction|SetCraftingState (select (CallFunction|AnythingtoCraft?) "NewEnumerator2" "NewEnumerator0")))))
                (:then_1
                  ;[1 1 1] Crafting Work
                  (if (and (Utilities|Enum|Equal(Enum) (Variables|Default|GetCraftingState) "NewEnumerator1") (not (Utilities|CurrentRecipeIsNothing?)))
                    (bind (_completed_recipe _crafted_goods _time_remaining) (CallFunction|WorkCurrentRecipe (LocalVariables|GettmpDeltaTime)))
                    (if _completed_recipe
                      (Utilities|Array|AppendArray (LocalVariables|GettmpCraftedGoods) _crafted_goods))
                    (LocalVariables|SettmpDeltaTime _time_remaining)))
                (:then_2
                  ;[1 1 1] Add goods to inventory
                  (if (> (Utilities|Array|Length (LocalVariables|GettmpCraftedGoods)) 0)
                    (Default|AddGoodsInventoryBatch (Variables|Default|GetInventoryRef) (LocalVariables|GettmpCraftedGoods))
                    (Utilities|Array|Clear (LocalVariables|GettmpCraftedGoods))))))
            ;[1 1 1] If there is still time left, then we've gone idle.
            (if (Utilities|Enum|Equal(Enum) (Variables|Default|GetCraftingState) "NewEnumerator1")
              (if (> (LocalVariables|GettmpDeltaTime) 0.0)
                (CallFunction|SetCraftingState (select (CallFunction|AnythingtoCraft?) "NewEnumerator2" "NewEnumerator0"))))))
        (else
          (goto _label_2))))
    (:NewEnumerator1
      (goto _label_3))
    (:NewEnumerator2
      (goto _label))))

(fn CraftItemComplete
  (Utilities|FlowControl|Sequence
    (:then_0
      (LocalVariables|SettmpCompletedRecipe (Variables|Default|GetCurrentRecipe))
      (LocalVariables|SettmpDroppedGoods (Class|GoodsFunctionLibrary|EvaluateGoodsDrops (.CraftingResults (Utilities|Struct|BreakCraftingRecipe (Variables|Default|GetCurrentRecipe))) -1.0))
      (CallFunction|ClearCurrentRecipe)
      (Variables|Default|SetCurrentProgress 0.0)
      (Default|CallOnProgressChanged (CallFunction|GetPercentComplete)))
    (:then_1
      ;[1 1 1] Logging
      (Development|PrintString "Crafted:")
      (for _array_element (LocalVariables|GettmpDroppedGoods)
        (Development|PrintString (Utilities|String|BuildString(Float) (Utilities|String|ToString(Name) (.Name (Utilities|Struct|BreakGoodsQuantity _array_element))) " " (.Quantity (Utilities|Struct|BreakGoodsQuantity _array_element))))))
    (:then_2
      (Default|CallOnCraftComplete (LocalVariables|GettmpCompletedRecipe) (LocalVariables|GettmpDroppedGoods))
      (return (LocalVariables|GettmpDroppedGoods)))))

(fn GetTimeRemaining
  (bind _currentrecipe (Variables|Default|GetCurrentRecipe))
  (bind (_name _recipecategories _displayname _thumbnail _reciperequirements _unlockcosts _craftinginputs _craftingresults _bonuscraftingresults _tier _craftingtime) (Utilities|Struct|BreakCraftingRecipe _currentrecipe))
  (if (Utilities|Name|Equal(Name) _name "None")
    (return 0.0)
    (else
      (return (/ (- _craftingtime (Variables|Default|GetCurrentProgress)) (CallFunction|CalculatedCraftingSpeed))))))

(fn CalculatedCraftingSpeed
  (return (Variables|Default|GetCraftingSpeed)))

(fn GetCraftingTimeforRecipe
  (params (Recipe :type Crafting%20Recipe%20Structure))
  (return (/ (.CraftingTime (Utilities|Struct|BreakCraftingRecipe Recipe)) (CallFunction|CalculatedCraftingSpeed))))

(fn PauseCrafting
  (CallFunction|SetCraftingState "NewEnumerator3")
  (Utilities|Time|PauseTimerbyHandle (Variables|Default|GetCraftingTimer)))

(fn CancelCrafting
  ;[1 1 1] ToDo: Refund Inputs
  (Variables|Default|SetCraftingState "NewEnumerator0")
  (Variables|Default|SetCurrentProgress 0.0)
  (CallFunction|ClearCurrentRecipe)
  (Default|CallOnProgressChanged 0.0))

(fn AddtoCraftingQueue
  (params (Recipe :type Crafting%20Recipe%20Structure) (Quantity :type Integer))
  (bind _output_get (LocalVariables|SettmpQuantity Quantity))
  (if (!= _output_get 0)
    (Utilities|FlowControl|Sequence
      (:then_0
        ;[1 1 1] Add to existing slots
        (bind (_found_ _indexes _queueslots) (CallFunction|FindRecipeinQueue Recipe))
        (if _found_
          (bind _array_element (Utilities|Array|ForEachLoopwithBreak _queueslots :!label _label)
            (:LoopBody
              (bind _remainingquantitydelta (Default|AddSubtractQuantity _array_element (LocalVariables|GettmpQuantity)))
              (if (!= _remainingquantitydelta (LocalVariables|GettmpQuantity))
                (LocalVariables|SettmpQuantity _remainingquantitydelta)
                (LocalVariables|SetSlotQuantityChanged true))
              (if (not (> (LocalVariables|GettmpQuantity) 0))
                (goto _label Break))))))
      (:then_1
        ;[1 1 1] Add a new slots
        (while (and (> (LocalVariables|GettmpQuantity) 0) (< (Utilities|Array|Length (Variables|Default|GetRecipeQueue)) (Variables|Default|GetMaximum%20Queue%20Slots)))
          (bind _returnvalue (Game|ConstructObjectfromClass "/Game/FungusFarm/Blueprints/Crafting/FF_CraftQueueSlot.FF_CraftQueueSlot_C" self 1 (Variables|Default|GetMaximum%20Stacks%20Per%20Slot) Recipe))
          (bind _result (Math|Integer|DecrementInt (LocalVariables|GettmpQuantity))
            (:%20%20
              (bind _remainingquantitydelta_2 (Default|AddSubtractQuantity _returnvalue _result))
              (LocalVariables|SettmpQuantity _remainingquantitydelta_2)
              (Utilities|Array|Add (Variables|Default|GetRecipeQueue) _returnvalue)
              (Utilities|Array|Add (LocalVariables|GettmpAddedSlotBPs) _returnvalue)))))
      (:then_2
        ;[1 1 1] Notify listeners
        (Utilities|FlowControl|Sequence
          (:then_0
            (if (LocalVariables|GetSlotQuantityChanged)
              (Default|CallOnQueuedRecipesQuantityChanged)))
          (:then_1
            (if (> (Utilities|Array|Length (LocalVariables|GettmpAddedSlotBPs)) 0)
              (Default|CallOnQueueSlotsAdded (LocalVariables|GettmpAddedSlotBPs)))))))))

(fn RemovefromCraftingQueue
  (params (Recipe :type Crafting%20Recipe%20Structure) (Quantity :type Integer))
  (bind _result (Utilities|NegateInt Quantity)
    (:%20%20
      (LocalVariables|SettmpRemoveQuantity _result)
      (Utilities|FlowControl|Sequence
        (:then_0
          ;[1 1 1] Remove recipes
          (bind (_found_ _indexes _queueslots) (CallFunction|FindRecipeinQueue Recipe))
          (if _found_
            (bind (_array_element _array_index) (Utilities|Array|ForEachLoopwithBreak _queueslots :!label _label)
              (:LoopBody
                (bind (_new_quantity _remainingquantitydelta) (Default|AddSubtractQuantity _array_element (LocalVariables|GettmpRemoveQuantity)))
                (LocalVariables|SettmpRemoveQuantity _remainingquantitydelta)
                (if (<= _new_quantity 0)
                  (Utilities|Array|Add (LocalVariables|GettmpRemoveEmptyIndexes) (Utilities|Array|Get(acopy) _indexes _array_index)))
                (if (>= (LocalVariables|GettmpRemoveQuantity) 0)
                  (goto _label Break))))))
        (:then_1
          ;[1 1 1] Remove empty queue slots
          (for _array_element_2 (LocalVariables|GettmpRemoveEmptyIndexes)
            (Utilities|Array|Add (LocalVariables|GettmpRemovedSlots) (Utilities|Array|Get(acopy) (Variables|Default|GetRecipeQueue) _array_element_2))
            (Utilities|Array|RemoveIndex (Variables|Default|GetRecipeQueue) _array_element_2)))
        (:then_2
          ;[1 1 1] Notify listeners of removed slots
          (if (> (Utilities|Array|Length (LocalVariables|GettmpRemovedSlots)) 0)
            (Default|CallOnQueueSlotsRemoved (LocalVariables|GettmpRemovedSlots))))
        (:then_3
          (bind _result_2 (Utilities|NegateInt (LocalVariables|GettmpRemoveQuantity))
            (:%20%20
              (return _result_2))))))))

(fn UnpauseCrafting
  (if (Class|KismetSystemLibrary|IsTimerPausedHandle (Variables|Default|GetCraftingTimer))
    (Utilities|Time|UnpauseTimerbyHandle (Variables|Default|GetCraftingTimer)))
  (if (Utilities|Enum|Equal(Enum) (Variables|Default|GetCraftingState) "NewEnumerator3")
    (CallFunction|SetCraftingState (select (Utilities|CurrentRecipeIsNothing?) "NewEnumerator0" "NewEnumerator1"))))

(fn SetCraftingState
  (params (New%20State :type FF_CraftingState%20Enum :default "NewEnumerator0"))
  (if (Utilities|Enum|NotEqual(Enum) (Variables|Default|GetCraftingState) New%20State)
    (LocalVariables|SettmpOldState (Variables|Default|GetCraftingState))
    (bind _output_get (Variables|Default|SetCraftingState New%20State))
    (switch Utilities|FlowControl|Switch|SwitchonFF_CraftingState _output_get)))

(fn ClearCurrentRecipe
  (Variables|Default|SetCurrentRecipe (Utilities|Struct|MakeCraftingRecipe "None" (Utilities|Array|MakeArray) "" 0 (Utilities|Array|MakeArray) (Utilities|Array|MakeArray) (Utilities|Array|MakeArray) (Utilities|Array|MakeArray) (Utilities|Array|MakeArray))))

(fn WorkCurrentRecipe
  (params (Delta%20Time :type Float%20%28single-precision%29))
  (LocalVariables|SettmpRemainingTime Delta%20Time)
  (if (>= (+ (* Delta%20Time (CallFunction|CalculatedCraftingSpeed)) (Variables|Default|GetCurrentProgress)) (.CraftingTime (Utilities|Struct|BreakCraftingRecipe (Variables|Default|GetCurrentRecipe))))
    (LocalVariables|SettmpRemainingTime (- (LocalVariables|GettmpRemainingTime) (/ (- (.CraftingTime (Utilities|Struct|BreakCraftingRecipe (Variables|Default|GetCurrentRecipe))) (Variables|Default|GetCurrentProgress)) (CallFunction|CalculatedCraftingSpeed))))
    (bind _produced_goods (CallFunction|CraftItemComplete))
    (return true _produced_goods (LocalVariables|GettmpRemainingTime))
    (else
      (Variables|Default|SetCurrentProgress (+ (* Delta%20Time (CallFunction|CalculatedCraftingSpeed)) (Variables|Default|GetCurrentProgress)))
      (Default|CallOnProgressChanged (CallFunction|GetPercentComplete))
      (return false 0 0.0))))

(fn PopNextCraftableinQueue
  (if (> (Utilities|Array|Length (Variables|Default|GetRecipeQueue)) 0)
    (Utilities|FlowControl|Sequence
      (:then_0
        ;[1 1 1] Find the first craftable recipe
        (bind _array_element (Utilities|Array|ForEachLoopwithBreak (Variables|Default|GetRecipeQueue) :!label _label)
          (:LoopBody
            (bind _hasall (Default|HasAllGoods? (Variables|Default|GetInventoryRef) (.CraftingInputs (Utilities|Struct|BreakCraftingRecipe (Variables|/Game/FungusFarm/Blueprints/Crafting/FF_CraftQueueSlot.FF_CraftQueueSlot_C|GetRecipe _array_element)))))
            (if _hasall
              (LocalVariables|SettmpRecipe (Variables|/Game/FungusFarm/Blueprints/Crafting/FF_CraftQueueSlot.FF_CraftQueueSlot_C|GetRecipe _array_element))
              (LocalVariables|SettmpRecipeFound true)
              (goto _label Break)))))
      (:then_1
        ;[1 1 1] Remove inputs from inventory
        (if (LocalVariables|GettmpRecipeFound)
          (bind _successful (Default|RemoveGoodsInventoryBatch (Variables|Default|GetInventoryRef) (.CraftingInputs (Utilities|Struct|BreakCraftingRecipe (LocalVariables|GettmpRecipe)))))
          (LocalVariables|SettmpRecipeFound _successful)))
      (:then_2
        ;[1 1 1] Remove it from queue
        (if (LocalVariables|GettmpRecipeFound)
          (bind _quantity_not_removed (CallFunction|RemovefromCraftingQueue (LocalVariables|GettmpRecipe) 1))
          (if (not (== _quantity_not_removed 0))
            (LocalVariables|SettmpRecipeFound false))))
      (:then_3
        ;[1 1 1] Set Current Recipe and Return
        (bind _output_get (Variables|Default|SetCurrentRecipe (LocalVariables|GettmpRecipe) :!label _label_2))
        (Default|CallOnNewCurrentRecipe _output_get)
        (return (LocalVariables|GettmpRecipeFound) (LocalVariables|GettmpRecipe))))
    (else
      (goto _label_2))))

(fn FindRecipeinQueue
  (params (Recipe :type Crafting%20Recipe%20Structure))
  (for (_array_element _array_index) (Variables|Default|GetRecipeQueue)
    (if (Utilities|Name|Equal(Name) (.Name (Utilities|Struct|BreakCraftingRecipe (Variables|/Game/FungusFarm/Blueprints/Crafting/FF_CraftQueueSlot.FF_CraftQueueSlot_C|GetRecipe _array_element))) (.Name (Utilities|Struct|BreakCraftingRecipe Recipe)))
      (Utilities|Array|Add (LocalVariables|GettmpQueueSlots) _array_element)
      (Utilities|Array|Add (LocalVariables|GettmpIndexes) _array_index)))
  (return (> (Utilities|Array|Length (LocalVariables|GettmpQueueSlots)) 0) (LocalVariables|GettmpIndexes) (LocalVariables|GettmpQueueSlots)))

(fn CanCraft?
  (params (Recipe :type Crafting%20Recipe%20Structure))
  (bind (_name _recipecategories _displayname _thumbnail _reciperequirements _unlockcosts _craftinginputs _craftingresults _bonuscraftingresults _tier) (Utilities|Struct|BreakCraftingRecipe Recipe))
  (bind _inventoryref (Variables|Default|GetInventoryRef))
  (if (and (CallFunction|HasAllNames? _recipecategories (Variables|Default|GetRequiredRecipeCategories)) (<= _tier (Variables|Default|GetMaximumTier)))
    (bind _asff_game_state (Utilities|Casting|CastToFF_GameState (Game|GetGameState))
      (:then
        (Utilities|IsValid _inventoryref
          (:Is%20Valid
            (bind _hasall (Default|HasAllGoods? _inventoryref _craftinginputs))
            (return (Default|RecipeUnlocked? _asff_game_state _name) _hasall))
          (:Is%20Not%20Valid
            (return (Default|RecipeUnlocked? _asff_game_state _name) false))))
      (:CastFailed
        _)))
  (return false false))

(fn GetPercentComplete
  (if (Utilities|CurrentRecipeIsNothing?)
    (return 0.0)
    (else
      (return (/ (Variables|Default|GetCurrentProgress) (.CraftingTime (Utilities|Struct|BreakCraftingRecipe (Variables|Default|GetCurrentRecipe))))))))

(fn AnythingtoCraft?
  (return (or (not (Utilities|CurrentRecipeIsNothing?)) (> (Utilities|Array|Length (Variables|Default|GetRecipeQueue)) 0))))

(fn RemovefromCraftingQueueSlot
  (params (Slot :type FF%20Craft%20Queue%20Slot%20Object%20Reference) (Quantity :type Integer))
  (LocalVariables|SettmpRemoveQuantity (* Quantity -1))
  (Utilities|FlowControl|Sequence
    (:then_0
      (bind (_new_quantity _remainingquantitydelta) (Default|AddSubtractQuantity Slot (LocalVariables|GettmpRemoveQuantity)))
      (LocalVariables|SettmpRemoveQuantity _remainingquantitydelta)
      (if (<= _new_quantity 0)
        (Utilities|Array|RemoveItem (Variables|Default|GetRecipeQueue) Slot)
        (Default|CallOnQueueSlotsRemoved (Utilities|Array|MakeArray Slot))
        (else
          (Default|CallOnQueuedRecipesQuantityChanged))))
    (:then_1
      (bind _result (Utilities|NegateInt (LocalVariables|GettmpRemoveQuantity))
        (:%20%20
          (return _result))))))

(fn ChangeQuantityinQueueSlotStruct
  (params (Slot :type Crafting%20Slot%20Structure) (Quantity%20Delta :type Integer))
  (bind _value (Utilities|Struct|BreakCraftingSlot Slot))
  (bind _maximum_stacks_per_slot (Variables|Default|GetMaximum%20Stacks%20Per%20Slot))
  (bind _returnvalue (+ Quantity%20Delta _value))
  (bind _returnvalue_2 (Math|Integer|Clamp(Integer) _returnvalue 0 _maximum_stacks_per_slot))
  (if (== Quantity%20Delta 0)
    (return _value 0)
    (else
      (LocalVariables|SettmpRemaining (- _returnvalue _returnvalue_2))
      (bind _structout (Utilities|Struct|SetmembersinCraftingSlot Slot _returnvalue_2))
      (Default|CallOnQueuedRecipesQuantityChanged)
      (return (.Value (Utilities|Struct|BreakCraftingSlot _structout)) (LocalVariables|GettmpRemaining)))))

(fn EmptytheCraftingQueue
  (bind _recipequeue (Variables|Default|GetRecipeQueue))
  (bind _output (Utilities|Array|Get(acopy) _recipequeue))
  (while (> (Utilities|Array|Length (Variables|Default|GetRecipeQueue)) 0)
    (CallFunction|RemovefromCraftingQueue (Variables|/Game/FungusFarm/Blueprints/Crafting/FF_CraftQueueSlot.FF_CraftQueueSlot_C|GetRecipe _output) (Variables|/Game/FungusFarm/Blueprints/Crafting/FF_CraftQueueSlot.FF_CraftQueueSlot_C|GetQuantity _output))))

(fn CurrentRecipeIsValid?
  (return (not (Utilities|Name|Equal(Name) (.Name (Utilities|Struct|BreakCraftingRecipe (Variables|Default|GetCurrentRecipe))) "None"))))

(fn SetInventory
  (params (InventoryComponent :type FF%20Goods%20Inventory%20Component%20Object%20Reference%20%28by%20ref%29))
  (Variables|Default|SetInventoryRef InventoryComponent))

(fn GetGoodsRequiredforQueue
  (for _array_element (Variables|Default|GetRecipeQueue)
    (if (> (Variables|/Game/FungusFarm/Blueprints/Crafting/FF_CraftQueueSlot.FF_CraftQueueSlot_C|GetQuantity _array_element) 0)
      (Utilities|Array|AppendArray (LocalVariables|GettmpAllGoods) (CallFunction|MultiplyInventory (.CraftingInputs (Utilities|Struct|BreakCraftingRecipe (Variables|/Game/FungusFarm/Blueprints/Crafting/FF_CraftQueueSlot.FF_CraftQueueSlot_C|GetRecipe _array_element))) (Math|Conversions|ToFloat(Integer) (Variables|/Game/FungusFarm/Blueprints/Crafting/FF_CraftQueueSlot.FF_CraftQueueSlot_C|GetQuantity _array_element)) false))))
  (bind _summed_goods (CallFunction|SumGoodsArray (LocalVariables|GettmpAllGoods)))
  (return _summed_goods))