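; Game mode for Fungus Farm that routes home, farm, lab and market level-load events to the player controller.
; Each event casts player 0's controller to FF_PlayerController_BP and shows the matching menu or passes on the current level name, with the home menu optional.
; BeginPlay sets the gameplay goals provider's image.
; Older level-streaming load and unload chains for home and farm remain in the graph but are unconnected.
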(event Custom|LoadHomeLevel
  (params (DontShowHomeMenu :type Boolean))
  (if (not DontShowHomeMenu)
    (bind _asff_player_controller_bp (Utilities|Casting|CastToFF_PlayerController_BP (Game|GetPlayerController 0)))
    (Default|ShowHomeMenu _asff_player_controller_bp)))

(event Custom|LoadCurrentFarmLevel
  (bind _asff_player_controller_bp (Utilities|Casting|CastToFF_PlayerController_BP (Game|GetPlayerController 0)))
  (Default|OnFarmLoaded _asff_player_controller_bp (Variables|Default|GetCurrentFarmLevelName)))

(event Custom|LoadCurrentLabLevel
  (bind _asff_player_controller_bp (Utilities|Casting|CastToFF_PlayerController_BP (Game|GetPlayerController 0)))
  (Default|OnLabLoaded _asff_player_controller_bp (Variables|Default|GetCurrentLabLevelName)))

(event Custom|LoadMarketLevel
  (bind _asff_player_controller_bp (Utilities|Casting|CastToFF_PlayerController_BP (Game|GetPlayerController 0)))
  (Default|ShowMarketMenu _asff_player_controller_bp))

(event EventBeginPlay
  (Variables|/Script/FungusFarm.GoalsProviderComponent|SetProviderImage (Variables|Default|GetGameplayGoalsProvider) "/Game/FungusFarm/Assets/Textures/Hexagram_512.Hexagram_512"))

(fn ConstructionScript)