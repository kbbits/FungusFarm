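; Fairydew drop resource node, a sprite-based physics drop that splats on impact and blinks as its remaining lifespan runs low.
; The first hit zeroes roll and yaw, spawns a Niagara splat, updates the state sprite and stops physics after a short delay.
; Tick pulses sprite brightness with a two-second triangle wave, built from modulo and absolute values, during the final ten seconds of LifespanAfterStopped.
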(event Custom|StopPhysics
  (bind _resourcesprite (Variables|Default|GetResourceSprite))
  (Utilities|FlowControl|Delay 0.25)
  (Class|PrimitiveComponent|SetAllPhysicsLinearVelocity _resourcesprite "0, 0, 0" false)
  (Physics|SetSimulatePhysics _resourcesprite false))

(event EventBeginPlay
  (|CallParentFunction) ; This node is disabled and will not be called.\nDrag off pins to build functionality.
)

(event Collision|EventActorBeginOverlap
  (params (OtherActor :type Actor%20Object%20Reference)))

(event EventTick
  (params (DeltaSeconds :type Float%20%28single-precision%29))
  (bind _lifespanafterstopped (Variables|Default|GetLifespanAfterStopped))
  (bind _returnvalue (Math|Float|%(Float) _lifespanafterstopped 2.0))
  (bind _returnvalue_2 (- _returnvalue 1.0))
  (bind _returnvalue_3 (Math|Float|Absolute(Float) _returnvalue_2))
  (bind _returnvalue_4 (- _returnvalue_3 1.0))
  (bind _returnvalue_5 (Math|Float|Absolute(Float) _returnvalue_4))
  (bind _returnvalue_6 (Math|Float|MapRangeClamped _returnvalue_5 0.0 1.0 0.2 1.0))
  (|CallParentFunction DeltaSeconds)
  (if (< (Variables|Default|GetLifespanAfterStopped) 1e+01)
    (Utilities|IsValid (Variables|Default|GetResourceSprite)
      (:Is%20Valid
        (Sprite|SetSpriteColor (Variables|Default|GetResourceSprite) (Utilities|Struct|MakeLinearColor _returnvalue_6 _returnvalue_6 _returnvalue_6 1.0))))))

(fn ConstructionScript
  (|CallParentFunction))

(fn OnHitFX
  (params (HitMagnitude :type Float%20%28single-precision%29))
  (|CallParentFunction HitMagnitude)
  (if (not (Variables|Default|GetAlreadyHit))
    (Variables|Default|SetAlreadyHit true)
    (Transformation|SetActorRotation (Math|Rotator|MakeRotator 0.0 (.Pitch (Math|Rotator|BreakRotator (Transformation|GetActorRotation))) 0.0))
    (Niagara|SpawnSystematLocation "/Game/FungusFarm/Assets/Particles/FairydewSplat/FairydewSplat_NS.FairydewSplat_NS" (Transformation|GetWorldLocation (Variables|Default|GetResourceSprite)) "0, 0, 0" "1.000000,1.000000,1.000000" true true "AutoRelease")
    (Variables|Default|SetIsMoving false)
    (CallFunction|SetSpritebyState)
    (CallFunction|StopPhysics)))