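; Physics-driven dropped resource node that plays impact sounds, tracks whether it is moving, and can destroy itself once at rest.
; Hard self-moved hits play a random sound with volume scaled by impact strength.
; Physics sleep or a velocity threshold check updates IsMoving, and Tick counts down any positive post-stop lifespan while stopped.
; SetSpriteByState overrides the parent to show ready or not-ready moving sprites.
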(event OnComponentSleep(ResourceSprite)
  (params (SleepingComponent :type Primitive%20Component%20Object%20Reference) (BoneName :type Name :default "None"))
  (Variables|Default|SetIsMoving false)
  (CallFunction|OnStoppedFX))

(event OnComponentWake(ResourceSprite)
  (params (WakingComponent :type Primitive%20Component%20Object%20Reference) (BoneName :type Name :default "None"))
  (Sprite|SetSpriteColor (Variables|Default|GetResourceSprite) "(R=1.000000,G=1.000000,B=1.000000,A=1.000000)"))

(event Custom|OnStopTimerCheck
  (if (<= (Math|Vector|VectorLength (Transformation|GetVelocity)) (Variables|Default|GetStopVelocityThreshold))
    (Variables|Default|SetIsMoving false)
    (CallFunction|OnStoppedFX)
    (else
      (Variables|Default|SetIsMoving true))))

(event Custom|PlayHitSound
  (params (VolumePercent :type Float%20%28single-precision%29))
  (bind _onhitsounds (Variables|PhsxDropResourceNode|GetOnHitSounds))
  (bind _returnvalue (Utilities|Array|Length _onhitsounds))
  (bind _returnvalue_2 (- _returnvalue 1))
  (bind _returnvalue_3 (Math|Random|RandomIntegerinRange 0 _returnvalue_2))
  (bind _output (Utilities|Array|Get(acopy) _onhitsounds _returnvalue_3))
  (Utilities|IsValid _output
    (:Is%20Valid
      (Audio|PlaySoundatLocation _output (Transformation|GetWorldLocation (Variables|Default|GetResourceSprite)) "0, 0, 0" VolumePercent 1.0 0.0 0 0 0))))

(event EventBeginPlay
  (|CallParentFunction) ; This node is disabled and will not be called.\nDrag off pins to build functionality.
)

(event Collision|EventHit
  (params (MyComp :type Primitive%20Component%20Object%20Reference) (Other :type Actor%20Object%20Reference) (OtherComp :type Primitive%20Component%20Object%20Reference) (bSelfMoved :type Boolean) (HitLocation :type Vector :default "0, 0, 0") (HitNormal :type Vector :default "0, 0, 0") (NormalImpulse :type Vector :default "0, 0, 0") (Hit :type Hit%20Result%20Structure%20%28by%20ref%29))
  (bind _returnvalue (Math|Vector|VectorLength NormalImpulse))
  (if (and bSelfMoved (>= _returnvalue 4e+02))
    (CallFunction|OnHitFX _returnvalue)))

(event EventTick
  (params (DeltaSeconds :type Float%20%28single-precision%29))
  (if (and (> (Variables|Default|GetLifespanAfterStopped) 0.0) (not (Variables|Default|GetIsMoving)))
    (bind _output_get (Variables|Default|SetLifespanAfterStopped (- (Variables|Default|GetLifespanAfterStopped) DeltaSeconds)))
    (if (<= _output_get 0.0)
      (Actor|DestroyActor))))

(fn ConstructionScript
  (|CallParentFunction))

(fn OnHitFX
  (params (HitMagnitude :type Float%20%28single-precision%29))
  (CallFunction|PlayHitSound (Math|Float|MapRangeClamped HitMagnitude 5e+02 8e+03 0.1 1.0)))

(fn OnStoppedFX)

(fn SetSpritebyState
  (if (Variables|Default|GetIsMoving)
    (if (Variables|Default|GetReadyToHarvest)
      (Utilities|IsValid (Variables|Default|GetMovingReadySprite)
        (:Is%20Valid
          (Rendering|Components|Sprite|SetSprite (Variables|Default|GetResourceSprite) (Variables|Default|GetMovingReadySprite))))
      (else
        (Utilities|IsValid (Variables|Default|GetMovingNotReadySprite)
          (:Is%20Valid
            (Rendering|Components|Sprite|SetSprite (Variables|Default|GetResourceSprite) (Variables|Default|GetMovingNotReadySprite))))))
    (else
      (|CallParentFunction))))