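; ResourceNodeBase is a base Blueprint for clickable resource nodes that grant goods to the player.
; A click on its ResourceSprite runs HandleClick, which checks that the player controller is in a specific input mode with a FingerTool_BP-derived tool.
; If so, the controller drops goods sprinkles just offset from the cursor hit location, and the node's configured goods and quantity are added to the player inventory.
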(event OnClicked(ResourceSprite)
  (params (TouchedComponent :type Primitive%20Component%20Object%20Reference) (ButtonPressed :type Key%20Structure))
  (CallFunction|HandleClick))

(fn ConstructionScript)

(fn HandleClick
  (bind (_valid_ _inventory) (CallFunction|GetPlayerInventory))
  (bind _clickgoodsname (Variables|Default|GetClickGoodsName))
  (bind _clickgoodsquantity (Variables|Default|GetClickGoodsQuantity))
  (bind _goodsquantity (Utilities|Struct|MakeGoodsQuantity _clickgoodsname _clickgoodsquantity))
  (bind _asff_player_controller (Utilities|Casting|CastToFF_PlayerController (Game|GetPlayerController 0)))
  (bind _output_get (LocalVariables|SettmpPlayerController _asff_player_controller))
  (Utilities|IsValid (Variables|/Game/FungusFarm/Blueprints/FF_PlayerController.FF_PlayerController_C|GetCurrentTool _output_get)
    (:Is%20Valid
      (if (and (Utilities|Enum|Equal(Enum) (Variables|/Game/FungusFarm/Blueprints/FF_PlayerController.FF_PlayerController_C|GetInputMode _output_get) "NewEnumerator2") (Utilities|ClassIsChildOf (Utilities|GetClass (Variables|/Game/FungusFarm/Blueprints/FF_PlayerController.FF_PlayerController_C|GetCurrentTool _output_get)) "/Game/FungusFarm/Blueprints/Tools/FingerTool_BP.FingerTool_BP_C"))
        (Default|DropGoodsSprinkles (LocalVariables|GettmpPlayerController) (Utilities|Array|MakeArray _goodsquantity) (Math|Vector|MakeVector (.X (Math|Vector|BreakVector (.Location (Collision|BreakHitResult (.HitResult (Game|Player|GetHitResultUnderCursorbyChannel (LocalVariables|GettmpPlayerController) "TraceTypeQuery1" false)))))) (+ (.Y (Math|Vector|BreakVector (.Location (Collision|BreakHitResult (.HitResult (Game|Player|GetHitResultUnderCursorbyChannel (LocalVariables|GettmpPlayerController) "TraceTypeQuery1" false)))))) 2.0) (.Z (Math|Vector|BreakVector (.Location (Collision|BreakHitResult (.HitResult (Game|Player|GetHitResultUnderCursorbyChannel (LocalVariables|GettmpPlayerController) "TraceTypeQuery1" false))))))) 1e+01 1e+01)
        (if _valid_
          (Default|AddGoodsInventory _inventory _goodsquantity))))))