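; PhsxDropDropper is a resource-node spawner that repeatedly spawns a configured drop node class at random points within its SpawnBox bounds.
; A one-shot timer with a random min/max interval triggers each spawn and then re-arms itself, with a DoOnce guarding against double scheduling.
; Tick mirrors the timer's remaining time into NextSpawnSeconds, and scheduling reuses any positive value there instead of rolling a new delay.
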(event Custom|OnSpawnDropNode
  (bind _spawnbox (Variables|Default|GetSpawnBox))
  (bind (_origin _boxextent) (Collision|GetComponentBounds _spawnbox))
  (Game|SpawnActorfromClass (Variables|Default|GetDropNodeToSpawn) (Math|Transform|MakeTransform (Math|Random|RandomPointinBoundingBox _origin _boxextent) "0, 0, 0" (Variables|Default|GetOverrideSpawnScale)) "AdjustIfPossibleButAlwaysSpawn" 0 0)
  (Variables|Default|SetNextSpawnSeconds 0.0)
  (Utilities|FlowControl|Sequence
    (:then_0
      (Utilities|FlowControl|DoOnce false) ; enters at Reset
    )
    (:then_1
      (if (Utilities|Time|IsValidTimerHandle (Variables|Default|GetSpawnTimer))
        (Utilities|Time|ClearandInvalidateTimerbyHandle (Variables|Default|GetSpawnTimer)))
      (CallFunction|CheckSpawnTime))))

(event Custom|CheckSpawnTime
  (if (> (Variables|Default|GetSpawnIntervalMax) 0.0)
    (if (> (Variables|Default|GetNextSpawnSeconds) 0.0)
      _
      (else
        (Variables|Default|SetNextSpawnSeconds (Math|Random|RandomFloatinRange (Variables|Default|GetSpawnIntervalMin) (Variables|Default|GetSpawnIntervalMax)))))
    (Utilities|FlowControl|DoOnce false
      (:Completed
        (bind _returnvalue (Utilities|Time|SetTimerbyEvent (delegate Custom|OnSpawnDropNode) (Variables|Default|GetNextSpawnSeconds)))
        (Variables|Default|SetSpawnTimer _returnvalue)))))

(event EventBeginPlay
  (CallFunction|CheckSpawnTime))

(event EventTick
  (params (DeltaSeconds :type Float%20%28single-precision%29))
  (if (Utilities|Time|IsValidTimerHandle (Variables|Default|GetSpawnTimer))
    (Variables|Default|SetNextSpawnSeconds (Utilities|Time|GetTimerRemainingTimebyHandle (Variables|Default|GetSpawnTimer)))))

(fn ConstructionScript)