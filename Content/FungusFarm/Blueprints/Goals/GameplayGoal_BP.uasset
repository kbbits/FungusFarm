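; Gameplay goal Blueprint for FungusFarm that wraps GoalData and grants the goal's rewards on completion.
; ApplyCompletedAwards unlocks recipes, crops and tools on the game state, then returns all awards, leaving goods for the caller to grant.
; Dot-delimited "GoalProvider.Start.<Name>" award strings create secondary goal providers through FFGameMode and register them with the player's goals manager, chaining new goals.
; Serialization events are empty stubs.
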(event Custom|RefreshFromSerialized)

(event Custom|SaveToSerialized)

(fn ApplyCompletedAwards
  (params (Game%20State :type FF%20Game%20State%20Object%20Reference) (PlayerController :type FF%20Player%20Controller%20BP%20Object%20Reference))
  (bind _goal_data (Variables|Default|GetGoal%20Data))
  (bind (_uniquename _displayname _onavailablemessage _completedmessage _hidden _canabandon _canrepeat _announced _prerequisitegoals _harvestedgoodstocomplete _soldgoodstocomplete _donatedgoodstocomplete _craftedrecipestocomplete _harvestedgoodsprogress _soldgoodsprogress _donatedgoodsprogress _craftedrecipesprogress _unlockedcraftingrecipes _unlockedcrops _unlockedtools _otherawards _goodsawarded) (Utilities|Struct|BreakGameplayGoal _goal_data))
  (LocalVariables|SettmpGameState Game%20State)
  (LocalVariables|SettmpPlayerController PlayerController)
  (Utilities|FlowControl|Sequence
    (:then_0
      (bind _output_get (LocalVariables|SettmpUnlockedRecipes _unlockedcraftingrecipes))
      (for _array_element _output_get
        (Default|UnlockRecipe (LocalVariables|GettmpGameState) _array_element)))
    (:then_1
      (bind _output_get_2 (LocalVariables|SettmpUnlockedCrops _unlockedcrops))
      (for _array_element_2 _output_get_2
        (Default|UnlockCrop (LocalVariables|GettmpGameState) _array_element_2)))
    (:then_2
      (bind _output_get_3 (LocalVariables|SettmpUnlockedTools _unlockedtools))
      (for _array_element_3 _output_get_3
        (Default|UnlockTool (LocalVariables|GettmpGameState) _array_element_3)))
    (:then_3
      (LocalVariables|SettmpGoodsAwarded _goodsawarded))
    (:then_4
      (bind _output_get_4 (LocalVariables|SettmpOtherAwards _otherawards))
      (for _array_element_4 _output_get_4
        (LocalVariables|SettmpParsedGoalString (Utilities|String|ParseIntoArray (Utilities|String|ToString(Name) _array_element_4) "."))
        (if (== (Utilities|Array|Length (LocalVariables|GettmpParsedGoalString)) 3)
          (if (Utilities|String|StartsWith (Utilities|Array|Get(acopy) (LocalVariables|GettmpParsedGoalString)) "goalprovider")
            (if (Utilities|String|StartsWith (Utilities|Array|Get(acopy) (LocalVariables|GettmpParsedGoalString) 1) "start")
              (bind _asffgame_mode (Utilities|Casting|CastToFFGameMode (Variables|/Script/Engine.GameStateBase|GetAuthorityGameMode (LocalVariables|GettmpGameState))))
              (bind _returnvalue (Class|FFGameMode|AddSecondaryGoalProvider _asffgame_mode (Utilities|String|StringToName (Utilities|Array|Get(acopy) (LocalVariables|GettmpParsedGoalString) 2))))
              (Utilities|IsValid _returnvalue
                (:Is%20Valid
                  (Class|ActorGoalsComponent|AddGoalProvider (Variables|/Script/FungusFarm.FFPlayerControllerBase|GetGameplayGoalsManager (LocalVariables|GettmpPlayerController)) _returnvalue))))))))
    (:then_5
      (return (LocalVariables|GettmpUnlockedRecipes) (LocalVariables|GettmpUnlockedCrops) (LocalVariables|GettmpUnlockedTools) (LocalVariables|GettmpOtherAwards) (LocalVariables|GettmpGoodsAwarded)))))

(fn GetUniqueName
  (return (.UniqueName (Utilities|Struct|BreakGameplayGoal (Variables|Default|GetGoal%20Data)))))

(fn IsHidden
  (return (.Hidden (Utilities|Struct|BreakGameplayGoal (Variables|Default|GetGoal%20Data)))))