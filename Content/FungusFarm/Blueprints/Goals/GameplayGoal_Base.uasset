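; Base gameplay goal for the farming game, driven by GoalData, that tracks progress toward completion and provides rewards.
; Update functions tally harvested goods, sold goods and crafted recipes in maps, though crafting progress is seeded from harvest requirement names.
; The completion check stops at the first shortfall and returns remaining harvest and crafting amounts, but not sales.
; Completion unlocks recipes and crops on GameState and returns goods for the caller to award.
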(fn OnGoalCompleted
  (params (Game%20State :type FF%20Game%20State%20Object%20Reference))
  (bind _goal_data (Variables|Default|GetGoal%20Data))
  (bind (_uniquename _displayname _onavailablemessage _completedmessage _hidden _prerequisitegoals _harvestedgoodstocomplete _soldgoodstocomplete _craftedrecipestocomplete _unlockedcraftingrecipes _unlockedcrops _unlockedtools _otherawards _goodsawarded) (Utilities|Struct|BreakGameplayGoal _goal_data))
  (Utilities|FlowControl|Sequence
    (:then_0
      (for _array_element _unlockedcraftingrecipes
        (Default|UnlockRecipe Game%20State _array_element)))
    (:then_1
      (for _array_element_2 _unlockedcrops
        (Default|UnlockCrop Game%20State _array_element_2)))
    (:then_2
      (LocalVariables|SettmpGoodsAwarded _goodsawarded)
      (return _unlockedcraftingrecipes _unlockedcrops (LocalVariables|GettmpGoodsAwarded)))))

(fn CheckGoalQualifiesCompleted
  (params (Game%20State :type FF%20Game%20State%20Object%20Reference) (Player%20Controller :type FF%20Player%20Controller%20Object%20Reference))
  (bind _goal_data (Variables|Default|GetGoal%20Data))
  (bind (_uniquename _displayname _onavailablemessage _completedmessage _hidden _prerequisitegoals _harvestedgoodstocomplete _soldgoodstocomplete _craftedrecipestocomplete) (Utilities|Struct|BreakGameplayGoal _goal_data))
  (LocalVariables|SettmpGameState Game%20State)
  (LocalVariables|SettmpPlayerController Player%20Controller)
  (Utilities|FlowControl|Sequence
    (:then_0
      ;[1 1 1] Check harvest totals
      (bind _array_element (Utilities|Array|ForEachLoopwithBreak _harvestedgoodstocomplete :!label _label)
        (:LoopBody
          (if (not (>= (.Value (Utilities|Map|Find (Variables|Default|GetHarvestedProgress) (.Name (Utilities|Struct|BreakGoodsQuantity _array_element)))) (.Quantity (Utilities|Struct|BreakGoodsQuantity _array_element))))
            (Utilities|Map|Add (LocalVariables|GettmpRemainingHarvest) (.Name (Utilities|Struct|BreakGoodsQuantity _array_element)) (+ (.Value (Utilities|Map|Find (LocalVariables|GettmpRemainingHarvest) (.Name (Utilities|Struct|BreakGoodsQuantity _array_element)))) (- (.Quantity (Utilities|Struct|BreakGoodsQuantity _array_element)) (.Value (Utilities|Map|Find (Variables|Default|GetHarvestedProgress) (.Name (Utilities|Struct|BreakGoodsQuantity _array_element)))))))
            (LocalVariables|SettmpQualifiesComplete false)
            (goto _label Break)))))
    (:then_1
      ;[1 1 1] Check Sold Goods
      (if (LocalVariables|GettmpQualifiesComplete)
        (bind _array_element_2 (Utilities|Array|ForEachLoopwithBreak _soldgoodstocomplete :!label _label_2)
          (:LoopBody
            (if (not (>= (.Value (Utilities|Map|Find (Variables|Default|GetSoldGoodsProgress) (.Name (Utilities|Struct|BreakGoodsQuantity _array_element_2)))) (.Quantity (Utilities|Struct|BreakGoodsQuantity _array_element_2))))
              (Utilities|Map|Add (LocalVariables|GettmpRemainingSoldGoods) (.Name (Utilities|Struct|BreakGoodsQuantity _array_element_2)) (+ (.Value (Utilities|Map|Find (LocalVariables|GettmpRemainingSoldGoods) (.Name (Utilities|Struct|BreakGoodsQuantity _array_element_2)))) (- (.Quantity (Utilities|Struct|BreakGoodsQuantity _array_element_2)) (.Value (Utilities|Map|Find (Variables|Default|GetSoldGoodsProgress) (.Name (Utilities|Struct|BreakGoodsQuantity _array_element_2)))))))
              (LocalVariables|SettmpQualifiesComplete false)
              (goto _label_2 Break))))))
    (:then_2
      ;[1 1 1] Check recipe crafting
      (if (LocalVariables|GettmpQualifiesComplete)
        (bind _keys (Utilities|Map|Keys _craftedrecipestocomplete))
        (bind _array_element_3 (Utilities|Array|ForEachLoopwithBreak _keys :!label _label_3)
          (:LoopBody
            (if (> (Math|Conversions|ToFloat(Integer) (.Value (Utilities|Map|Find _craftedrecipestocomplete _array_element_3))) (.Value (Utilities|Map|Find (Variables|Default|GetCraftedRecipesProgress) _array_element_3)))
              (Utilities|Map|Add (LocalVariables|GettmpRemainingRecipeCraftings) _array_element_3 (+ (- (.Value (Utilities|Map|Find _craftedrecipestocomplete _array_element_3)) (Math|Float|Truncate (.Value (Utilities|Map|Find (Variables|Default|GetCraftedRecipesProgress) _array_element_3)))) (.Value (Utilities|Map|Find (LocalVariables|GettmpRemainingRecipeCraftings) _array_element_3))))
              (LocalVariables|SettmpQualifiesComplete false)
              (goto _label_3 Break))))))
    (:then_3
      (return (LocalVariables|GettmpQualifiesComplete) (LocalVariables|GettmpRemainingHarvest) (LocalVariables|GettmpRemainingRecipeCraftings)))))

(fn GetUniqueName
  (return (.UniqueName (Utilities|Struct|BreakGameplayGoal (Variables|Default|GetGoal%20Data)))))

(fn UpdateHarvestedGoodsProgress
  (params (GoodsHarvested :type Array%20of%20Goods%20Quantity%20Structures))
  (bind _goal_data (Variables|Default|GetGoal%20Data))
  (bind _harvestedgoodstocomplete (Utilities|Struct|BreakGameplayGoal _goal_data))
  (if (> (Utilities|Array|Length _harvestedgoodstocomplete) 0)
    (if (== (Utilities|Map|Length (Variables|Default|GetHarvestedProgress)) 0)
      (for _array_element _harvestedgoodstocomplete
        (Utilities|Map|Add (Variables|Default|GetHarvestedProgress) (.Name (Utilities|Struct|BreakGoodsQuantity _array_element)) 0.0)))
    (for _array_element_2 GoodsHarvested
      (if (.ReturnValue (Utilities|Map|Find (Variables|Default|GetHarvestedProgress) (.Name (Utilities|Struct|BreakGoodsQuantity _array_element_2))))
        (Utilities|Map|Add (Variables|Default|GetHarvestedProgress) (.Name (Utilities|Struct|BreakGoodsQuantity _array_element_2)) (+ (.Value (Utilities|Map|Find (Variables|Default|GetHarvestedProgress) (.Name (Utilities|Struct|BreakGoodsQuantity _array_element_2)))) (.Quantity (Utilities|Struct|BreakGoodsQuantity _array_element_2))))))))

(fn UpdateSoldGoodsProgress
  (params (SoldGoods :type Array%20of%20Goods%20Quantity%20Structures))
  (bind _goal_data (Variables|Default|GetGoal%20Data))
  (bind _soldgoodstocomplete (Utilities|Struct|BreakGameplayGoal _goal_data))
  (if (> (Utilities|Array|Length _soldgoodstocomplete) 0)
    (if (== (Utilities|Map|Length (Variables|Default|GetSoldGoodsProgress)) 0)
      (for _array_element _soldgoodstocomplete
        (Utilities|Map|Add (Variables|Default|GetSoldGoodsProgress) (.Name (Utilities|Struct|BreakGoodsQuantity _array_element)) 0.0)))
    (for _array_element_2 SoldGoods
      (if (.ReturnValue (Utilities|Map|Find (Variables|Default|GetSoldGoodsProgress) (.Name (Utilities|Struct|BreakGoodsQuantity _array_element_2))))
        (Utilities|Map|Add (Variables|Default|GetSoldGoodsProgress) (.Name (Utilities|Struct|BreakGoodsQuantity _array_element_2)) (+ (.Value (Utilities|Map|Find (Variables|Default|GetSoldGoodsProgress) (.Name (Utilities|Struct|BreakGoodsQuantity _array_element_2)))) (.Quantity (Utilities|Struct|BreakGoodsQuantity _array_element_2))))))))

(fn UpdateCraftedRecipesProgress
  (params (CraftedRecipe :type Name))
  (bind _goal_data (Variables|Default|GetGoal%20Data))
  (bind _craftedrecipesprogress (Variables|Default|GetCraftedRecipesProgress))
  (bind (_uniquename _displayname _onavailablemessage _completedmessage _hidden _prerequisitegoals _harvestedgoodstocomplete _soldgoodstocomplete _craftedrecipestocomplete) (Utilities|Struct|BreakGameplayGoal _goal_data))
  (bind (_value _returnvalue) (Utilities|Map|Find _craftedrecipesprogress CraftedRecipe))
  (if (> (Utilities|Map|Length _craftedrecipestocomplete) 0)
    (if (== (Utilities|Map|Length (Variables|Default|GetCraftedRecipesProgress)) 0)
      (for _array_element _harvestedgoodstocomplete
        (Utilities|Map|Add (Variables|Default|GetCraftedRecipesProgress) (.Name (Utilities|Struct|BreakGoodsQuantity _array_element)) 0.0)))
    (if _returnvalue
      (Utilities|Map|Add (Variables|Default|GetCraftedRecipesProgress) CraftedRecipe (+ _value 1.0)))))

(fn IsHidden
  (return (.Hidden (Utilities|Struct|BreakGameplayGoal (Variables|Default|GetGoal%20Data)))))