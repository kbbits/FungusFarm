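; Goal giver Blueprint that supplies gameplay goals to the player through its GoalGiverProvider.
; Shortly after BeginPlay it registers that provider with the GameplayGoalsManager on the first player's FF_PlayerController_BP.
; A one-shot timer set by DelayBeforeStart then clears the provider's DisableNewGoals flag and prints its friendly name and GUID for debugging.
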(event Custom|EnableGoals
  (bind _goalgiverprovider (Variables|Default|GetGoalGiverProvider))
  (Variables|/Script/FungusFarm.GoalsProviderComponent|SetbDisableNewGoals _goalgiverprovider false)
  (bind _returnvalue (Class|GameplayGoalProvider|GetGameplayGoalProviderFriendlyName _goalgiverprovider))
  (bind _returnvalue_2 (Class|GameplayGoalProvider|GetGameplayGoalProviderGuid _goalgiverprovider))
  (Development|PrintString (Utilities|String|Append "Enabling provider  " _returnvalue " GUID " (Guid|ToString(Guid) _returnvalue_2))))

(event EventBeginPlay
  (Utilities|FlowControl|Delay 0.5)
  (bind _asff_player_controller_bp (Utilities|Casting|CastToFF_PlayerController_BP (Game|GetPlayerController 0)))
  (Class|ActorGoalsComponent|AddGoalProvider (Variables|/Script/FungusFarm.FFPlayerControllerBase|GetGameplayGoalsManager _asff_player_controller_bp) (Variables|Default|GetGoalGiverProvider))
  (Utilities|Time|SetTimerbyEvent (delegate Custom|EnableGoals) (Variables|Default|GetDelayBeforeStart)))

(fn ConstructionScript)