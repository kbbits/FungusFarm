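; FF_NormalGameMode is Fungus Farm's normal game mode, which works out which gameplay goals are available given the completed ones.
; GetAvailableGameplayGoals scans the GameplayGoals data table, skipping completed goals and any with unmet prerequisites.
; Each remaining row is wrapped in a newly constructed GameplayGoal_Base object, outered to the game state, and returned in an array.
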(fn ConstructionScript)

(fn GetAvailableGameplayGoals
  (params (Completed%20Goals :type Array%20of%20Names))
  (Utilities|FlowControl|Sequence
    (:then_0
      (LocalVariables|SettmpAvailableGoals (Utilities|Array|MakeArray)))
    (:then_1
      (bind _outrownames (DataTable|GetDataTableRowNames (Variables|Default|GetGameplay%20Goals)))
      (for _array_element _outrownames
        (bind _returnvalue (Utilities|GetDataTableRow (Variables|Default|GetGameplay%20Goals) _array_element)
          (:then
            (if (not (Utilities|Array|ContainsItem Completed%20Goals (.Name (Utilities|Struct|BreakGameplayGoal _returnvalue))))
              (LocalVariables|SettmpHasPreReqs true)
              (bind _array_element_2 (Utilities|Array|ForEachLoopwithBreak (.PrerequisiteGoals (Utilities|Struct|BreakGameplayGoal _returnvalue)) :!label _label)
                (:LoopBody
                  (if (not (Utilities|Array|ContainsItem Completed%20Goals _array_element_2))
                    (LocalVariables|SettmpHasPreReqs false)
                    (goto _label Break)))
                (:Completed
                  (if (LocalVariables|GettmpHasPreReqs)
                    (bind _returnvalue_2 (Game|ConstructObjectfromClass "/Game/FungusFarm/Blueprints/Goals/GameplayGoal_Base.GameplayGoal_Base_C" (Game|GetGameState) (|Copy _returnvalue)))
                    (Utilities|Array|Add (LocalVariables|GettmpAvailableGoals) _returnvalue_2)))))))))
    (:then_2
      (return (LocalVariables|GettmpAvailableGoals)))))