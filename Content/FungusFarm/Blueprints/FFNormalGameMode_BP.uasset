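; Game mode Blueprint for FungusFarm holding draft logic for gameplay goals; both function entries are unwired, so none of it runs.
; RandomGoalTmp's disconnected nodes build a sell goal from an unlocked recipe by RecipeBias roll, otherwise a crop harvest goal, both awarding SoulPearls.
; NewGoalTmp's disconnected nodes select GameplayGoals table rows that aren't already active and whose prerequisite goals are completed.
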(fn ConstructionScript
  (|CallParentFunction))

(fn RandomGoalTmp
  (params (MinTier :type Integer) (MaxTier :type Integer)))

(fn NewGoalTmp
  (params (CurrentGoals :type Array%20of%20Gameplay%20Goal%20Structures) (CompletedGoals :type Array%20of%20Names)))