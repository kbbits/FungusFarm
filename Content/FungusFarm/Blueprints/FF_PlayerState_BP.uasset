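; Player state Blueprint for Fungus Farm that tracks the player's tools, recipe unlocks and a god mode flag.
; On BeginPlay and on unlock, tool codes resolve through a name-to-class map into cached tool objects, one per class, and the player controller is notified.
; Tool lookup can construct uncached tools on request.
; An optional test flag unlocks every recipe from the game state.
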(event EventBeginPlay
  (Tools|InitAvailableTools))

(event EventUnlockTool
  (params (ToolName :type Name :default "None"))
  (|CallParentFunction ToolName)
  (Tools|AddTool ToolName))

(fn ConstructionScript)

(fn UnlockDefaultRecipes
  (params (UnlockTestRecipes :type Boolean))
  (if UnlockTestRecipes
    (bind _asff_game_state (Utilities|Casting|CastToFF_GameState (Game|GetGameState)))
    (bind _all_recipes (Default|GetAllRecipes _asff_game_state))
    (for _array_element _all_recipes
      (Class|FFPlayerState|UnlockRecipe (.Name (Utilities|Struct|BreakCraftingRecipe _array_element))))))

(fn GodMode?
  (return (Variables|Default|GetGodMode)))

(fn SetGodMode
  (params (GodMode :type Boolean))
  (Variables|Default|SetGodMode GodMode))

(fn GetAvailableTools
  (return (Variables|Default|GetAvailableToolsCache)))

(fn InitAvailableTools
  (Utilities|Array|Clear (Variables|Default|GetAvailableToolsCache))
  (for _array_element (Variables|Default|GetUnlockedTools)
    (Tools|AddTool _array_element))
  (return (Variables|Default|GetAvailableToolsCache)))

(fn AddTool
  (params (ToolCode :type Name%20%28by%20ref%29))
  (bind _toolnameclassmap (Variables|Default|GetToolNameClassMap))
  (bind (_value _returnvalue) (Utilities|Map|Find _toolnameclassmap ToolCode))
  (if _returnvalue
    (bind _array_element (Utilities|Array|ForEachLoopwithBreak (Variables|Default|GetAvailableToolsCache))
      (:LoopBody
        (Utilities|IsValid _array_element
          (:Is%20Valid
            (if (== (Utilities|GetClass _array_element) _value)
              (return)))))
      (:Completed
        (bind _returnvalue_2 (Game|ConstructObjectfromClass _value self))
        (Utilities|Array|Add (Variables|Default|GetAvailableToolsCache) _returnvalue_2)
        (bind _asff_player_controller_bp (Utilities|Casting|CastToFF_PlayerController_BP (Game|GetPlayerController 0)))
        (Default|OnToolsChanged _asff_player_controller_bp)))))

(fn GetToolbyCode
  (params (ToolCode :type Name) (IncludeUnavailableTools :type Boolean))
  (bind _toolnameclassmap (Variables|Default|GetToolNameClassMap))
  (bind (_value _returnvalue) (Utilities|Map|Find _toolnameclassmap ToolCode))
  (if (Utilities|Name|NotEqual(Name) ToolCode "None")
    (bind _array_element (Utilities|Array|ForEachLoopwithBreak (Variables|Default|GetAvailableToolsCache) :!label _label)
      (:LoopBody
        (if (Utilities|Name|Equal(Name) (Variables|/Game/FungusFarm/Blueprints/Tools/ToolBase_BP.ToolBase_BP_C|GetTool%20Code _array_element) ToolCode)
          (LocalVariables|SettmpTool _array_element)
          (goto _label Break)))
      (:Completed
        (if (not (Utilities|IsValid (LocalVariables|GettmpTool)))
          (if IncludeUnavailableTools
            (if _returnvalue
              (bind _returnvalue_2 (Game|ConstructObjectfromClass _value self))
              (LocalVariables|SettmpTool _returnvalue_2)
              (return (LocalVariables|GettmpTool))
              (else
                _))))
        (return (LocalVariables|GettmpTool))))
    (else
      (return (LocalVariables|GettmpTool)))))