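; Inventory component that stores goods as a name-to-quantity map, with functions to add, remove, query and transfer them.
; Adds and successful removals call a goods delta notification with the change and the current quantity.
; Batch removal uses an in-use flag and checks every item's quantity before removing any.
; Transfers to another inventory, of given goods or the whole contents, add to the receiver only after removal here succeeds.
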(fn AddGoodsInventory
  (params (Goods :type Goods%20Quantity%20Structure))
  (bind _name (Utilities|Struct|BreakGoodsQuantity Goods))
  (bind (_name_2 _quantity) (Utilities|Struct|BreakGoodsQuantity Goods))
  (Utilities|FlowControl|Sequence
    (:then_0
      (Utilities|Map|Add (Variables|Default|GetGoodsInventory) _name_2 (select (Utilities|Map|Contains (Variables|Default|GetGoodsInventory) _name_2) (+ (.Value (Utilities|Map|Find (Variables|Default|GetGoodsInventory) _name_2)) _quantity) _quantity)))
    (:then_1
      (Default|CallOnGoodsInventoryDelta Goods (Utilities|Struct|MakeGoodsQuantity _name (CallFunction|GetGoodsInventoryQuantity _name))))))

(fn AddGoodsInventoryBatch
  (params (Goods :type Array%20of%20Goods%20Quantity%20Structures))
  (for _array_element Goods
    (CallFunction|AddGoodsInventory _array_element)))

(fn RemoveGoodsInventory!
  (params (GoodsToRemove :type Goods%20Quantity%20Structure))
  (bind (_name _quantity) (Utilities|Struct|BreakGoodsQuantity GoodsToRemove))
  (Utilities|Map|Add (Variables|Default|GetGoodsInventory) _name (- (.Value (Utilities|Map|Find (Variables|Default|GetGoodsInventory) _name)) _quantity)))

(fn RemoveGoodsInventory
  (params (GoodsToRemove :type Goods%20Quantity%20Structure))
  (bind (_name _quantity) (Utilities|Struct|BreakGoodsQuantity GoodsToRemove))
  (bind (_successful _quantityremaining) (CallFunction|NameFloatMapRemoveQuantity (Variables|Default|GetGoodsInventory) _name _quantity))
  (if _successful
    (Default|CallOnGoodsInventoryDelta (Utilities|Struct|MakeGoodsQuantity _name (* _quantity -1.0)) (Utilities|Struct|MakeGoodsQuantity _name _quantityremaining))
    (return true)
    (else
      (return false))))

(fn RemoveGoodsInventoryBatch
  (params (GoodsToRemove :type Array%20of%20Goods%20Quantity%20Structures))
  (if (Variables|Default|GetInventoryInUse)
    (return false true)
    (else
      (Variables|Default|SetInventoryInUse true)
      (bind _array_element (Utilities|Array|ForEachLoopwithBreak GoodsToRemove :!label _label)
        (:LoopBody
          (bind _hasall (CallFunction|NameFloatMapHasQuantity? (Variables|Default|GetGoodsInventory) (.Name (Utilities|Struct|BreakGoodsQuantity _array_element)) (.Quantity (Utilities|Struct|BreakGoodsQuantity _array_element))))
          (if (not _hasall)
            (LocalVariables|SettmpHasAllInventory false)
            (goto _label Break)))
        (:Completed
          (if (LocalVariables|GettmpHasAllInventory)
            (for _array_element_2 GoodsToRemove
              (CallFunction|RemoveGoodsInventory! _array_element_2)
              (Default|CallOnGoodsInventoryDelta (Utilities|Struct|MakeGoodsQuantity (.Name (Utilities|Struct|BreakGoodsQuantity _array_element_2)) (* (.Quantity (Utilities|Struct|BreakGoodsQuantity _array_element_2)) -1.0)) (Utilities|Struct|MakeGoodsQuantity (.Name (Utilities|Struct|BreakGoodsQuantity _array_element_2)) (CallFunction|GetGoodsInventoryQuantity (.Name (Utilities|Struct|BreakGoodsQuantity _array_element_2)))))))
          (Variables|Default|SetInventoryInUse false)
          (return (LocalVariables|GettmpHasAllInventory) false))))))

(fn GetGoodsInventoryQuantity
  (params (GoodsName :type Name))
  (bind _goodsinventory (Variables|Default|GetGoodsInventory))
  (bind (_value _returnvalue) (Utilities|Map|Find _goodsinventory GoodsName))
  (return (select _returnvalue _value 0.0)))

(fn HasGoods?
  (params (RequiredGoods :type Goods%20Quantity%20Structure))
  (bind (_name _quantity) (Utilities|Struct|BreakGoodsQuantity RequiredGoods))
  (bind _hasall (CallFunction|NameFloatMapHasQuantity? (Variables|Default|GetGoodsInventory) _name _quantity))
  (return _hasall))

(fn HasAllGoods?
  (params (RequiredGoods :type Array%20of%20Goods%20Quantity%20Structures))
  (if (> (Utilities|Array|Length RequiredGoods) 0)
    (for _array_element RequiredGoods
      (Utilities|Map|Add (LocalVariables|GettmpRequiredGoodsMap) (.Name (Utilities|Struct|BreakGoodsQuantity _array_element)) (.Quantity (Utilities|Struct|BreakGoodsQuantity _array_element))))
    (bind _has_all (CallFunction|NameFloatMapHasAll? (Variables|Default|GetGoodsInventory) (LocalVariables|GettmpRequiredGoodsMap)))
    (return _has_all)
    (else
      (return true))))

(fn GetAllInventoryasMap
  (bind _keys (Utilities|Map|Keys (Variables|Default|GetGoodsInventory)))
  (for _array_element _keys
    (Utilities|Map|Add (LocalVariables|GettmpInventory) _array_element (.Value (Utilities|Map|Find (Variables|Default|GetGoodsInventory) _array_element))))
  (return (LocalVariables|GettmpInventory)))

(fn TransferGoodstoOther
  (params (ReceivingInventory :type FF%20Goods%20Inventory%20Component%20Object%20Reference%20%28by%20ref%29) (GoodsToTransfer :type Goods%20Quantity%20Structure%20%28by%20ref%29))
  (Utilities|IsValid ReceivingInventory
    (:Is%20Valid
      (LocalVariables|SettmpRecievingInventory ReceivingInventory)
      (bind _output_get (LocalVariables|SettmpTransferringGoods GoodsToTransfer))
      (bind _successful (CallFunction|RemoveGoodsInventory _output_get))
      (if _successful
        (CallFunction|AddGoodsInventory (LocalVariables|GettmpRecievingInventory) (LocalVariables|GettmpTransferringGoods))
        (return true)))
    (:Is%20Not%20Valid
      (return false))))

(fn IsEmpty?
  (return (== (Utilities|Map|Length (Variables|Default|GetGoodsInventory)) 0)))

(fn TransferAllGoodstoOther
  (params (ReceivingInventory :type FF%20Goods%20Inventory%20Component%20Object%20Reference%20%28by%20ref%29))
  (LocalVariables|SettmpRecievingInventory ReceivingInventory)
  (Utilities|FlowControl|Sequence
    (:then_0
      (bind _goods_array (CallFunction|GoodsMaptoArray (Variables|Default|GetGoodsInventory)))
      (bind _output_get (LocalVariables|SettmpTransferringGoods _goods_array))
      (bind _successful (CallFunction|RemoveGoodsInventoryBatch _output_get))
      (if _successful
        (CallFunction|AddGoodsInventoryBatch (LocalVariables|GettmpRecievingInventory) (LocalVariables|GettmpTransferringGoods))
        (LocalVariables|SettmpSuccessful true)))
    (:then_1
      (return (LocalVariables|GettmpSuccessful)))))