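; Game state for the mushroom farming game, serving as the hub for game data, unlocks, progress totals, pausing and slot-based save/load.
; On BeginPlay it pauses, builds unlocked tool objects, async-loads data table thumbnails against a counter and finds the farm manager.
; Lookup functions expose crop, recipe, goods, equipment and plot tables, plus the market inventory.
; Harvest, sale and monitored-crafter events accumulate totals that update the player controller's GameplayGoalsManager.
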(event Resume(SaveExtentionLifetime)
  ;[1 1 1] Save Load
  (CallFunction|RefreshFarmManager))

(event Custom|LoadAssetsInData
  ;[1 1 1] Asset Loading
  (Utilities|FlowControl|Sequence
    (:then_0
      (Variables|Default|SetTotalAssetsToLoad 0)
      (for _array_element (Utilities|Array|MakeArray (Variables|Default|GetCropData) (Variables|Default|GetCraftingRecipeData) (Variables|Default|GetGoodsData) (Variables|Default|GetEquipmentData))
        (bind _outrownames (DataTable|GetDataTableRowNames _array_element))
        (Variables|Default|SetTotalAssetsToLoad (+ (Variables|Default|GetTotalAssetsToLoad) (Utilities|Array|Length _outrownames)))))
    (:then_1
      (bind _all_crops (Crops|GetAllCropData))
      (for _array_element_2 _all_crops
        (Utilities|AsyncLoadAsset (.Thumbnail (Utilities|Struct|BreakCropType _array_element_2))
          (:Completed
            (CallFunction|AssetLoaded)))))
    (:then_2
      (bind _all_recipes (CraftingRecipes|GetAllRecipes))
      (for _array_element_3 _all_recipes
        (Utilities|AsyncLoadAsset (.Thumbnail (Utilities|Struct|BreakCraftingRecipe _array_element_3))
          (:Completed
            (CallFunction|AssetLoaded)))))
    (:then_3
      (bind _goods (CallFunction|GetAllGoods))
      (for _array_element_4 _goods
        (Utilities|AsyncLoadAsset (.Thumbnail (Utilities|Struct|BreakGoodsType _array_element_4))
          (:Completed
            (CallFunction|AssetLoaded)))))
    (:then_4
      (bind _equipment (CallFunction|GetAllEquipmentData))
      (for _array_element_5 _equipment
        (Utilities|AsyncLoadAsset (.Thumbnail (Utilities|Struct|BreakEquipmentType _array_element_5))
          (:Completed
            (CallFunction|AssetLoaded)))))))

(event Custom|BindToMonitoredCrafter
  (params (Crafter :type FF%20Actor%20Crafter%20Component%20Object%20Reference))
  ;[1 1 1] Tracking Crafting
  (EventDispatchers|BindEventtoOnCraftComplete Crafter (delegate Custom|OnCrafterItemComplete)))

(event Custom|UnbindMonitoredCrafter
  (params (Crafter :type FF%20Actor%20Crafter%20Component%20Object%20Reference))
  ;[1 1 1] Tracking Crafting
  (Utilities|IsValid Crafter
    (:Is%20Valid
      (EventDispatchers|UnbindEventfromOnCraftComplete Crafter (delegate Custom|OnCrafterItemComplete)))))

(event Custom|QuitGame
  ;[1 1 1] Quit Game
  (Game|QuitGame 0 "Quit" false))

(event Custom|OnCrafterItemComplete
  (params (Completed%20Recipe :type Crafting%20Recipe%20Structure) (Produced%20Goods :type Array%20of%20Goods%20Quantity%20Structures))
  ;[1 1 1] Tracking Crafting
  (TrackingandGoals|TrackCraftedRecipes Completed%20Recipe Produced%20Goods))

(event Custom|AssetLoaded
  ;[1 1 1] Asset Loading
  (Math|Integer|IncrementInt (Variables|Default|GetTotalAssetsLoaded)
    (:%20%20
      (if (== (Variables|Default|GetTotalAssetsToLoad) (Variables|Default|GetTotalAssetsLoaded))
        (CallFunction|OnAssetsLoaded)))))

(event Custom|SaveGame
  ;[1 1 1] Save Load
  (CallFunction|Pause)
  (Development|PrintString (Utilities|String|BuildString(Integer) "" "Saving slot: " (Variables|Default|GetCurrentSaveSlot)) false true "(R=0.000000,G=0.660000,B=1.000000,A=1.000000)" 5.0)
  (Utilities|IsValid (Class|SaveManager|GetCurrentInfo (Subsystems|GetSaveManager))
    (:Is%20Valid
      (Class|SaveManager|SetActivePreset (Subsystems|GetSaveManager) (Variables|Default|GetSavePreset))
      (Class|SaveManager|BPSaveSlottoId (Subsystems|GetSaveManager) (Variables|Default|GetCurrentSaveSlot) true (Utilities|Struct|MakeScreenshotSize 640 360) true
        (:Continue
          (Development|PrintString "Save Successful" true true "(R=0.000000,G=0.660000,B=1.000000,A=1.000000)" 5.0))
        (:Failed
          (Development|PrintString "Save Failed" true true "(R=1.000000,G=0.008024,B=0.000000,A=1.000000)" 5.0))))
    (:Is%20Not%20Valid
      (Development|PrintString "Slot Invalid" true true "(R=0.000000,G=0.660000,B=1.000000,A=1.000000)" 5.0))))

(event Custom|LoadGame
  ;[1 1 1] Save Load
  (Utilities|FlowControl|Sequence
    (:then_0
      (CallFunction|Pause))
    (:then_1
      (Class|SaveManager|BPReloadCurrentSlot (Subsystems|GetSaveManager)
        (:Continue
          (Development|PrintString "Load Successful" true true "(R=0.000000,G=0.660000,B=1.000000,A=1.000000)" 5.0))
        (:Failed
          (Development|PrintString "Load Failed" true true "(R=1.000000,G=0.008024,B=0.000000,A=1.000000)" 5.0))))))

(event Custom|OnAssetsLoaded
  ;[1 1 1] Asset Loading
  (Development|PrintString (Utilities|String|Append "LOADED: " (Utilities|String|ToString(Integer) (Variables|Default|GetTotalAssetsLoaded)) " of " (Utilities|String|ToString(Integer) (Variables|Default|GetTotalAssetsToLoad))) true true "(R=0.010323,G=1.000000,B=0.000000,A=1.000000)" 4.0)
  (Utilities|Casting|CastToFFGameMode_BP (Game|GetGameMode)))

(event EventBeginPlay
  ;[1 1 1] Begin Play
  (CallFunction|Pause)
  (bind _asff_platform_game_instance (Utilities|Casting|CastToFF_PlatformGameInstance (Game|GetGameInstance)))
  (Variables|Default|SetFF_GameInstance _asff_platform_game_instance)
  (PlayerTools|LoadInitTools)
  (CallFunction|LoadAssetsinData)
  (CallFunction|RefreshFarmManager))

(fn ConstructionScript)

(fn ClassforCropType
  (params (CropType :type CropTypes%20Enum :default "NewEnumerator2"))
  (return (Utilities|Select :Index CropType :NewEnumerator2 0 :NewEnumerator0 "/Game/FungusFarm/Blueprints/Crops/amanita_01_BP.Amanita_01_BP_C" :NewEnumerator1 "/Game/FungusFarm/Blueprints/Crops/WhiteButton_01_BP.WhiteButton_01_BP_C" :NewEnumerator3 "/Game/FungusFarm/Blueprints/Crops/BlueMycena_01_BP.BlueMycena_01_BP_C")))

(fn CalculatedProductionRates
  (Utilities|IsValid (Variables|Default|GetCurrentFarmManager)
    (:Is%20Valid
      (return (Default|CalculatedProductionRates (Variables|Default|GetCurrentFarmManager))))
    (:Is%20Not%20Valid
      (return 0))))

(fn SetCurrentFarmManager
  (params (Manager :type Farm%20Manager%20Base%20BP%20Object%20Reference))
  (Variables|Default|SetCurrentFarmManager Manager))

(fn Pause
  (bind _returnvalue (Game|SetGamePaused true))
  (if _returnvalue
    (Default|CallOnGamePaused)))

(fn Unpause
  (bind _returnvalue (Game|SetGamePaused false))
  (if _returnvalue
    (Default|CallOnGameUnPaused)))

(fn RecipeUnlocked?
  (params (Recipe%20Code :type Name))
  (return (Utilities|Array|ContainsItem (Variables|Default|GetUnlockedRecipes) Recipe%20Code)))

(fn UnlockRecipe
  (params (Recipe%20Code :type Name))
  (Utilities|Array|AddUnique (Variables|Default|GetUnlockedRecipes) Recipe%20Code))

(fn GetAllRecipes
  (LocalVariables|SettmpAllRecipes (Utilities|Array|MakeArray))
  (bind _outrownames (DataTable|GetDataTableRowNames (Variables|Default|GetCraftingRecipeData)))
  (for _array_element _outrownames
    (bind _returnvalue (Utilities|GetDataTableRow (Variables|Default|GetCraftingRecipeData) _array_element)
      (:then
        (Utilities|Array|Add (LocalVariables|GettmpAllRecipes) (|Copy _returnvalue)))))
  (return (LocalVariables|GettmpAllRecipes)))

(fn GetAllUnlockedRecipes
  (params (Minimum%20Tier :type Integer) (Maximum%20Tier :type Integer) (RequiredCategories :type Array%20of%20Names) (AnyCategory :type Boolean))
  (Utilities|FlowControl|Sequence
    (:then_0
      ;[1 1 1 1 16] Init our locals
      (LocalVariables|SettmpMinTier Minimum%20Tier)
      (LocalVariables|SettmpMaxTier Maximum%20Tier)
      (LocalVariables|SettmpRequiredCategories RequiredCategories)
      (LocalVariables|SettmpAnyCategory AnyCategory)
      (LocalVariables|SettmpAllRecipes (Utilities|Array|MakeArray)))
    (:then_1
      (for _array_element (Variables|Default|GetUnlockedRecipes)
        (if (Utilities|Name|NotEqual(Name) _array_element "Nothing")
          (bind _returnvalue (Utilities|GetDataTableRow (Variables|Default|GetCraftingRecipeData) _array_element)
            (:then
              (if (and (or (== (LocalVariables|GettmpMinTier) -1) (<= (LocalVariables|GettmpMinTier) (.Tier (Utilities|Struct|BreakCraftingRecipe _returnvalue)))) (or (== (LocalVariables|GettmpMaxTier) -1) (>= (LocalVariables|GettmpMaxTier) (.Tier (Utilities|Struct|BreakCraftingRecipe _returnvalue)))))
                (if (== (Utilities|Array|Length (LocalVariables|GettmpRequiredCategories)) 0)
                  (Utilities|Array|Add (LocalVariables|GettmpAllRecipes) (|Copy _returnvalue) :!label _label)
                  (elif (LocalVariables|GettmpAnyCategory)
                    (if (CallFunction|HasAnyNames? (.RecipeCategories (Utilities|Struct|BreakCraftingRecipe _returnvalue)) (LocalVariables|GettmpRequiredCategories))
                      (goto _label))
                    (elif (CallFunction|HasAllNames? (.RecipeCategories (Utilities|Struct|BreakCraftingRecipe _returnvalue)) (LocalVariables|GettmpRequiredCategories))
                      (goto _label)))))))))
      (return (LocalVariables|GettmpAllRecipes)))))

(fn RecipesUnlocked?
  (params (Recipe%20Codes :type Array%20of%20Names))
  (bind _array_element (Utilities|Array|ForEachLoopwithBreak Recipe%20Codes :!label _label)
    (:LoopBody
      (if (not (Utilities|Array|ContainsItem (Variables|Default|GetUnlockedRecipes) _array_element))
        (LocalVariables|SettmpAllUnlocked false)
        (goto _label Break)))
    (:Completed
      (return (LocalVariables|GettmpAllUnlocked)))))

(fn GetAllCropData
  (LocalVariables|SettmpAllCrops (Utilities|Array|MakeArray))
  (bind _outrownames (DataTable|GetDataTableRowNames (Variables|Default|GetCropData)))
  (for _array_element _outrownames
    (bind _returnvalue (Utilities|GetDataTableRow (Variables|Default|GetCropData) _array_element)
      (:then
        (Utilities|Array|Add (LocalVariables|GettmpAllCrops) (|Copy _returnvalue)))))
  (return (LocalVariables|GettmpAllCrops)))

(fn GetAllUnlockedCropData
  (LocalVariables|SettmpAllUnlocked (Utilities|Array|MakeArray))
  (for _array_element (Variables|Default|GetUnlockedCrops)
    (bind _returnvalue (Utilities|GetDataTableRow (Variables|Default|GetCropData) _array_element)
      (:then
        (Utilities|Array|Add (LocalVariables|GettmpAllUnlocked) (|Copy _returnvalue)))))
  (return (LocalVariables|GettmpAllUnlocked)))

(fn GetFarmManager
  (return (Variables|Default|GetCurrentFarmManager)))

(fn GetAllTools
  (return (Variables|Default|GetAllTools)))

(fn LoadInitTools
  (Utilities|Array|Clear (Variables|Default|GetAllTools))
  (for _array_element (Variables|Default|GetUnlockedTools)
    (PlayerTools|AddTool _array_element))
  (return (Variables|Default|GetAllTools)))

(fn GetToolbyCode
  (params (Tool%20Code :type Name))
  (bind _array_element (Utilities|Array|ForEachLoopwithBreak (Variables|Default|GetAllTools) :!label _label)
    (:LoopBody
      (if (Utilities|Name|Equal(Name) (Variables|/Game/FungusFarm/Blueprints/Tools/ToolBase_BP.ToolBase_BP_C|GetTool%20Code _array_element) Tool%20Code)
        (LocalVariables|SetlclTool _array_element)
        (goto _label Break)))
    (:Completed
      (return (LocalVariables|GetlclTool)))))

(fn CropUnlocked?
  (params (Crop%20Name :type Name))
  (return (Utilities|Array|ContainsItem (Variables|Default|GetUnlockedCrops) Crop%20Name)))

(fn UnlockCrop
  (params (Crop%20Name :type Name))
  (Utilities|Array|AddUnique (Variables|Default|GetUnlockedCrops) Crop%20Name))

(fn ToolUnlocked?
  (params (Tool%20Name :type Name))
  (return (Utilities|Array|ContainsItem (Variables|Default|GetUnlockedTools) Tool%20Name)))

(fn UnlockTool
  (params (Tool%20Name :type Name))
  (Utilities|Array|AddUnique (Variables|Default|GetUnlockedTools) Tool%20Name)
  (PlayerTools|AddTool Tool%20Name))

(fn GetCropData
  (params (Crop%20Name :type Name))
  (bind _returnvalue (Utilities|GetDataTableRow (Variables|Default|GetCropData) Crop%20Name)
    (:then
      (return true (|Copy _returnvalue)))
    (:RowNotFound
      (return false ""))))

(fn GetGoodsData
  (params (Goods%20Name :type Name))
  (bind _returnvalue (Utilities|GetDataTableRow (Variables|Default|GetGoodsData) Goods%20Name)
    (:then
      (return true (|Copy _returnvalue)))
    (:RowNotFound
      (return false ""))))

(fn ClassforCropName
  (params (Crop%20Name :type Name))
  (bind (_found_ _crop_data) (Crops|GetCropData Crop%20Name))
  (if _found_
    (bind _ascrop_base_bp (Utilities|Casting|CastToCropBase_BPClass (.ActorClass (Utilities|Struct|BreakCropType _crop_data)))
      (:then
        (return _ascrop_base_bp))
      (:CastFailed
        _)))
  (return 0))

(fn GetRecipeData
  (params (Recipe%20Code :type Name))
  (if (Utilities|Name|Equal(Name) Recipe%20Code "None")
    _
    (else
      (bind _returnvalue (Utilities|GetDataTableRow (Variables|Default|GetCraftingRecipeData) Recipe%20Code)
        (:then
          (return true (|Copy _returnvalue)))
        (:RowNotFound
          _))))
  (return false ""))

(fn TrackGoodsHarvestedTotals
  (params (Goods :type Goods%20Quantity%20Structure) (SkipUpdates :type Boolean))
  (bind (_name _quantity) (Utilities|Struct|BreakGoodsQuantity Goods))
  (Utilities|FlowControl|Sequence
    (:then_0
      ;[1 1 1] Update totals
      (Utilities|Map|Add (Variables|TrackingandGoals|GetGoodsHarvestedTotals) _name (select (Utilities|Map|Contains (Variables|TrackingandGoals|GetGoodsHarvestedTotals) _name) (+ (.Value (Utilities|Map|Find (Variables|TrackingandGoals|GetGoodsHarvestedTotals) _name)) _quantity) _quantity)))
    (:then_1
      (if (not SkipUpdates)
        ;[1 1 1] Update Goals
        (LocalVariables|SettmpGoods (Utilities|Array|MakeArray Goods))
        (bind _gameplaygoalsmanager (Utilities|GetGameplayGoalsManager))
        (Class|ActorGoalsComponent|UpdateHarvestedGoodsProgress _gameplaygoalsmanager (LocalVariables|GettmpGoods))))))

(fn TrackGoodsHarvestedTotalsBatch
  (params (Goods :type Array%20of%20Goods%20Quantity%20Structures))
  (for _array_element Goods
    (TrackingandGoals|TrackGoodsHarvestedTotals _array_element true))
  (bind _gameplaygoalsmanager (Utilities|GetGameplayGoalsManager))
  (Class|ActorGoalsComponent|UpdateHarvestedGoodsProgress _gameplaygoalsmanager Goods))

(fn CheckHarvestedGoodsTotals
  (params (Check%20Harvested%20Goods :type Goods%20Quantity%20Structure))
  (bind (_name _quantity) (Utilities|Struct|BreakGoodsQuantity Check%20Harvested%20Goods))
  (bind _goodsharvestedtotals (Variables|TrackingandGoals|GetGoodsHarvestedTotals))
  (bind (_value _returnvalue) (Utilities|Map|Find _goodsharvestedtotals _name))
  (bind _returnvalue_2 (>= _value _quantity))
  (bind _returnvalue_3 (select _returnvalue _returnvalue_2 false))
  (return _returnvalue_3 (select _returnvalue_3 0.0 (- _quantity _value))))

(fn TrackCraftedRecipes
  (params (Crafted%20Recipe :type Crafting%20Recipe%20Structure) (Produced%20Goods :type Array%20of%20Goods%20Quantity%20Structures))
  (bind _name (Utilities|Struct|BreakCraftingRecipe Crafted%20Recipe))
  (Utilities|FlowControl|Sequence
    (:then_0
      ;[1 1 1] Track the recipe crafting
      (Utilities|Map|Add (Variables|TrackingandGoals|GetCraftedRecipesTotals) _name (+ (.Value (Utilities|Map|Find (Variables|TrackingandGoals|GetCraftedRecipesTotals) _name)) 1)))
    (:then_1
      ;[1 1 1] Track goods crafted
      (for _array_element Produced%20Goods
        (Utilities|Map|Add (Variables|TrackingandGoals|GetGoodsCraftedTotals) (.Name (Utilities|Struct|BreakGoodsQuantity _array_element)) (select (Utilities|Map|Contains (Variables|TrackingandGoals|GetGoodsCraftedTotals) (.Name (Utilities|Struct|BreakGoodsQuantity _array_element))) (+ (.Value (Utilities|Map|Find (Variables|TrackingandGoals|GetGoodsCraftedTotals) (.Name (Utilities|Struct|BreakGoodsQuantity _array_element)))) (.Quantity (Utilities|Struct|BreakGoodsQuantity _array_element))) (.Quantity (Utilities|Struct|BreakGoodsQuantity _array_element))))))
    (:then_2
      ;[1 1 1] Update goals
      (bind _gameplaygoalsmanager (Utilities|GetGameplayGoalsManager))
      (Class|ActorGoalsComponent|UpdateCraftedRecipesProgress _gameplaygoalsmanager (.Name (Utilities|Struct|BreakCraftingRecipe Crafted%20Recipe)) 1))))

(fn CheckCraftedRecipesTotals
  (params (Recipe%20Name :type Name) (Times%20Crafted :type Integer))
  (bind _craftedrecipestotals (Variables|TrackingandGoals|GetCraftedRecipesTotals))
  (bind _value (Utilities|Map|Find _craftedrecipestotals Recipe%20Name))
  (bind _returnvalue (>= _value Times%20Crafted))
  (return _returnvalue (select _returnvalue 0 (- Times%20Crafted _value))))

(fn EquipmentDataforGoods
  (params (Goods%20Info :type Goods%20Type%20Structure))
  (bind _name (Utilities|Struct|BreakGoodsType Goods%20Info))
  (bind (_found _equipment_data) (CallFunction|GetEquipmentData _name))
  (if _found
    (return true _equipment_data)
    (else
      (return false ""))))

(fn GetEquipmentData
  (params (Equipment%20Name :type Name))
  (bind _returnvalue (Utilities|GetDataTableRow (Variables|Default|GetEquipmentData) Equipment%20Name)
    (:then
      (return true (|Copy _returnvalue)))
    (:RowNotFound
      (return false ""))))

(fn GoodsDataforEquipment
  (params (Equipment :type Equipment%20Type%20Structure))
  (bind _outrownames (DataTable|GetDataTableRowNames (Variables|Default|GetGoodsData)))
  (bind _array_element (Utilities|Array|ForEachLoopwithBreak _outrownames :!label _label)
    (:LoopBody
      (bind _returnvalue (Utilities|GetDataTableRow (Variables|Default|GetGoodsData) _array_element)
        (:then
          (if (Utilities|Name|Equal(Name) (.EquipmentName (Utilities|Struct|BreakGoodsType _returnvalue)) (.Name (Utilities|Struct|BreakEquipmentType Equipment)))
            (LocalVariables|SettmpGoodsInfo (|Copy _returnvalue))
            (LocalVariables|SettmpFound true)
            (goto _label Break)))))
    (:Completed
      (return (LocalVariables|GettmpFound) (LocalVariables|GettmpGoodsInfo)))))

(fn GetCropPlotData
  (params (Crop%20Plot%20Name :type Name))
  (bind _returnvalue (Utilities|GetDataTableRow (Variables|Default|GetCropPlotData) Crop%20Plot%20Name)
    (:then
      (return true (|Copy _returnvalue)))
    (:RowNotFound
      (return false ""))))

(fn GetFarmManagerModData
  (params (Modifier%20Name :type Name))
  (return false ""))

(fn GetCropPlotModData
  (params (Mod%20Name :type Name))
  (bind _returnvalue (Utilities|GetDataTableRow (Variables|Default|GetCropPlotModsData) Mod%20Name)
    (:then
      (return true (|Copy _returnvalue)))
    (:RowNotFound
      (return false ""))))

(fn GetAllGoods
  (bind _outrownames (DataTable|GetDataTableRowNames (Variables|Default|GetGoodsData)))
  (for _array_element _outrownames
    (bind _returnvalue (Utilities|GetDataTableRow (Variables|Default|GetGoodsData) _array_element)
      (:then
        (Utilities|Array|Add (LocalVariables|GettmpAllGoods) (|Copy _returnvalue)))))
  (return (LocalVariables|GettmpAllGoods)))

(fn GetAllEquipmentData
  (bind _outrownames (DataTable|GetDataTableRowNames (Variables|Default|GetEquipmentData)))
  (for _array_element _outrownames
    (bind _returnvalue (Utilities|GetDataTableRow (Variables|Default|GetEquipmentData) _array_element)
      (:then
        (Utilities|Array|Add (LocalVariables|GettmpAllEquipment) (|Copy _returnvalue)))))
  (return (LocalVariables|GettmpAllEquipment)))

(fn GetAllCropPlotModData
  (bind _outrownames (DataTable|GetDataTableRowNames (Variables|Default|GetCropPlotModsData)))
  (for _array_element _outrownames
    (bind _returnvalue (Utilities|GetDataTableRow (Variables|Default|GetCropPlotModsData) _array_element)
      (:then
        (Utilities|Array|Add (LocalVariables|GettmpAllCropPlotMods) (|Copy _returnvalue)))))
  (return (LocalVariables|GettmpAllCropPlotMods)))

(fn HasMarketInventory
  (params (Requirements :type Goods%20Quantity%20Structure))
  (bind _hasall (Default|HasGoods? (Variables|Default|GetMarketInventory) Requirements))
  (return _hasall))

(fn RemoveMarketInventory
  (params (GoodsInfo :type Goods%20Quantity%20Structure))
  (bind _marketinventory (Variables|Default|GetMarketInventory))
  (bind _successful (Default|RemoveGoodsInventory _marketinventory GoodsInfo))
  (return _successful (Default|GetGoodsInventoryQuantity _marketinventory (.Name (Utilities|Struct|BreakGoodsQuantity GoodsInfo)))))

(fn GetMarketInventoryQuantity
  (params (Type :type Name))
  (return (Default|GetGoodsInventoryQuantity (Variables|Default|GetMarketInventory) Type)))

(fn RefreshMarketInventory
  (if (Default|IsEmpty? (Variables|Default|GetMarketInventory))
    (Default|AddGoodsInventoryBatch (Variables|Default|GetMarketInventory) (LocalVariables|GettmpDefaultMarketInventory))))

(fn RefreshFarmManager
  (bind _outactors (Actor|GetAllActorsOfClass "/Game/FungusFarm/Blueprints/Equipment/FarmManagerBase_BP.FarmManagerBase_BP_C"))
  (bind _array_element (Utilities|Array|ForEachLoopwithBreak _outactors :!label _label)
    (:LoopBody
      (bind _output_get (Variables|Default|SetCurrentFarmManager _array_element))
      (Default|RefreshPlotReferences _output_get)
      (goto _label Break))))

(fn GiveDefaultGoods
  (Default|AddGoodsInventoryBatch (.Inventory (CallFunction|GetPlayerInventory)) (LocalVariables|GettmpDefaultGoods)))

(fn TrackGoodsSoldTotals
  (params (Goods :type Goods%20Quantity%20Structure) (Skip%20Goal%20Check :type Boolean))
  (bind (_name _quantity) (Utilities|Struct|BreakGoodsQuantity Goods))
  (Utilities|FlowControl|Sequence
    (:then_0
      ;[1 1 1] Update totals
      (Utilities|Map|Add (Variables|TrackingandGoals|GetGoodsSoldTotals) _name (select (Utilities|Map|Contains (Variables|TrackingandGoals|GetGoodsSoldTotals) _name) (+ (.Value (Utilities|Map|Find (Variables|TrackingandGoals|GetGoodsSoldTotals) _name)) _quantity) _quantity)))
    (:then_1
      (if (not Skip%20Goal%20Check)
        ;[1 1 1] Update Goals
        (LocalVariables|SettmpGoods (Utilities|Array|MakeArray Goods))
        (bind _gameplaygoalsmanager (Utilities|GetGameplayGoalsManager))
        (Class|ActorGoalsComponent|UpdateSoldGoodsProgress _gameplaygoalsmanager (LocalVariables|GettmpGoods))))))

(fn GetMarketInventory
  (bind _inventorymap (Default|GetAllInventoryasMap (Variables|Default|GetMarketInventory)))
  (return _inventorymap))

(fn AddTool
  (params (Tool%20Name :type Name))
  (bind _tmptoolnameclassmap (LocalVariables|GettmpToolNameClassMap))
  (bind (_value _returnvalue) (Utilities|Map|Find _tmptoolnameclassmap Tool%20Name))
  (if _returnvalue
    (bind _returnvalue_2 (Game|ConstructObjectfromClass _value self))
    (Utilities|Array|Add (Variables|Default|GetAllTools) _returnvalue_2)
    (bind _asff_player_controller_bp (Utilities|Casting|CastToFF_PlayerController_BP (Game|GetPlayerController 0)))
    (Default|OnToolsChanged _asff_player_controller_bp)))