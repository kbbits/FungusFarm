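; Game mode base for Fungus Farm that handles switching between the home, farm, lab and market screens.
; Each load event casts player zero's controller to FF_PlayerController and forwards to its loaded, unloaded or menu-showing handler, passing the current farm or lab level name.
; An older level-streaming version, with blocking loads and unloads and streaming flushes, remains in the graph but is disconnected.
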(event Custom|LoadHomeLevel
  (params (DontShowHomeMenu :type Boolean))
  (bind _asff_player_controller (Utilities|Casting|CastToFF_PlayerController (Game|GetPlayerController 0)))
  (Default|OnFarmUnloaded _asff_player_controller)
  (if (not DontShowHomeMenu)
    (Default|ShowHomeMenu _asff_player_controller)))

(event Custom|LoadCurrentFarmLevel
  (bind _asff_player_controller (Utilities|Casting|CastToFF_PlayerController (Game|GetPlayerController 0)))
  (Default|OnFarmLoaded _asff_player_controller (Variables|Default|GetCurrentFarmLevelName)))

(event Custom|LoadCurrentLabLevel
  (bind _asff_player_controller (Utilities|Casting|CastToFF_PlayerController (Game|GetPlayerController 0)))
  (Default|OnLabLoaded _asff_player_controller (Variables|Default|GetCurrentLabLevelName)))

(event Custom|LoadMarketLevel
  (bind _asff_player_controller (Utilities|Casting|CastToFF_PlayerController (Game|GetPlayerController 0)))
  (Default|ShowMarketMenu _asff_player_controller))

(fn ConstructionScript)