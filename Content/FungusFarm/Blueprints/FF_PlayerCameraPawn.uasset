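; Player camera pawn for FungusFarm that pans across the world's XZ plane and eases along Y.
; MoveRight and MoveUp axis inputs feed the FloatingPawnMovement component as X and Z movement.
; Tick interpolates the actor's Y toward TargetYLocation, which starts at the spawn Y and is not changed elsewhere in this graph.
; An orthographic-width zoom interpolation remains in the graph but is disconnected.
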(event Custom|MoveRight
  (params (AxisValue :type Float%20%28single-precision%29))
  (if (> (Math|Float|Absolute(Float) AxisValue) 0.0)
    (Class|PawnMovementComponent|AddInputVector (Variables|Default|GetFloatingPawnMovement) (Math|Vector|MakeVector (* AxisValue 1.0) 0.0 0.0) false)))

(event Custom|MoveUp
  (params (Add%20Value :type Float%20%28single-precision%29))
  (if (> (Math|Float|Absolute(Float) Add%20Value) 0.0)
    (Class|PawnMovementComponent|AddInputVector (Variables|Default|GetFloatingPawnMovement) (Math|Vector|MakeVector 0.0 0.0 (* Add%20Value 1.0)) false)))

(event EventTick
  (params (DeltaSeconds :type Float%20%28single-precision%29))
  (bind _returnvalue (Transformation|GetActorLocation))
  (bind (_x _y _z) (Math|Vector|BreakVector _returnvalue))
  (if (not (== (Variables|Default|GetTargetYLocation) _y))
    (Transformation|SetActorLocation (Math|Vector|MakeVector _x (Math|Interpolation|FInterpTo _y (Variables|Default|GetTargetYLocation) DeltaSeconds 1e+01) _z) false false)))

(event EventBeginPlay
  (Variables|Default|SetTargetYLocation (.Y (Math|Vector|BreakVector (Transformation|GetActorLocation)))))

(fn ConstructionScript)