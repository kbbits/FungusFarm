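; ModSlot_CAC_BP is a child actor component that hosts a ModSlot and restores its link to the equipment slotted in it.
; RefreshChildSlotReferences searches all ModEquipment_Base actors for the one whose MyID matches a valid SlottedEquipmentID GUID.
; On a match, it casts the child actor to ModSlot and passes that equipment to OnEquipmentPlaced.
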(event Custom|RefreshChildSlotReferences
  (if (Guid|IsValidGuid (Variables|Default|GetSlottedEquipmentID))
    (bind _outactors (Actor|GetAllActorsOfClass "/Game/FungusFarm/Blueprints/Equipment/EquipmentMods/ModEquipment_Base.ModEquipment_Base_C"))
    (bind _array_element (Utilities|Array|ForEachLoopwithBreak _outactors :!label _label)
      (:LoopBody
        (if (== (Variables|/Game/FungusFarm/Blueprints/Equipment/Equipment_Base.Equipment_Base_C|GetMyID _array_element) (Variables|Default|GetSlottedEquipmentID))
          (bind _asmod_slot (Utilities|Casting|CastToModSlot (Variables|Default|GetChildActor)))
          (Default|OnEquipmentPlaced _asmod_slot _array_element)
          (goto _label Break))))))