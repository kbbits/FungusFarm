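; Base Blueprint for spirit totems, placeable equipment that grants global gameplay effects while set on a SpiritTotem_Target.
; Modifiers accumulate up to the totem's level and register with the global manager on place, removed on pickup.
; Contributed goods fill per-level requirements; leveling refreshes effects, tracks an upgrade recipe, plays a shake animation and swaps the level sprite.
; Clicking the sprite moves the camera to its target and opens the totem menu.
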(event OnClicked(EquipmentSprite)
  (params (TouchedComponent :type Primitive%20Component%20Object%20Reference) (ButtonPressed :type Key%20Structure :default "None"))
  (bind _asff_player_camera_pawn (Utilities|Casting|CastToFF_PlayerCameraPawn (Game|Player|GetPlayerPawn 0)))
  (bind _asspirit_totem_target (Utilities|Casting|CastToSpiritTotem_Target (Variables|Default|GetCurrentPlaceableTarget)))
  (Default|NavigatetoAnchorTarget _asff_player_camera_pawn _asspirit_totem_target)
  (bind _asff_player_controller_bp (Utilities|Casting|CastToFF_PlayerController_BP (Game|GetPlayerController 0)))
  (Default|ShowTotemMenu _asff_player_controller_bp self))

(event OnBeginCursorOver(EquipmentSprite)
  (params (TouchedComponent :type Primitive%20Component%20Object%20Reference))
  (bind _asff_player_controller_bp (Utilities|Casting|CastToFF_PlayerController_BP (Game|GetPlayerController 0)))
  (Variables|Default|SetOriginalCursor (Variables|/Script/Engine.PlayerController|GetCurrentMouseCursor _asff_player_controller_bp))
  (Variables|/Script/Engine.PlayerController|SetCurrentMouseCursor _asff_player_controller_bp "Default"))

(event OnEndCursorOver(EquipmentSprite)
  (params (TouchedComponent :type Primitive%20Component%20Object%20Reference))
  (bind _asff_player_controller_bp (Utilities|Casting|CastToFF_PlayerController_BP (Game|GetPlayerController 0)))
  (Variables|/Script/Engine.PlayerController|SetCurrentMouseCursor _asff_player_controller_bp (Variables|Default|GetOriginalCursor)))

(event Custom|OnLevelUp
  (bind _equipmentsprite (Variables|Default|GetEquipmentSprite))
  (bind _equipmentsprite_2 (Variables|Default|GetEquipmentSprite))
  (bind _equipmentsprite_3 (Variables|Default|GetEquipmentSprite))
  (Variables|Default|SettmpSpriteLocationOrig (Transformation|GetWorldLocation _equipmentsprite_2))
  (Variables|Default|SettmpSpriteScaleOrig (Transformation|GetWorldScale _equipmentsprite_2))
  (bind (_direction _scaleshake _locationshake) (Timeline|LevelUpAnim PlayFromStart)
    (:Update
      (Transformation|SetWorldLocation _equipmentsprite_3 (+ (Variables|Default|GettmpSpriteLocationOrig) (* _locationshake 4.0)) false true)
      (Transformation|SetWorldScale3D _equipmentsprite_3 (* (Variables|Default|GettmpSpriteScaleOrig) _scaleshake)))
    (:Finished
      (Transformation|SetWorldLocation _equipmentsprite (Variables|Default|GettmpSpriteLocationOrig) false true)
      (Transformation|SetWorldScale3D _equipmentsprite (Variables|Default|GettmpSpriteScaleOrig))
      (Audio|PlaySound2D "/Game/FungusFarm/Assets/Sound/Effects/Pops_01_Cue.Pops_01_Cue" 1.0 1.0 0.0 0 self)
      (CallFunction|UpdateVis)
      (Default|CallOnTotemLeveledUp self))))

(event EventOnPlaceEquipment
  (|CallParentFunction)
  (CallFunction|ApplyEffects))

(event EventOnPickupEquipment
  (|CallParentFunction)
  (CallFunction|RemoveEffects))

(event EventHighlightPlacableTargets
  (|CallParentFunction)
  (bind _outactors (Actor|GetAllActorsOfClass "/Game/FungusFarm/Blueprints/Equipment/SpiritTotems/SpiritTotem_Target.SpiritTotem_Target_C"))
  (for _array_element _outactors
    (bind _hasequipment (Default|HasEquipment? _array_element))
    (if (not _hasequipment)
      (bind _can_accept (Default|CanAcceptEquipment? _array_element self))
      (if _can_accept
        (Default|HighlightforAccepting _array_element self)))))

(event EventUnHighlightPlacableTargets
  (|CallParentFunction)
  (bind _outactors (Actor|GetAllActorsOfClass "/Game/FungusFarm/Blueprints/Equipment/SpiritTotems/SpiritTotem_Target.SpiritTotem_Target_C"))
  (for _array_element _outactors
    (Default|UnhighlightforAccepting _array_element)))

(event EventBeginPlay
  (|CallParentFunction)
  (CallFunction|RemoveEffects)
  (if (and (Variables|Default|GetPlaced) (Variables|Default|GetReady))
    (CallFunction|ApplyEffects)))

(event EventOnLoadFinished
  (params (Filter :type SE%20Level%20Filter%20Structure%20%28by%20ref%29) (bError :type Boolean))
  (|CallParentFunction Filter bError)
  (CallFunction|RemoveEffects)
  (if (and (Variables|Default|GetPlaced) (Variables|Default|GetReady))
    (CallFunction|ApplyEffects)))

(fn ConstructionScript
  (|CallParentFunction)
  (CallFunction|UpdateVis))

(fn ApplyEffects
  (Class|GlobalManager|AddGlobalEffects (CallFunction|GetGlobalManager) (CallFunction|GetActiveModifiers)))

(fn GetActiveModifiers
  (if (>= (Variables|Default|GetTotemLevel) 0)
    (for _index (range 0 (Math|Integer|Min(Integer) (Variables|Default|GetTotemLevel) (Utilities|Array|LastIndex (Variables|Default|GetGlobalModifiersByLevel))))
      (if (Utilities|Name|NotEqual(Name) (.UniqueName (Utilities|Struct|BreakGlobalEffect (Utilities|Array|Get(acopy) (Variables|Default|GetGlobalModifiersByLevel) _index))) "None")
        (Utilities|Array|Add (LocalVariables|GettmpActiveModifiers) (Utilities|Array|Get(acopy) (Variables|Default|GetGlobalModifiersByLevel) _index)))))
  (return (LocalVariables|GettmpActiveModifiers)))

(fn RemoveEffects
  (for _array_element (CallFunction|GetActiveModifiers)
    (Utilities|Array|Add (LocalVariables|GettmpEffectNames) (.UniqueName (Utilities|Struct|BreakGlobalEffect _array_element))))
  (Class|GlobalManager|RemoveGlobalEffects (CallFunction|GetGlobalManager) (LocalVariables|GettmpEffectNames)))

(fn GetRemaningLevelUpRequiremets
  (return (.ReturnValue (Class|GoodsFunctionLibrary|SubtractGoodsQuantities (CallFunction|GetNextLevelUpRequirementsBase) (.GoodsQuantities (Utilities|Struct|BreakGoodsQuantitySet (Variables|Default|GetContributionsToNextLevel))) false))))

(fn GetNextLevelUpRequirementsBase
  (if (Utilities|Array|IsValidIndex (Variables|Default|GetLevelUpRequirements) (Variables|Default|GetTotemLevel))
    (return (.GoodsQuantities (Utilities|Struct|BreakGoodsQuantitySet (Utilities|Array|Get(acopy) (Variables|Default|GetLevelUpRequirements) (Variables|Default|GetTotemLevel)))))
    (else
      (return (Utilities|Array|MakeArray)))))

(fn AtMaxTotemLevel?
  (return (>= (Variables|Default|GetTotemLevel) (+ (Utilities|Array|LastIndex (Variables|Default|GetLevelUpRequirements)) 1))))

(fn AddtoLevelUpProgress
  (params (AddedGoods :type Array%20of%20Goods%20Quantity%20Structures))
  (bind _contributionstonextlevel (Variables|Default|GetContributionsToNextLevel))
  (bind _goodsquantities (Utilities|Struct|BreakGoodsQuantitySet _contributionstonextlevel))
  (bind (_bsuccessful _returnvalue) (Class|GoodsFunctionLibrary|SumGoodsQuantities _goodsquantities AddedGoods false false))
  (if _bsuccessful
    (Utilities|Struct|SetmembersinGoodsQuantitySet (Variables|Default|GetContributionsToNextLevel) _returnvalue)
    (if (== (Utilities|Array|Length (CallFunction|GetRemaningLevelUpRequiremets)) 0)
      (Utilities|Array|Clear (.GoodsQuantities (Utilities|Struct|BreakGoodsQuantitySet (Variables|Default|GetContributionsToNextLevel))))
      (CallFunction|RemoveEffects)
      (Variables|Default|SetTotemLevel (+ (Variables|Default|GetTotemLevel) 1))
      (CallFunction|ApplyEffects)
      (CallFunction|TrackLevelUpRecipeforTotemLevel (Variables|Default|GetTotemLevel))
      (CallFunction|OnLevelUp)
      (return true)
      (else
        (return false)))
    (else
      (return false))))

(fn LevelUpRecipeforTotemLevel
  (params (TotemLevel :type Integer))
  (bind _asff_game_state (Utilities|Casting|CastToFF_GameState (Game|GetGameState)))
  (return (.Found (Default|GetRecipeData _asff_game_state (Utilities|String|StringToName (Utilities|String|Append (Utilities|String|ToString(Name) (Variables|Default|GetLevelUpRecipeBaseName)) "Upgrade" (Utilities|String|ToString(Integer) TotemLevel))))) (.Recipe (Default|GetRecipeData _asff_game_state (Utilities|String|StringToName (Utilities|String|Append (Utilities|String|ToString(Name) (Variables|Default|GetLevelUpRecipeBaseName)) "Upgrade" (Utilities|String|ToString(Integer) TotemLevel)))))))

(fn TrackLevelUpRecipeforTotemLevel
  (params (TotemLevel :type Integer))
  (bind (_found _recipe) (CallFunction|LevelUpRecipeforTotemLevel TotemLevel))
  (if _found
    (bind _asff_game_state (Utilities|Casting|CastToFF_GameState (Game|GetGameState)))
    (Default|TrackCraftedRecipes _asff_game_state _recipe (Utilities|Array|MakeArray))
    (return)))

(fn UpdateVis
  (Utilities|FlowControl|Sequence
    (:then_0
      (if (Utilities|Array|IsValidIndex (Variables|Default|GetTotemSprites) (Variables|Default|GetTotemLevel))
        (bind _returnvalue (Utilities|LoadAssetBlocking (Utilities|Array|Get(acopy) (Variables|Default|GetTotemSprites) (Variables|Default|GetTotemLevel))))
        (bind _aspaper_sprite (Utilities|Casting|CastToPaperSprite _returnvalue))
        (Rendering|Components|Sprite|SetSprite (Variables|Default|GetEquipmentSprite) _aspaper_sprite)))
    (:then_1
      (Rendering|Components|TextRender|SetText (Variables|Default|GetTextRender) (Utilities|Text|ToText(Integer) (Variables|Default|GetTotemLevel))))))

(fn GetContributedQuanityforGoods
  (params (GoodsName :type Name))
  (bind _array_element (Utilities|Array|ForEachLoopwithBreak (.GoodsQuantities (Utilities|Struct|BreakGoodsQuantitySet (Variables|Default|GetContributionsToNextLevel))))
    (:LoopBody
      (if (Utilities|Name|Equal(Name) (.Name (Utilities|Struct|BreakGoodsQuantity _array_element)) GoodsName)
        (return (.Quantity (Utilities|Struct|BreakGoodsQuantity _array_element)))))
    (:Completed
      (return 0.0))))

(fn GetCurrentThumbnail
  (if (Utilities|Array|IsValidIndex (Variables|Default|GetTotemThumbnails) (Variables|Default|GetTotemLevel))
    (bind _returnvalue (Utilities|LoadAssetBlocking (Utilities|Array|Get(acopy) (Variables|Default|GetTotemThumbnails) (Variables|Default|GetTotemLevel))))
    (bind _astexture_2d (Utilities|Casting|CastToTexture2D _returnvalue)
      (:then
        (return _astexture_2d))
      (:CastFailed
        _)))
  (return "/Game/FungusFarm/Assets/Textures/Unknown_256.Unknown_256"))

(fn RefreshReferences
  (if true
    (bind _success (|CallParentFunction))
    (return _success)))

(fn UpdateSpriteAppearance
  (|CallParentFunction)
  (CallFunction|UpdateVis))