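; Base actor for Fungus Farm equipment that follows the cursor as a green/red ghost sprite until placed.
; A cursor trace finds an IPlaceableEquipmentTarget, which must accept it with no invalid overlaps; misses project onto the last hit's Y-depth plane.
; Placing notifies the target and sets Ready after a short delay; pickup notifies it and returns matching goods to GameState inventory.
; A gate refreshes ghost color one update after validity changes.
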(event EventOnPlaceEquipment
  (if (CallFunction|IsValidLocation?)
    (Variables|PlaceableEquipment|SetPlaced true)
    (Sprite|SetSpriteColor (Variables|Default|GetEquipmentSprite) (CallFunction|GetGhostColor))
    (Utilities|IsValid (Utilities|ToObject(Interface) (Variables|PlaceableEquipment|GetCurrentPlaceableTarget))
      (:Is%20Valid
        (Default|OnEquipmentPlaced (Variables|PlaceableEquipment|GetCurrentPlaceableTarget) self)
        (Utilities|FlowControl|Delay 0.2)
        (Variables|PlaceableEquipment|SetReady true)))))

(event EventOnBeginPlaceEquipment
  (Variables|PlaceableEquipment|SetReady false)
  (Variables|PlaceableEquipment|SetPlaced false)
  (CallFunction|OnMoveEquipment))

(event EventOnMoveEquipment
  (bind (_valid_ _location) (CallFunction|GetPlaceLocation))
  (CallFunction|SetValidLocation _valid_)
  (Transformation|SetActorLocation _location false true))

(event EventOnPickupEquipment
  (Utilities|IsValid (Utilities|ToObject(Interface) (Variables|PlaceableEquipment|GetCurrentPlaceableTarget))
    (:Is%20Valid
      (Default|OnEquipmentRemoved (Variables|PlaceableEquipment|GetCurrentPlaceableTarget) self))
    (:Is%20Not%20Valid
      _))
  (bind _asff_game_state (Utilities|Casting|CastToFF_GameState (Game|GetGameState)))
  (if (.Found? (Default|GoodsDataforEquipment _asff_game_state (Variables|Default|GetEquipmentData)))
    (Default|AddGoodsInventory _asff_game_state (Utilities|Struct|MakeGoodsQuantity (.Name (Utilities|Struct|BreakGoodsType (.Goods%20Info (Default|GoodsDataforEquipment _asff_game_state (Variables|Default|GetEquipmentData))))) 1.0))
    (Variables|PlaceableEquipment|SetReady false)
    (Variables|PlaceableEquipment|SetPlaced false)))

(fn ConstructionScript
  (|CallParentFunction))

(fn GetPlaceLocation
  (bind _returnvalue (Game|GetPlayerController 0))
  (bind (_worldlocation _worlddirection) (Game|Player|ConvertMouseLocationToWorldSpace _returnvalue))
  (bind (_hitresult _returnvalue_2) (Game|Player|GetHitResultUnderCursorbyChannel _returnvalue "TraceTypeQuery3" true))
  (bind (_bblockinghit _binitialoverlap _time _distance _location _impactpoint _normal _impactnormal _physmat _hitactor) (Collision|BreakHitResult _hitresult))
  (bind (_x _y _z) (Math|Vector|BreakVector _location))
  (if _returnvalue_2
    (Variables|PlaceableEquipment|SetPlaceDepthY (.Y (Math|Vector|BreakVector _location)))
    (bind _asiplaceable_equipment_target (Utilities|Casting|CastToIPlaceableEquipmentTarget _hitactor)
      (:then
        (Variables|PlaceableEquipment|SetCurrentPlaceableTarget _asiplaceable_equipment_target)
        (bind _can_accept (Class|IPlaceableEquipmentTarget|CanAcceptEquipment?(Message) _hitactor self))
        (if _can_accept
          (return (== (Variables|PlaceableEquipment|GetInvalidOverlaps) 0) (Math|Vector|MakeVector _x (Variables|PlaceableEquipment|GetPlaceDepthY) _z))
          (else
            _)))
      (:CastFailed
        _))
    (Variables|PlaceableEquipment|SetCurrentPlaceableTarget 0)
    (return false (Math|Vector|MakeVector _x (Variables|PlaceableEquipment|GetPlaceDepthY) _z))
    (else
      (Variables|PlaceableEquipment|SetCurrentPlaceableTarget 0)
      (return false (.Intersection (Class|KismetMathLibrary|LinePlaneIntersection _worldlocation (+ _worldlocation (* _worlddirection 1e+04)) (Class|KismetMathLibrary|MakePlanefromPointandNormal (Math|Vector|MakeVector 0.0 (Variables|PlaceableEquipment|GetPlaceDepthY) 0.0) "0,1.000000, 0")))))))

(fn GetGhostColor
  (return (select (Variables|PlaceableEquipment|GetPlaced) (Utilities|Struct|MakeLinearColor 1.0 1.0 1.0 1.0) (select (Variables|PlaceableEquipment|GetValidLocation) (Utilities|Struct|MakeLinearColor 0.0 1.0 0.0 0.4) (Utilities|Struct|MakeLinearColor 1.0 0.0 0.0 0.4)))))

(fn SetValidLocation
  (params (Valid? :type Boolean))
  (if (Math|Boolean|Equal(Boolean) Valid? (Variables|PlaceableEquipment|GetValidLocation))
    (Utilities|FlowControl|Gate false :!label _label
      (:Exit
        (Sprite|SetSpriteColor (Variables|Default|GetEquipmentSprite) (CallFunction|GetGhostColor))
        (goto _label Close)))
    (else
      (Variables|PlaceableEquipment|SetValidLocation Valid?)
      (goto _label Open))))

(fn IsValidLocation?
  (return (Variables|PlaceableEquipment|GetValidLocation)))