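; Mod slot actor, a placement target that holds one ModEquipment_Base item of an accepted class and exposes its attribute modifiers.
; Placed items snap to ModSpot; placement, removal and enable/disable changes fire dispatchers.
; The parent ModSlot_CAC_BP child actor component stores the slotted item's ID, and slots without that parent self-destruct five seconds after BeginPlay.
; Highlighting swaps dynamic materials and toggles the image plane's collision to accept placement.
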(event OnClicked(SlotImagePlane)
  (params (TouchedComponent :type Primitive%20Component%20Object%20Reference) (ButtonPressed :type Key%20Structure :default "None")))

(event Custom|RemoveModEquipment
  (Utilities|IsValid (Variables|Default|GetMyModEquipment)
    (:Is%20Valid
      (bind _asff_player_controller_bp (Utilities|Casting|CastToFF_PlayerController_BP (Game|GetPlayerController 0)))
      (Default|PickupEquipment _asff_player_controller_bp (Variables|Default|GetMyModEquipment) (not (.bDestroyOnRemove (Utilities|Struct|BreakEquipmentModType (Variables|/Game/FungusFarm/Blueprints/Equipment/EquipmentMods/ModEquipment_Base.ModEquipment_Base_C|GetEquipmentModData (Variables|Default|GetMyModEquipment)))))))))

(event Custom|NotifyModEquipmentEvent
  (params (EventType :type EEquipmentModEvent%20Enum :default "CropPlanted"))
  (bind _mymodequipment (Variables|Default|GetMyModEquipment))
  (Utilities|IsValid _mymodequipment
    (:Is%20Valid
      (Default|OnNotifyModEquipmentEvent _mymodequipment EventType))))

(event EventOnEquipmentEnabled
  (params (EnabledEquipment :type I%20Placeable%20Equipment%20Interface))
  (bind _asmod_equipment_base (Utilities|Casting|CastToModEquipment_Base EnabledEquipment))
  (if (== _asmod_equipment_base (Variables|Default|GetMyModEquipment))
    (Default|CallOnModifierEquipmentStateChanged self (Variables|Default|GetMyModEquipment))))

(event EventOnEquipmentDisabled
  (params (DisabledEquipment :type I%20Placeable%20Equipment%20Interface))
  (bind _asmod_equipment_base (Utilities|Casting|CastToModEquipment_Base DisabledEquipment))
  (if (== _asmod_equipment_base (Variables|Default|GetMyModEquipment))
    (Default|CallOnModifierEquipmentStateChanged self (Variables|Default|GetMyModEquipment))))

(event EventHighlightforAccepting
  (params (EquipmentToPlace :type I%20Placeable%20Equipment%20Interface))
  (Utilities|IsValid (Variables|Default|GetDynSlotGlowMaterial)
    (:Is%20Valid
      _)
    (:Is%20Not%20Valid
      (bind _returnvalue (Rendering|Material|CreateDynamicMaterialInstance (Variables|Default|GetSlotImagePlane) 0 "/Game/FungusFarm/Assets/Materials/FF_GlowEdge_MI.FF_GlowEdge_MI" "None" :!class /Script/Engine.PrimitiveComponent))
      (Variables|Default|SetDynSlotGlowMaterial _returnvalue)
      (Rendering|Material|SetTextureParameterValue (Variables|Default|GetDynSlotGlowMaterial) "MaterialTexture" (Variables|Default|GetSlotImage))))
  (Rendering|Material|SetMaterial (Variables|Default|GetSlotImagePlane) 0 (Variables|Default|GetDynSlotGlowMaterial))
  (Collision|SetCollisionProfileName (Variables|Default|GetSlotImagePlane) "PlaceableTarget" true :!class /Script/Engine.PrimitiveComponent))

(event EventOnEquipmentPlaced
  (params (Placed%20Equipment :type I%20Placeable%20Equipment%20Interface))
  (bind _asmod_equipment_base (Utilities|Casting|CastToModEquipment_Base Placed%20Equipment))
  (bind _output_get (Variables|Default|SetMyModEquipment _asmod_equipment_base))
  (bind _asmod_slot_cac_bp (Utilities|Casting|CastToModSlot_CAC_BP (Transformation|GetAttachParent (Variables|Default|GetScene)))
    (:then
      (Variables|/Script/FungusFarm.ModSlot_CAC|SetSlottedEquipmentID _asmod_slot_cac_bp (Variables|/Game/FungusFarm/Blueprints/Equipment/Equipment_Base.Equipment_Base_C|GetMyID _output_get))
      (Variables|/Game/FungusFarm/Blueprints/Equipment/PlaceableEquipment_Base.PlaceableEquipment_Base_C|SetCurrentPlaceableTarget (Variables|Default|GetMyModEquipment) self)
      (Transformation|AttachActorToActor _output_get self "None" "SnapToTarget" "KeepRelative" "KeepRelative" true)
      (Transformation|SetRelativeLocation (Variables|/Script/Engine.Actor|GetRootComponent _output_get) (.Location (Math|Transform|BreakTransform (Transformation|GetRelativeTransform (Variables|Default|GetModSpot)))) false true)
      (Default|CallOnModifierEquipmentPlaced self (Variables|Default|GetMyModEquipment)))
    (:CastFailed
      (Utilities|Casting|CastToIHasModSlots (Components|GetOwner _asmod_slot_cac_bp)))))

(event EventOnEquipmentRemoved
  (params (Removed%20Equipment :type I%20Placeable%20Equipment%20Interface))
  (bind _asmod_equipment_base (Utilities|Casting|CastToModEquipment_Base Removed%20Equipment))
  (if (== _asmod_equipment_base (Variables|Default|GetMyModEquipment))
    (Transformation|DetachFromActor _asmod_equipment_base "KeepWorld" "KeepWorld" "KeepWorld")
    (Variables|Default|SetMyModEquipment 0)
    (bind _asmod_slot_cac_bp (Utilities|Casting|CastToModSlot_CAC_BP (Transformation|GetAttachParent (Variables|Default|GetScene))))
    (Guid|InvalidateGuid (Variables|/Script/FungusFarm.ModSlot_CAC|GetSlottedEquipmentID _asmod_slot_cac_bp))
    (Default|CallOnModifierEquipmentRemoved self)))

(event EventUnhighlightforAccepting
  (Rendering|Material|SetMaterial (Variables|Default|GetSlotImagePlane) 0 (Variables|Default|GetDynSlotNormalMaterial))
  (Collision|SetCollisionProfileName (Variables|Default|GetSlotImagePlane) "NoCollision" true :!class /Script/Engine.PrimitiveComponent))

(event EventBeginPlay
  (Utilities|FlowControl|Delay 5.0)
  (Utilities|Casting|CastToModSlot_CAC_BP (Transformation|GetAttachParent (Variables|Default|GetScene))
    (:CastFailed
      (Development|PrintString (Utilities|String|Append "Destroying ModSlot " (Utilities|GetDisplayName self)))
      (Actor|DestroyActor))))

(fn ConstructionScript
  (bind _returnvalue (Rendering|Material|CreateDynamicMaterialInstance (Variables|Default|GetSlotImagePlane) 0 (Rendering|Material|GetMaterial (Variables|Default|GetSlotImagePlane) 0) "None" :!class /Script/Engine.PrimitiveComponent))
  (bind _output_get (Variables|Default|SetDynSlotNormalMaterial _returnvalue))
  (Rendering|Material|SetTextureParameterValue _output_get "MaterialTexture" (Variables|Default|GetSlotImage))
  (Rendering|Material|SetMaterial (Variables|Default|GetSlotImagePlane) 0 (Variables|Default|GetDynSlotNormalMaterial)))

(fn GetAllModifiers
  (Utilities|IsValid (Variables|Default|GetMyModEquipment)
    (:Is%20Valid
      (Utilities|Array|AppendArray (LocalVariables|GettmpAttributeModifiers) (Default|GetModifiers (Variables|Default|GetMyModEquipment))))
    (:Is%20Not%20Valid
      _))
  (return (LocalVariables|GettmpAttributeModifiers)))

(fn GetEquipmentMod
  (return (CallFunction|IsOccupied?) (Variables|Default|GetMyModEquipment)))

(fn IsOccupied?
  (return (Utilities|IsValid (Variables|Default|GetMyModEquipment))))

(fn GetModSlotParentActor
  (bind _asmod_slot_cac_bp (Utilities|Casting|CastToModSlot_CAC_BP (Transformation|GetAttachParent (Variables|Default|GetScene))))
  (return (Default|GetModSlotParent _asmod_slot_cac_bp)))

(fn CanAcceptEquipment?
  (params (Equipment :type Equipment%20Base%20Object%20Reference))
  (bind _asmod_equipment_base (Utilities|Casting|CastToModEquipment_Base Equipment)
    (:then
      (bind _array_element (Utilities|Array|ForEachLoopwithBreak (Variables|Default|GetAcceptsClasses) :!label _label)
        (:LoopBody
          (if (Utilities|ClassIsChildOf (Utilities|GetClass _asmod_equipment_base) _array_element)
            (LocalVariables|SettmpCanAccept true)
            (goto _label Break)))
        (:Completed
          (return (LocalVariables|GettmpCanAccept)))))
    (:CastFailed
      (return false))))

(fn GetCurrentEquipment
  (return (Variables|Default|GetMyModEquipment)))

(fn GetCurrentEquipmentID
  (bind _mymodequipment (Variables|Default|GetMyModEquipment))
  (bind _asmod_slot_cac_bp (Utilities|Casting|CastToModSlot_CAC_BP (Transformation|GetAttachParent (Variables|Default|GetScene)))
    (:then
      (return (Variables|/Script/FungusFarm.ModSlot_CAC|GetSlottedEquipmentID _asmod_slot_cac_bp)))
    (:CastFailed
      (return (select (Utilities|IsValid _mymodequipment) (Variables|/Game/FungusFarm/Blueprints/Equipment/Equipment_Base.Equipment_Base_C|GetMyID _mymodequipment) (LocalVariables|GettmpNullGUID))))))

(fn GetPlaceLocation
  (return (Transformation|GetWorldLocation (Variables|Default|GetModSpot))))

(fn HasEquipment?
  (return (Utilities|IsValid (Variables|Default|GetMyModEquipment))))