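; Base Blueprint for placeable lab equipment that crafts recipes and opens the lab equipment menu when clicked while placed and ready.
; A crafter component works from the goods inventory, takes allowed recipe categories from equipment data and serializes through SaveManager events.
; Tagged collision overlaps are counted as invalid during placement, and pickup transfers stored goods to the player's inventory.
; The HUD thumbnail shows the current recipe, falling back to the equipment's own.
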(event OnComponentBeginOverlap(EquipmentCollisionBox)
  (params (OverlappedComponent :type Primitive%20Component%20Object%20Reference) (OtherActor :type Actor%20Object%20Reference) (OtherComp :type Primitive%20Component%20Object%20Reference) (OtherBodyIndex :type Integer) (bFromSweep :type Boolean) (SweepResult :type Hit%20Result%20Structure%20%28by%20ref%29))
  (if (not (Variables|Default|GetPlaced))
    (if (not (== OtherActor self))
      (if (Components|ComponentHasTag OtherComp "EquipmentCollision")
        (Math|Integer|IncrementInt (Variables|Default|GetInvalidOverlaps))))))

(event OnComponentEndOverlap(EquipmentCollisionBox)
  (params (OverlappedComponent :type Primitive%20Component%20Object%20Reference) (OtherActor :type Actor%20Object%20Reference) (OtherComp :type Primitive%20Component%20Object%20Reference) (OtherBodyIndex :type Integer))
  (if (not (Variables|Default|GetPlaced))
    (if (not (== OtherActor self))
      (if (Components|ComponentHasTag OtherComp "EquipmentCollision")
        (Math|Integer|DecrementInt (Variables|Default|GetInvalidOverlaps))))))

(event OnClicked(EquipmentSprite)
  (params (TouchedComponent :type Primitive%20Component%20Object%20Reference) (ButtonPressed :type Key%20Structure))
  (if (and (Variables|Default|GetPlaced) (Variables|Default|GetReady))
    (bind _asff_player_controller_bp (Utilities|Casting|CastToFF_PlayerController_BP (Game|GetPlayerController 0)))
    (Default|ShowLabEquipmentMenu _asff_player_controller_bp self)))

(event EventBeginPlay
  (|CallParentFunction)
  (Default|SetInventory (Variables|Default|GetFF_ActorCrafter_Component) (Variables|Default|GetFF_GoodsInventory_Component))
  (Class|SaveManager|SubscribeforEvents (Subsystems|GetSaveManager) self)
  (CallFunction|UpdateSpriteAppearance))

(event EventOnPickupEquipment
  (bind (_valid_ _inventory) (CallFunction|GetPlayerInventory))
  (bind _ff_goodsinventory_component (Variables|Default|GetFF_GoodsInventory_Component))
  (Utilities|FlowControl|Sequence
    (:then_0
      (Utilities|IsValid _ff_goodsinventory_component
        (:Is%20Valid
          (if _valid_
            (Default|TransferAllGoodstoOther _ff_goodsinventory_component _inventory)))))
    (:then_1
      (|CallParentFunction))))

(event EventInitfromData
  (bind _equipmentdata (Variables|Default|GetEquipmentData))
  (bind _allowedrecipecategories (Utilities|Struct|BreakEquipmentType _equipmentdata))
  (|CallParentFunction)
  (if (> (Utilities|Array|Length _allowedrecipecategories) 0)
    (Variables|/Game/FungusFarm/Blueprints/Crafting/FF_ActorCrafter_Component.FF_ActorCrafter_Component_C|SetAllowedRecipeCategories (Variables|Default|GetFF_ActorCrafter_Component) _allowedrecipecategories)))

(event EventOnSaveBegan
  (Default|SavetoSerialized (Variables|Default|GetFF_ActorCrafter_Component)))

(event EventOnLoadFinished
  (params (bError :type Boolean))
  (Default|RefreshfromSerialized (Variables|Default|GetFF_ActorCrafter_Component))
  (CallFunction|RefreshReferences)
  (CallFunction|UpdateSpriteAppearance))

(fn ConstructionScript
  (|CallParentFunction))

(fn GetHudThumbnail
  (if (Default|CurrentRecipeIsValid? (Variables|Default|GetFF_ActorCrafter_Component))
    (return (.Thumbnail (Utilities|Struct|BreakCraftingRecipe (Variables|/Game/FungusFarm/Blueprints/Crafting/FF_ActorCrafter_Component.FF_ActorCrafter_Component_C|GetCurrentRecipe (Variables|Default|GetFF_ActorCrafter_Component)))))
    (else
      (return (.Thumbnail (Utilities|Struct|BreakEquipmentType (Variables|Default|GetEquipmentData)))))))