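; Base crop plot equipment that registers with the farm manager when placed and spawns, hosts and tracks one crop.
; Base stats from game state plot data feed modifiable attribute components, recalculated from child-actor mod slots whenever their equipment changes.
; Growth rate requires sufficient mineral and protein capacity and is penalized outside the crop's temperature and moisture tolerances.
; Crop events are forwarded to mod slots, and resume relinks the crop by GUID.
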(event OnClicked(EquipmentSprite)
  (params (TouchedComponent :type Primitive%20Component%20Object%20Reference) (ButtonPressed :type Key%20Structure))
  (if (Variables|Default|GetPlaced)
    (CallFunction|ShowPlotMenu)))

(event OnClicked(PlotGUI)
  (params (TouchedComponent :type Primitive%20Component%20Object%20Reference) (ButtonPressed :type Key%20Structure))
  (bind _mycrop (Variables|Plot|GetMyCrop))
  (Utilities|IsValid _mycrop
    (:Is%20Valid
      (if (Utilities|Enum|Equal(Enum) (Default|GetGrowState _mycrop) "NewEnumerator4")
        (Default|HandleClick _mycrop)))))

(event Resume(Lifetime)
  (CallFunction|Init)
  (CallFunction|RefreshReferences)
  (bind _asgrowth_progress_widget (Utilities|Casting|CastToGrowthProgressWidget (UserInterface|GetUserWidgetObject (Variables|Default|GetPlotGUI))))
  (Default|SetPlot _asgrowth_progress_widget self)
  (CallFunction|RefreshModifierCalculations)
  (CallFunction|UpdatePlotGUI))

(event OnComponentBeginOverlap(EquipmentCollisionBox)
  (params (OverlappedComponent :type Primitive%20Component%20Object%20Reference) (OtherActor :type Actor%20Object%20Reference) (OtherComp :type Primitive%20Component%20Object%20Reference) (OtherBodyIndex :type Integer) (bFromSweep :type Boolean) (SweepResult :type Hit%20Result%20Structure%20%28by%20ref%29))
  (if (not (Variables|Default|GetPlaced))
    (if (not (== OtherActor self))
      (if (Components|ComponentHasTag OtherComp "EquipmentCollision")
        (Math|Integer|IncrementInt (Variables|Default|GetInvalidOverlaps))))))

(event OnComponentEndOverlap(EquipmentCollisionBox)
  (params (OverlappedComponent :type Primitive%20Component%20Object%20Reference) (OtherActor :type Actor%20Object%20Reference) (OtherComp :type Primitive%20Component%20Object%20Reference) (OtherBodyIndex :type Integer))
  (if (not (Variables|Default|GetPlaced))
    (if (not (== OtherActor self))
      (if (Components|ComponentHasTag OtherComp "EquipmentCollision")
        (Math|Integer|DecrementInt (Variables|Default|GetInvalidOverlaps))))))

(event Custom|SetCrop
  (params (Is%20Planted? :type Boolean) (New%20Crop%20Data :type Crop%20Type%20Structure))
  (bind _self self)
  (Utilities|FlowControl|Sequence
    (:then_0
      (bind _output_get (Variables|Plot|SetSelectedCropData New%20Crop%20Data))
      (if (Utilities|Name|NotEqual(Name) (.Name (Utilities|Struct|BreakCropType _output_get)) "None")
        (bind _asff_game_state (Utilities|Casting|CastToFF_GameState (Game|GetGameState)))
        (bind _returnvalue (Game|SpawnActorfromClass (Default|ClassforCropName _asff_game_state (.Name (Utilities|Struct|BreakCropType _output_get))) (Math|Transform|MakeTransform (Transformation|GetWorldLocation (Variables|Default|GetCropSpot))) "AlwaysSpawn" _self _self (Variables|Default|GetMyID) (Variables|Plot|GetSelectedCropData) 0))
        (Variables|Plot|SetMyCrop _returnvalue)
        (Transformation|AttachComponentToComponent _returnvalue (Variables|Default|GetCropSpot) "None" "SnapToTarget" "KeepRelative" "KeepRelative" true)))
    (:then_1
      (if Is%20Planted?
        (Default|SetGrowState (Variables|Plot|GetMyCrop) "NewEnumerator1")
        (else
          (Default|SetGrowState (Variables|Plot|GetMyCrop) "NewEnumerator5"))))))

(event Custom|DispatchOnModifierPlaced
  (params (Mod%20Slot :type Mod%20Slot%20Object%20Reference) (Added%20Mod%20Equipment :type Mod%20Equipment%20Base%20Object%20Reference))
  (CallFunction|RefreshModifierCalculations))

(event Custom|DispatchOnModiferRemoved
  (params (Mod%20Slot :type Mod%20Slot%20Object%20Reference))
  (CallFunction|RefreshModifierCalculations))

(event Custom|DispatchOnModifierStateChanged
  (params (Slot :type Mod%20Slot%20Object%20Reference) (ModEquipment :type Mod%20Equipment%20Base%20Object%20Reference))
  (CallFunction|RefreshModifierCalculations))

(event Custom|OnCropPlanted
  (bind _mod_slots (CallFunction|GetModSlots))
  (for _array_element _mod_slots
    (Default|NotifyModEquipmentEvent _array_element "CropPlanted")))

(event Custom|OnCropReadyToHarvest
  (bind _mod_slots (CallFunction|GetModSlots))
  (for _array_element _mod_slots
    (Default|NotifyModEquipmentEvent _array_element "ReadyToHarvest")))

(event Custom|OnCropHarvested
  (bind _mod_slots (CallFunction|GetModSlots))
  (for _array_element _mod_slots
    (Default|NotifyModEquipmentEvent _array_element "Harvested")))

(event EventBeginPlay
  (|CallParentFunction)
  (Utilities|FlowControl|Sequence
    (:then_1
      (bind _asgrowth_progress_widget (Utilities|Casting|CastToGrowthProgressWidget (UserInterface|GetUserWidgetObject (Variables|Default|GetPlotGUI))))
      (Default|SetPlot _asgrowth_progress_widget self))
    (:then_2
      (bind _mod_slots (CallFunction|GetModSlots))
      (for _array_element _mod_slots
        (EventDispatchers|BindEventtoOnModifierEquipmentPlaced _array_element (delegate Custom|DispatchOnModifierPlaced))
        (EventDispatchers|BindEventtoOnModifierEquipmentRemoved _array_element (delegate Custom|DispatchOnModiferRemoved))
        (EventDispatchers|BindEventtoOnModifierEquipmentStateChanged _array_element (delegate Custom|DispatchOnModifierStateChanged))))
    (:then_3
      (CallFunction|RefreshModifierCalculations))))

(event EventOnPickupEquipment
  (bind _mod_slots (CallFunction|GetModSlots))
  (for _array_element _mod_slots
    (Default|RemoveModEquipment _array_element))
  (bind _asff_game_state (Utilities|Casting|CastToFF_GameState (Game|GetGameState)))
  (bind _currentfarmmanager (Default|GetFarmManager _asff_game_state))
  (Default|RemoveCropfromPlot _currentfarmmanager self)
  (|CallParentFunction)
  (Default|RemovePlot _currentfarmmanager self))

(event EventInitfromData
  (|CallParentFunction)
  (CallFunction|Init))

(event EventOnPlaceEquipment
  (|CallParentFunction)
  (if (Variables|Default|GetPlaced)
    (bind _asff_game_state (Utilities|Casting|CastToFF_GameState (Game|GetGameState)))
    (Default|AddPlot (Variables|/Game/FungusFarm/Blueprints/FF_GameState.FF_GameState_C|GetCurrentFarmManager _asff_game_state) self)))

(fn ConstructionScript
  (|CallParentFunction))

(fn ShowPlotMenu
  (if (Variables|Default|GetPlaced)
    (bind _asff_player_controller_bp (Utilities|Casting|CastToFF_PlayerController_BP (Game|GetPlayerController 0)))
    (Default|ShowCropPlotMgmt _asff_player_controller_bp self)))

(fn UpdatePlotGUI
  (bind _mycrop (Variables|Plot|GetMyCrop))
  (bind _asgrowth_progress_widget (Utilities|Casting|CastToGrowthProgressWidget (UserInterface|GetUserWidgetObject (Variables|Default|GetPlotGUI))))
  (Utilities|IsValid (Variables|Plot|GetMyCrop)
    (:Is%20Valid
      (Utilities|FlowControl|Sequence
        (:then_0
          ;[1 1 1] Display as Percent
          (Utilities|IsValid (Variables|Plot|GetMyCrop)
            (:Is%20Valid
              (Default|SetProgressPercent _asgrowth_progress_widget (/ (Variables|/Game/FungusFarm/Blueprints/Crops/CropBase_BP.CropBase_BP_C|GetCurrentGrowth _mycrop) (.GrowthTime (Utilities|Struct|BreakCropType (Variables|/Game/FungusFarm/Blueprints/Crops/CropBase_BP.CropBase_BP_C|GetCrop%20Data _mycrop))))))
            (:Is%20Not%20Valid
              (Default|SetProgressPercent _asgrowth_progress_widget 0.0))))))
    (:Is%20Not%20Valid
      (Default|SetProgressPercent _asgrowth_progress_widget 0.0))))

(fn CanAcceptCrop?
  (params (Crop :type Crop%20Type%20Structure))
  (bind (_name _displayname _thumbnail _thumbnailhardref _actorclass _plantingcost _harvestgoods _harvestgoodsbonus _sprinklegoods _growthtime _idealtemperature _temperaturetoleracerange _idealmoisture _moisturetoleracerange _requiredmineralcapacity _requiredproteincapacity) (Utilities|Struct|BreakCropType Crop))
  (return (and (>= (CallFunction|GetMineralCapacity) _requiredmineralcapacity) (>= (CallFunction|GetProteinCapacity) _requiredproteincapacity))))

(fn GetCropModifiers
  (return 0.0 "NewEnumerator0" "NewEnumerator0" (Variables|Plot|GetCachedCropModifiers)))

(fn Init
  (bind _equipmentdata (Variables|Default|GetEquipmentData))
  (bind _subtypename (Utilities|Struct|BreakEquipmentType _equipmentdata))
  (if (Utilities|Name|NotEqual(Name) (.Name (Utilities|Struct|BreakEquipmentType (Variables|Default|GetEquipmentData))) "None")
    (bind _asff_game_state (Utilities|Casting|CastToFF_GameState (Game|GetGameState)))
    (if (.Found? (Default|GetCropPlotData _asff_game_state _subtypename))
      (bind _output_get (Variables|Plot|SetCropPlotData (.Crop%20Plot%20Info (Default|GetCropPlotData _asff_game_state _subtypename))))
      (Class|ModifiableAttributeAC|SetBaseValue (Variables|Default|GetmattrGrowthRate) (.BaseGrowthRate (Utilities|Struct|BreakCropPlotInfo _output_get)))
      (Class|ModifiableAttributeAC|SetBaseValue (Variables|Default|GetmattrTemperature) (.BaseTemperature (Utilities|Struct|BreakCropPlotInfo _output_get)))
      (Class|ModifiableAttributeAC|SetBaseValue (Variables|Default|GetmattrMoisture) (.BaseMoisture (Utilities|Struct|BreakCropPlotInfo _output_get)))
      (Class|ModifiableAttributeAC|SetBaseValue (Variables|Default|GetmattrMineralCapacity) (.BaseMineralCapacity (Utilities|Struct|BreakCropPlotInfo _output_get)))
      (Class|ModifiableAttributeAC|SetBaseValue (Variables|Default|GetmattrProteinCapacity) (.BaseProteinCapacity (Utilities|Struct|BreakCropPlotInfo _output_get)))
      (else
        (Development|PrintString (Utilities|String|Append "No data found for CropPlot type:  " (Utilities|String|ToString(Name) _subtypename) " Using defaults.") true true "(R=1.000000,G=0.007843,B=0.000000,A=1.000000)" 1e+01)))))

(fn RefreshReferences
  (|CallParentFunction)
  (bind _outactors (Actor|GetAllActorsOfClass "/Game/FungusFarm/Blueprints/Crops/CropBase_BP.CropBase_BP_C"))
  (bind _array_element (Utilities|Array|ForEachLoopwithBreak _outactors :!label _label)
    (:LoopBody
      (if (and (Guid|IsValidGuid (Variables|/Game/FungusFarm/Blueprints/Crops/CropBase_BP.CropBase_BP_C|GetMyPlotsID _array_element)) (== (Variables|/Game/FungusFarm/Blueprints/Crops/CropBase_BP.CropBase_BP_C|GetMyPlotsID _array_element) (Variables|Default|GetMyID)))
        (Variables|Plot|SetMyCrop _array_element)
        ;[1 1 1] Also update the reverse reference in the crop
        (Variables|/Game/FungusFarm/Blueprints/Crops/CropBase_BP.CropBase_BP_C|SetMyPlot _array_element self)
        (goto _label Break)))
    (:Completed
      (return true))))

(fn ModifiableAttributebyCode
  (params (AttributeCode :type Name))
  (bind _array_element (Utilities|Array|ForEachLoopwithBreak (Actor|GetComponentsByClass "/Script/FungusFarm.ModifiableAttribute_AC") :!label _label)
    (:LoopBody
      (if (Utilities|Name|Equal(Name) (Variables|/Script/FungusFarm.ModifiableAttribute_AC|GetAttributeCode _array_element) AttributeCode)
        (LocalVariables|SettmpAttribute _array_element)
        (goto _label Break)))
    (:Completed
      (return (LocalVariables|GettmpAttribute) (Utilities|IsValid (LocalVariables|GettmpAttribute))))))

(fn AllowAutoHarvest?
  (return (> (Class|ModifiableAttributeAC|GetCurrentValue (Variables|Default|GetmattrAutoHarvest)) 0.0)))

(fn AllowAutoReplant?
  (return (> (Class|ModifiableAttributeAC|GetCurrentValue (Variables|Default|GetmattrAutoReplant)) 0.0)))

(fn GetTemperature
  (return (Class|ModifiableAttributeAC|GetCurrentValue (Variables|Default|GetmattrTemperature))))

(fn GetMoisture
  (return (Class|ModifiableAttributeAC|GetCurrentValue (Variables|Default|GetmattrMoisture))))

(fn GetCalculatedGrowthRate
  (return (CallFunction|GetCalculatedGrowthRateforCrop (Variables|Plot|GetSelectedCropData))))

(fn GetCalculatedGrowthRateforCrop
  (params (CropType :type Crop%20Type%20Structure%20%28by%20ref%29))
  (bind (_name _displayname _thumbnail _thumbnailhardref _actorclass _plantingcost _harvestgoods _harvestgoodsbonus _sprinklegoods _growthtime _idealtemperature _temperaturetoleracerange _idealmoisture _moisturetoleracerange _requiredmineralcapacity _requiredproteincapacity) (Utilities|Struct|BreakCropType CropType))
  (if (Math|Boolean|ANDBoolean (Utilities|Name|NotEqual(Name) _name "None") (>= (CallFunction|GetMineralCapacity) _requiredmineralcapacity) (>= (CallFunction|GetProteinCapacity) _requiredproteincapacity))
    (return (* (Class|ModifiableAttributeAC|GetCurrentValue (Variables|Default|GetmattrGrowthRate)) (* (select (> (Math|Float|Absolute(Float) (- (CallFunction|GetTemperature) _idealtemperature)) _temperaturetoleracerange) 0.1 1.0) (select (> (Math|Float|Absolute(Float) (- (CallFunction|GetMoisture) _idealmoisture)) _moisturetoleracerange) 0.1 1.0))))
    (else
      (return 0.0))))

(fn GetMineralCapacity
  (return (Class|ModifiableAttributeAC|GetCurrentValue (Variables|Default|GetmattrMineralCapacity))))

(fn GetProteinCapacity
  (return (Class|ModifiableAttributeAC|GetCurrentValue (Variables|Default|GetmattrProteinCapacity))))

(fn GetModSlots
  (LocalVariables|SettmpModSlots (Utilities|Array|MakeArray))
  (for _array_element (Actor|GetComponentsByClass "/Game/FungusFarm/Blueprints/Equipment/EquipmentMods/ModSlot_CAC_BP.ModSlot_CAC_BP_C")
    (bind _asmod_slot (Utilities|Casting|CastToModSlot (Variables|/Script/Engine.ChildActorComponent|GetChildActor _array_element)))
    (Utilities|Array|Add (LocalVariables|GettmpModSlots) _asmod_slot))
  (return (LocalVariables|GettmpModSlots)))

(fn RefreshModifierCalculations
  (Utilities|Array|Clear (Variables|Plot|GetCachedCropModifiers))
  (Utilities|FlowControl|Sequence
    (:then_0
      (bind _mod_slots (CallFunction|GetModSlots))
      (for _array_element _mod_slots
        (bind _modifiers (Default|GetAllModifiers _array_element))
        (Utilities|Array|AppendArray (Variables|Plot|GetCachedCropModifiers) _modifiers)))
    (:then_1
      (for _array_element_2 (Actor|GetComponentsByClass "/Script/FungusFarm.ModifiableAttribute_AC")
        (Class|ModifiableAttributeAC|ClearModifiers _array_element_2)
        (Class|ModifiableAttributeAC|AddModifiers _array_element_2 (Variables|Plot|GetCachedCropModifiers)))
      (Default|CallOnModifiersRefreshed)
      (return (Variables|Plot|GetCachedCropModifiers)))))