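; GlobalManager_BP is a manager that filters global effects by tags and places spirit totems in the world.
; GetValidEffectsForTags keeps effects whose required tags are all present and denied tags all absent.
; AddTotem finds a single empty SpiritTotem_Target tagged with the totem name, then spawns its sole accepted class using FF_GameState equipment data.
; The spawned totem is registered as placed and starts tracking its level-zero upgrade recipe.
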(event EventBeginPlay)

(event Collision|EventActorBeginOverlap
  (params (OtherActor :type Actor%20Object%20Reference)))

(event EventTick
  (params (DeltaSeconds :type Float%20%28single-precision%29)))

(fn ConstructionScript)

(fn EffectValidforTags
  (params (GlobalEffectToCheck :type Global%20Effect%20Structure%20%28by%20ref%29) (GlobalEffectsTags :type Array%20of%20Names))
  (bind (_displayname _uniquename _thumbnail _requiredtags _deniedtags) (Utilities|Struct|BreakGlobalEffect GlobalEffectToCheck))
  (LocalVariables|SettmpGlobalEffectsTags GlobalEffectsTags)
  (LocalVariables|SettmpTagsValid true)
  (bind _array_element (Utilities|Array|ForEachLoopwithBreak _requiredtags :!label _label)
    (:LoopBody
      (if (not (Utilities|Array|ContainsItem (LocalVariables|GettmpGlobalEffectsTags) _array_element))
        (LocalVariables|SettmpTagsValid false)
        (goto _label Break)))
    (:Completed
      (if (LocalVariables|GettmpTagsValid)
        (bind _array_element_2 (Utilities|Array|ForEachLoopwithBreak _deniedtags :!label _label_2)
          (:LoopBody
            (if (Utilities|Array|ContainsItem (LocalVariables|GettmpGlobalEffectsTags) _array_element_2)
              (LocalVariables|SettmpTagsValid false)
              (goto _label_2 Break)))
          (:Completed
            (return (LocalVariables|GettmpTagsValid))))
        (else
          (return (LocalVariables|GettmpTagsValid)))))))

(fn GetValidEffectsforTags
  (params (GlobalEffectsTags :type Array%20of%20Names))
  (for _array_element (Class|GlobalManager|GetGlobalEffects)
    (if (CallFunction|EffectValidforTags _array_element GlobalEffectsTags)
      (Utilities|Array|Add (LocalVariables|GettmpValidEffects) _array_element)))
  (return (LocalVariables|GettmpValidEffects)))

(fn AddTotem
  (params (TotemName :type Name))
  (bind _outactors (Actor|GetAllActorsOfClasswithTag "/Game/FungusFarm/Blueprints/Equipment/SpiritTotems/SpiritTotem_Target.SpiritTotem_Target_C" TotemName))
  (if (== (Utilities|Array|Length _outactors) 1)
    (bind _output_get (LocalVariables|SettmpTotemTarget (Utilities|Array|Get(acopy) _outactors)))
    (bind _hasequipment (Default|HasEquipment? _output_get))
    (if (not _hasequipment)
      (if (== (Utilities|Array|Length (Variables|/Game/FungusFarm/Blueprints/Equipment/PlaceableEquipmentTarget_BP.PlaceableEquipmentTarget_BP_C|GetAcceptsClasses (LocalVariables|GettmpTotemTarget))) 1)
        (bind _asff_game_state (Utilities|Casting|CastToFF_GameState (Game|GetGameState)))
        (if (.Found (Default|GetEquipmentData _asff_game_state TotemName))
          (bind _location (Default|GetPlaceLocation (LocalVariables|GettmpTotemTarget)))
          (bind _returnvalue (Game|SpawnActorfromClass (Utilities|Array|Get(acopy) (Variables|/Game/FungusFarm/Blueprints/Equipment/PlaceableEquipmentTarget_BP.PlaceableEquipmentTarget_BP_C|GetAcceptsClasses (LocalVariables|GettmpTotemTarget))) (Math|Transform|MakeTransform _location) "AdjustIfPossibleButAlwaysSpawn" 0 (.Equipment%20Data (Default|GetEquipmentData _asff_game_state TotemName)) 0))
          (Variables|/Game/FungusFarm/Blueprints/Equipment/PlaceableEquipment_Base.PlaceableEquipment_Base_C|SetValidLocation _returnvalue true)
          (Variables|/Game/FungusFarm/Blueprints/Equipment/PlaceableEquipment_Base.PlaceableEquipment_Base_C|SetCurrentPlaceableTarget _returnvalue (LocalVariables|GettmpTotemTarget))
          (Default|OnPlaceEquipment _returnvalue)
          (bind _asspirit_totem_base_bp (Utilities|Casting|CastToSpiritTotemBase_BP _returnvalue))
          (Default|TrackLevelUpRecipeforTotemLevel _asspirit_totem_base_bp))))))