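; A placement target for farm equipment that records which equipment occupies it and shows a sprite while empty.
; Placement and removal events set or clear the current equipment reference and its ID, hiding or showing the PaperSprite to match.
; The acceptance check passes any PlaceableEquipment_Base without testing whether the target is already occupied, and a getter exposes the current ID.
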(event EventOnEquipmentRemoved
  (params (Removed%20Equipment :type I%20Placeable%20Equipment%20Interface))
  (Variables|Default|SetCurrentEquipmentID "")
  (Variables|Default|SetCurrentEquipment 0)
  (Rendering|SetVisibility (Variables|Default|GetPaperSprite) true false))

(event EventOnEquipmentPlaced
  (params (Placed%20Equipment :type I%20Placeable%20Equipment%20Interface))
  (bind _id (Default|GetEquipmentID Placed%20Equipment))
  (Variables|Default|SetCurrentEquipmentID _id)
  (Variables|Default|SetCurrentEquipment Placed%20Equipment)
  (Rendering|SetVisibility (Variables|Default|GetPaperSprite) false false))

(fn ConstructionScript)

(fn CanAcceptEquipment?
  (params (Equipment :type Equipment%20Base%20Object%20Reference))
  (Utilities|Casting|CastToPlaceableEquipment_Base Equipment
    (:then
      (return true))
    (:CastFailed
      (return false))))

(fn GetCurrentEquipmentID
  (return (Variables|Default|GetCurrentEquipmentID)))