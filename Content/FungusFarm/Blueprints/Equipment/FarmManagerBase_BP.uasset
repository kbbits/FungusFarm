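; Farm manager base that drives crop growth, planting and replanting for every crop plot in the level.
; It gathers plots on BeginPlay and game load, then a looping timer, paused with the game, ticks each crop.
; Each tick carries leftover time through growth stages, auto-harvesting and auto-replanting where plots allow it.
; Planting costs come from the player's inventory, and per-crop production rates are summed across plots.
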(event Custom|DestroyCrop
  (params (Crop :type Crop%20Base%20BP%20Object%20Reference))
  (Actor|DestroyActor Crop))

(event Custom|ReplantPlot
  (params (Plot :type Crop%20Plot%20Base%20BP%20Object%20Reference))
  (CallFunction|DoReplantPlotifUnplanted Plot))

(event Custom|OnGameLoaded
  (params (SlotInfo :type Slot%20Info%20Object%20Reference))
  (Utilities|FlowControl|Sequence
    (:then_0
      ;[1 1 1] Init self first
      (CallFunction|InitfromData))
    (:then_1)
    (:then_2
      ;[1 1 1 1 16] Refresh Plot references and each Crop Plot's references. Plots will refresh their own equipped mods
      (CallFunction|RefreshPlotReferences))))

(event Custom|OnGamePaused
  (CallFunction|Pause))

(event Custom|OnGameUnpaused
  (CallFunction|Unpause))

(event EventBeginPlay
  (Utilities|FlowControl|Sequence
    (:then_0
      (bind _asff_game_state (Utilities|Casting|CastToFF_GameState (Game|GetGameState)))
      (EventDispatchers|BindEventtoOnGamePaused _asff_game_state (delegate Custom|OnGamePaused))
      (EventDispatchers|BindEventtoOnGameUnPaused _asff_game_state (delegate Custom|OnGameUnpaused)))
    (:then_1
      (CallFunction|InitfromData)
      (EventDispatchers|BindEventtoOnGameLoaded (Subsystems|GetSaveManager) (delegate Custom|OnGameLoaded)))
    (:then_2
      (CallFunction|RefreshPlotReferences))
    (:then_3
      ;[1 1 1] Setup grow timer
      (bind _returnvalue (Utilities|Time|SetTimerbyFunctionName 0 "GrowTick" 0.2 true))
      (Variables|Default|SetGrowTimer _returnvalue))))

(event EventInitfromData)

(event EventEndPlay
  (params (EndPlayReason :type EEndPlayReason%20Enum :default "Destroyed"))
  (Utilities|Time|ClearandInvalidateTimerbyHandle (Variables|Default|GetGrowTimer))
  (bind _asff_game_state (Utilities|Casting|CastToFF_GameState (Game|GetGameState)))
  (EventDispatchers|UnbindEventfromOnGamePaused _asff_game_state (delegate Custom|OnGamePaused))
  (EventDispatchers|UnbindEventfromOnGameUnPaused _asff_game_state (delegate Custom|OnGameUnpaused)))

(fn ConstructionScript)

(fn GrowTick
  (LocalVariables|SettmpDeltaTime (Class|KismetSystemLibrary|GetTimerElapsedTimeHandle (Variables|Default|GetGrowTimer)))
  (for _array_element (Variables|Default|GetPlots)
    (bind _output_get (LocalVariables|SettmpPlot _array_element))
    (LocalVariables|SettmpCropRemainingTime (LocalVariables|GettmpDeltaTime))
    (Utilities|FlowControl|Sequence :!label _label
      (:then_0
        (Utilities|IsValid (Variables|/Game/FungusFarm/Blueprints/Equipment/CropPlots/CropPlotBase_BP.CropPlotBase_BP_C|GetMyCrop (LocalVariables|GettmpPlot))
          (:Is%20Valid
            (bind _remaining_time (Default|GrowthTick (Variables|/Game/FungusFarm/Blueprints/Equipment/CropPlots/CropPlotBase_BP.CropPlotBase_BP_C|GetMyCrop (LocalVariables|GettmpPlot)) (LocalVariables|GettmpCropRemainingTime)))
            (LocalVariables|SettmpCropRemainingTime _remaining_time))))
      (:then_1
        (Utilities|IsValid (Variables|/Game/FungusFarm/Blueprints/Equipment/CropPlots/CropPlotBase_BP.CropPlotBase_BP_C|GetMyCrop (LocalVariables|GettmpPlot))
          (:Is%20Valid
            (if (Utilities|Enum|Equal(Enum) (Default|GetGrowState (Variables|/Game/FungusFarm/Blueprints/Equipment/CropPlots/CropPlotBase_BP.CropPlotBase_BP_C|GetMyCrop (LocalVariables|GettmpPlot))) "NewEnumerator4")
              (if (Default|AllowAutoHarvest? (LocalVariables|GettmpPlot))
                (Default|Harvest (Variables|/Game/FungusFarm/Blueprints/Equipment/CropPlots/CropPlotBase_BP.CropPlotBase_BP_C|GetMyCrop (LocalVariables|GettmpPlot))))))))
      (:then_2
        (if (Default|AllowAutoReplant? _output_get)
          (CallFunction|DoReplantPlotifUnplanted _output_get)))
      (:then_3
        (Utilities|IsValid (Variables|/Game/FungusFarm/Blueprints/Equipment/CropPlots/CropPlotBase_BP.CropPlotBase_BP_C|GetMyCrop _output_get)
          (:Is%20Valid
            (switch Utilities|FlowControl|Switch|SwitchonCropGrowState (Default|GetGrowState (Variables|/Game/FungusFarm/Blueprints/Equipment/CropPlots/CropPlotBase_BP.CropPlotBase_BP_C|GetMyCrop _output_get))
              (:NewEnumerator1
                _)
              (:NewEnumerator0
                _))
            (if (> (LocalVariables|GettmpCropRemainingTime) 0.0)
              (goto _label))))))))

(fn PlantCropinPlot
  (params (Crop%20Data :type Crop%20Type%20Structure) (Plot :type Crop%20Plot%20Base%20BP%20Object%20Reference))
  (bind (_valid_ _inventory) (CallFunction|GetPlayerInventory))
  (Utilities|FlowControl|Sequence
    (:then_0
      (if _valid_
        (bind _successful (Default|RemoveGoodsInventoryBatch _inventory (.PlantingCost (Utilities|Struct|BreakCropType Crop%20Data))))
        (LocalVariables|SetpaidPlanted? _successful)))
    (:then_1
      (Utilities|IsValid (Variables|/Game/FungusFarm/Blueprints/Equipment/CropPlots/CropPlotBase_BP.CropPlotBase_BP_C|GetMyCrop Plot)
        (:Is%20Valid
          (CallFunction|RemoveCropfromPlot Plot))))
    (:then_2
      (Default|SetCrop Plot (LocalVariables|GetpaidPlanted?) Crop%20Data)
      (if (LocalVariables|GetpaidPlanted?)
        (Default|OnCropPlanted Plot)))))

(fn RemoveCropfromPlot
  (params (Plot :type Crop%20Plot%20Base%20BP%20Object%20Reference))
  (Utilities|IsValid (Variables|/Game/FungusFarm/Blueprints/Equipment/CropPlots/CropPlotBase_BP.CropPlotBase_BP_C|GetMyCrop Plot)
    (:Is%20Valid
      (CallFunction|DestroyCrop (Variables|/Game/FungusFarm/Blueprints/Equipment/CropPlots/CropPlotBase_BP.CropPlotBase_BP_C|GetMyCrop Plot))
      (Variables|/Game/FungusFarm/Blueprints/Equipment/CropPlots/CropPlotBase_BP.CropPlotBase_BP_C|SetMyCrop Plot 0)
      (Variables|/Game/FungusFarm/Blueprints/Equipment/CropPlots/CropPlotBase_BP.CropPlotBase_BP_C|SetSelectedCropData Plot ""))))

(fn CalculatedProductionRates
  (for _array_element (Variables|Default|GetPlots)
    (Utilities|IsValid (Variables|/Game/FungusFarm/Blueprints/Equipment/CropPlots/CropPlotBase_BP.CropPlotBase_BP_C|GetMyCrop _array_element)
      (:Is%20Valid
        (bind _rates (Default|CalculatedProductionRates (Variables|/Game/FungusFarm/Blueprints/Equipment/CropPlots/CropPlotBase_BP.CropPlotBase_BP_C|GetMyCrop _array_element)))
        (bind _total_inventory (CallFunction|SumInventories (LocalVariables|GettmpRates) _rates))
        (LocalVariables|SettmpRates _total_inventory))))
  (return (LocalVariables|GettmpRates)))

(fn Pause
  (Utilities|Time|PauseTimerbyHandle (Variables|Default|GetGrowTimer)))

(fn Unpause
  (if (Class|KismetSystemLibrary|IsTimerPausedHandle (Variables|Default|GetGrowTimer))
    (Utilities|Time|UnpauseTimerbyHandle (Variables|Default|GetGrowTimer))))

(fn AddPlot
  (params (Plot :type Crop%20Plot%20Base%20BP%20Object%20Reference))
  (Utilities|Array|AddUnique (Variables|Default|GetPlots) Plot))

(fn DoReplantPlotifUnplanted
  (params (Plot :type Crop%20Plot%20Base%20BP%20Object%20Reference))
  (bind (_valid_ _inventory) (CallFunction|GetPlayerInventory))
  (bind _output_get (LocalVariables|SettmpPlot Plot))
  (if (Utilities|Name|NotEqual(Name) (.Name (Utilities|Struct|BreakCropType (Variables|/Game/FungusFarm/Blueprints/Equipment/CropPlots/CropPlotBase_BP.CropPlotBase_BP_C|GetSelectedCropData _output_get))) "None")
    (Utilities|IsValid (Variables|/Game/FungusFarm/Blueprints/Equipment/CropPlots/CropPlotBase_BP.CropPlotBase_BP_C|GetMyCrop (LocalVariables|GettmpPlot))
      (:Is%20Valid
        (if (Utilities|Enum|Equal(Enum) (Default|GetGrowState (Variables|/Game/FungusFarm/Blueprints/Equipment/CropPlots/CropPlotBase_BP.CropPlotBase_BP_C|GetMyCrop (LocalVariables|GettmpPlot))) "NewEnumerator5")
          (if _valid_ :!label _label
            (bind _successful (Default|RemoveGoodsInventoryBatch _inventory (.PlantingCost (Utilities|Struct|BreakCropType (Variables|/Game/FungusFarm/Blueprints/Equipment/CropPlots/CropPlotBase_BP.CropPlotBase_BP_C|GetSelectedCropData _output_get)))))
            (Utilities|IsValid (Variables|/Game/FungusFarm/Blueprints/Equipment/CropPlots/CropPlotBase_BP.CropPlotBase_BP_C|GetMyCrop (LocalVariables|GettmpPlot))
              (:Is%20Valid
                (if _successful
                  (Default|SetGrowState (Variables|/Game/FungusFarm/Blueprints/Equipment/CropPlots/CropPlotBase_BP.CropPlotBase_BP_C|GetMyCrop (LocalVariables|GettmpPlot)) "NewEnumerator1")
                  (Default|OnCropPlanted (LocalVariables|GettmpPlot) :!label _label_2)))
              (:Is%20Not%20Valid
                (Default|SetCrop (LocalVariables|GettmpPlot) _successful (Variables|/Game/FungusFarm/Blueprints/Equipment/CropPlots/CropPlotBase_BP.CropPlotBase_BP_C|GetSelectedCropData (LocalVariables|GettmpPlot)))
                (if _successful
                  (goto _label_2)))))))
      (:Is%20Not%20Valid
        (goto _label)))))

(fn RefreshPlotReferences
  ;[1 1 1] Find all plots
  (Variables|Default|SetPlots (Utilities|Array|MakeArray))
  (bind _outactors (Actor|GetAllActorsOfClass "/Game/FungusFarm/Blueprints/Equipment/CropPlots/CropPlotBase_BP.CropPlotBase_BP_C"))
  (for _array_element _outactors
    (CallFunction|AddPlot _array_element)))

(fn RemovePlot
  (params (Plot :type Crop%20Plot%20Base%20BP%20Object%20Reference))
  (Utilities|Array|RemoveItem (Variables|Default|GetPlots) Plot))

(fn FillTestVar
  (bind _asff_game_state (Utilities|Casting|CastToFF_GameState (Game|GetGameState)))
  (bind _unlocked_crops (Default|GetAllUnlockedCropData _asff_game_state))
  (bind _output_get (LocalVariables|SettmpColor (Utilities|Struct|MakeLinearColor (Math|Random|RandomFloat) (Math|Random|RandomFloat) (Math|Random|RandomFloat) 1.0)))
  (Development|PrintString (Utilities|String|Append "Added: " (Utilities|String|ToString(Name) (.Name (Utilities|Struct|BreakCropType (Utilities|Array|Get(acopy) _unlocked_crops))))) true true _output_get)
  (Utilities|Array|Add (Variables|Default|GetTestStructVar) (LocalVariables|GettmpColor))
  (Utilities|Array|Add (Variables|Default|GetCrafting%20Slots%20Test%20Var) (Utilities|Struct|MakeCraftingSlot (.Name (Utilities|Struct|BreakCropType (Utilities|Array|Get(acopy) _unlocked_crops))) (Math|Float|Truncate (.GrowthTime (Utilities|Struct|BreakCropType (Utilities|Array|Get(acopy) _unlocked_crops)))))))

(fn InspectTestVar
  (bind _tmpdebugstrings (LocalVariables|GettmpDebugStrings))
  (Utilities|FlowControl|Sequence
    (:then_0
      (Development|PrintString "Items in CraftingSlot TestVar" true true "(R=0.000000,G=0.660000,B=1.000000,A=1.000000)" 5.0)
      (for (_array_element _array_index) (Variables|Default|GetCrafting%20Slots%20Test%20Var)
        (Utilities|Array|Clear (LocalVariables|GettmpDebugStrings))
        (Utilities|Array|Add _tmpdebugstrings (Utilities|String|ToString(Name) (.Name (Utilities|Struct|BreakCraftingSlot _array_element))))
        (Utilities|Array|Add _tmpdebugstrings (Utilities|String|Append ": " (Utilities|String|ToString(Integer) (.Value (Utilities|Struct|BreakCraftingSlot _array_element)))))
        (Development|PrintString (Utilities|String|JoinStringArray (LocalVariables|GettmpDebugStrings) " 
") true true (Utilities|Array|Get(acopy) (Variables|Default|GetTestStructVar) _array_index) 5.0)))))