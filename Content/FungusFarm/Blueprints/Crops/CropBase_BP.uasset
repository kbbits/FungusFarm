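; Base crop for the farm: grows on a plot, consumes player goods, and is clicked to replant, collect sprinkles or harvest.
; GrowthTick carries time through warmup and growth, drawing proportional CropData inputs via InputsTick and stalling when inventory is busy or short.
; SetGrowState fires per-state hooks and refreshes crop and plot visuals.
; Harvest adds goods, totals and XP, with particle bursts textured from goods thumbnails.
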(event OnClicked(CropSprite)
  (params (TouchedComponent :type Primitive%20Component%20Object%20Reference) (ButtonPressed :type Key%20Structure))
  (CallFunction|HandleClick))

(event Custom|OnGrowthComplete
  (params (Old%20Grow%20State :type CropGrowState%20Enum :default "NewEnumerator5"))
  (Default|OnCropReadytoHarvest (Variables|Default|GetMyPlot)))

(event Custom|OnInputInventoryBusy
  (params (OldGrowState :type CropGrowState%20Enum :default "NewEnumerator5")))

(event Custom|OnUnplanted
  (params (Old%20Grow%20State :type CropGrowState%20Enum :default "NewEnumerator5")))

(event Custom|OnWarmupStart
  (params (OldGrowState :type CropGrowState%20Enum :default "NewEnumerator5")))

(event Custom|OnGrowthStart
  (params (OldGrowState :type CropGrowState%20Enum :default "NewEnumerator5")))

(event Custom|OnStarveStart
  (params (OldGrowState :type CropGrowState%20Enum :default "NewEnumerator5")))

(event EventBeginPlay)

(fn ConstructionScript)

(fn Harvest
  (bind (_harvest_goods _bonus_goods) (CallFunction|CalculateHarvestAmount))
  (bind (_valid_ _inventory) (CallFunction|GetPlayerInventory))
  (bind _myplot (Variables|Default|GetMyPlot))
  (Utilities|FlowControl|Sequence
    (:then_0
      (LocalVariables|SettmpHarvestGoods _harvest_goods)
      (LocalVariables|SettmpBonusGoods _bonus_goods)
      (if (> (+ (Utilities|Array|Length (LocalVariables|GettmpHarvestGoods)) (Utilities|Array|Length (LocalVariables|GettmpBonusGoods))) 0)
        (Audio|PlaySoundatLocation (Utilities|Select :Index (select (> (+ (Utilities|Array|Length (LocalVariables|GettmpHarvestGoods)) (Utilities|Array|Length (LocalVariables|GettmpBonusGoods))) 1) 1 0) :Option%200 "/Game/FungusFarm/Assets/Sound/Effects/PopShort_01.PopShort_01" :Option%201 "/Game/FungusFarm/Assets/Sound/Effects/Pops_01.Pops_01") (Transformation|GetWorldLocation (Variables|Default|GetSprinkleBox)) "0, 0, 0" 1.0 1.0 0.0 0 0 self)))
    (:then_1
      (CallFunction|DropSprinkles (LocalVariables|GettmpHarvestGoods))
      (CallFunction|DropSprinkles (LocalVariables|GettmpBonusGoods)))
    (:then_2
      (if _valid_
        (Default|AddGoodsInventoryBatch _inventory (LocalVariables|GettmpHarvestGoods))
        (Default|AddGoodsInventoryBatch _inventory (LocalVariables|GettmpBonusGoods))
        (Variables|Default|SetCurrentGrowth 0.0)
        (CallFunction|SetGrowState "NewEnumerator5")
        (bind _asff_game_state (Utilities|Casting|CastToFF_GameState (Game|GetGameState)))
        (Default|TrackGoodsHarvestedTotalsBatch _asff_game_state (LocalVariables|GettmpHarvestGoods))
        (Default|TrackGoodsHarvestedTotalsBatch _asff_game_state (LocalVariables|GettmpBonusGoods))
        (bind _asffplayer_state (Utilities|Casting|CastToFFPlayerState (Variables|/Script/Engine.Controller|GetPlayerState (Game|GetPlayerController 0))))
        (Class|FFPlayerState|AddExperience _asffplayer_state (CallFunction|GetHarvestExperience))))
    (:then_3
      (Utilities|IsValid _myplot
        (:Is%20Valid
          (Default|OnCropHarvested _myplot))))))

(fn UpdateGrowthGUI
  (bind _cropsprite (Variables|Default|GetCropSprite))
  (if (Utilities|Enum|Equal(Enum) (Variables|Default|GetGrowState) "NewEnumerator5")
    (Sprite|SetSpriteColor _cropsprite "(R=1.000000,G=0.244792,B=0.244792,A=1.000000)")
    (else
      (Sprite|SetSpriteColor _cropsprite "(R=1.000000,G=1.000000,B=1.000000,A=1.000000)"))))

(fn DropSprinkles
  (params (SprinkleGoods :type Array%20of%20Goods%20Quantity%20Structures))
  (bind _sprinklevolume (Variables|Default|GetSprinkleVolume))
  (bind _boxextent (Collision|GetComponentBounds _sprinklevolume))
  (bind (_x _y _z) (Math|Vector|BreakVector _boxextent))
  (for _array_element SprinkleGoods
    (bind _asff_game_state (Utilities|Casting|CastToFF_GameState (Game|GetGameState)))
    (if (.Found? (Default|GetGoodsData _asff_game_state (.Name (Utilities|Struct|BreakGoodsQuantity _array_element))))
      (bind _returnvalue (Rendering|Material|CreateDynamicMaterialInstance "/Game/FungusFarm/Assets/Materials/SprinkleParticle.SprinkleParticle" "None" :!class /Script/Engine.KismetMaterialLibrary))
      (bind _output_get (LocalVariables|SetTmpMaterial _returnvalue))
      (Rendering|Material|SetTextureParameterValue _output_get "SprinkleTexture" (Utilities|ResolveSoftReference (.Thumbnail (Utilities|Struct|BreakGoodsType (.GoodsData (Default|GetGoodsData _asff_game_state (.Name (Utilities|Struct|BreakGoodsQuantity _array_element))))))))
      (bind _returnvalue_2 (Effects|SpawnEmitteratLocation (select (Utilities|String|Contains (Utilities|String|ToString(Name) (.Name (Utilities|Struct|BreakGoodsQuantity _array_element))) "Spirit" true) "/Game/FungusFarm/Assets/Particles/SpiritFloat.SpiritFloat" "/Game/FungusFarm/Assets/Particles/SporesBasic.SporesBasic") (Transformation|GetWorldLocation (Variables|Default|GetSprinkleVolume))))
      (bind _output_get_2 (LocalVariables|SettmpEmitter _returnvalue_2))
      (Rendering|Material|SetMaterial _returnvalue_2 0 (LocalVariables|GetTmpMaterial))
      (Components|Activation|Deactivate _output_get_2)
      (Effects|Components|ParticleSystem|SetFloatParameter (LocalVariables|GettmpEmitter) "Count" (Math|Float|Clamp(Float) (select (> (.Quantity (Utilities|Struct|BreakGoodsQuantity _array_element)) 2e+01) (/ (.Quantity (Utilities|Struct|BreakGoodsQuantity _array_element)) 1e+01) (.Quantity (Utilities|Struct|BreakGoodsQuantity _array_element))) 0.0 1e+02))
      (Effects|Components|ParticleSystem|SetFloatParameter (LocalVariables|GettmpEmitter) "SpawnWidth" (* _x 1.8))
      (Effects|Components|ParticleSystem|SetFloatParameter (LocalVariables|GettmpEmitter) "SpawnHeight" _z)
      (Components|Activation|Activate (LocalVariables|GettmpEmitter) false))))

(fn HandleClick
  (if (not (Game|IsGamePaused))
    (Utilities|IsValid (Variables|Default|GetMyPlot)
      (:Is%20Valid
        (switch Utilities|FlowControl|Switch|SwitchonCropGrowState (Variables|Default|GetGrowState)
          (:NewEnumerator5
            (bind _asff_game_state (Utilities|Casting|CastToFF_GameState (Game|GetGameState)))
            (bind _currentfarmmanager (Default|GetFarmManager _asff_game_state))
            (Default|ReplantPlot _currentfarmmanager (Variables|Default|GetMyPlot)))
          (:NewEnumerator0
            (bind _output_get (LocalVariables|SettmpSprinkles (CallFunction|CalculateSprinkleAmount)))
            (if (> (Utilities|Array|Length _output_get) 0)
              (Audio|PlaySoundatLocation (Utilities|Select :Index (Math|Random|RandomIntegerinRange 0 1) :Option%200 "/Game/FungusFarm/Assets/Sound/Effects/PopShort_01.PopShort_01" :Option%201 "/Game/FungusFarm/Assets/Sound/Effects/PopShort_02.PopShort_02") (Transformation|GetWorldLocation (Variables|Default|GetSprinkleBox)) "0, 0, 0" 1.0 1.0 0.0 0 0 self)
              (CallFunction|DropSprinkles (LocalVariables|GettmpSprinkles))
              (Default|AddGoodsInventoryBatch (.Inventory (CallFunction|GetPlayerInventory)) (LocalVariables|GettmpSprinkles))))
          (:NewEnumerator4
            (CallFunction|Harvest)))))))

(fn InputsTick
  (params (DeltaTime :type Float%20%28single-precision%29))
  (bind (_valid_ _inventory) (CallFunction|GetPlayerInventory))
  (bind _crop_data (Variables|Default|GetCrop%20Data))
  (bind _growthinputrequirements (Utilities|Struct|BreakCropType _crop_data))
  (Utilities|IsValid (Variables|Default|GetMyPlot)
    (:Is%20Valid
      (if (> DeltaTime 0.0)
        (switch Utilities|FlowControl|Switch|SwitchonCropGrowState (Variables|Default|GetGrowState)
          (:NewEnumerator5
            (return))
          (:NewEnumerator1
            (return))
          (:NewEnumerator0
            _)
          (:NewEnumerator3
            _)
          (:NewEnumerator2
            _)
          (:NewEnumerator4
            (return)))
        (if (> (Utilities|Array|Length _growthinputrequirements) 0)
          (if _valid_
            (bind (_successful _inventorybusy) (Default|RemoveGoodsInventoryBatch _inventory (CallFunction|InputRequirementsPerTime _growthinputrequirements DeltaTime)))
            (if _successful
              (CallFunction|SetGrowState "NewEnumerator0" :!label _label)
              (elif _inventorybusy
                (CallFunction|SetGrowState "NewEnumerator3")
                (else
                  (CallFunction|SetGrowState "NewEnumerator2"))))
            (return))
          (else
            (goto _label)))
        (else
          (return))))
    (:Is%20Not%20Valid
      (return))))

(fn InputRequirementsPerTime
  (params (TotalHarvestRequirements :type Array%20of%20Goods%20Quantity%20Structures) (DeltaTime :type Float%20%28single-precision%29))
  (if (and (!= DeltaTime 0.0) (!= (Utilities|GetCropGrowthRate) 0.0))
    (for _array_element TotalHarvestRequirements
      (Utilities|Array|Add (LocalVariables|GettmpRequirements) (Utilities|Struct|MakeGoodsQuantity (.Name (Utilities|Struct|BreakGoodsQuantity _array_element)) (* DeltaTime (/ (.Quantity (Utilities|Struct|BreakGoodsQuantity _array_element)) (/ (.GrowthTime (Utilities|Struct|BreakCropType (Variables|Default|GetCrop%20Data))) (Utilities|GetCropGrowthRate)))))))
    (return (LocalVariables|GettmpRequirements))))

(fn SetGrowState
  (params (NewState :type CropGrowState%20Enum :default "NewEnumerator5"))
  (Utilities|FlowControl|Sequence
    (:then_0
      (if (Utilities|Enum|NotEqual(Enum) NewState (Variables|Default|GetGrowState))
        (LocalVariables|SettmpOldGrowState (Variables|Default|GetGrowState))
        (Variables|Default|SetGrowState NewState)
        (switch Utilities|FlowControl|Switch|SwitchonCropGrowState NewState
          (:NewEnumerator5
            (CallFunction|OnUnplanted (LocalVariables|GettmpOldGrowState)))
          (:NewEnumerator1
            (CallFunction|OnWarmupStart (LocalVariables|GettmpOldGrowState)))
          (:NewEnumerator0
            (CallFunction|OnGrowthStart (LocalVariables|GettmpOldGrowState)))
          (:NewEnumerator3
            (CallFunction|OnInputInventoryBusy (LocalVariables|GettmpOldGrowState)))
          (:NewEnumerator2
            (CallFunction|OnStarveStart (LocalVariables|GettmpOldGrowState)))
          (:NewEnumerator4
            (CallFunction|OnGrowthComplete (LocalVariables|GettmpOldGrowState))))))
    (:then_1
      (CallFunction|UpdateGrowthGUI)
      (Utilities|IsValid (Variables|Default|GetMyPlot)
        (:Is%20Valid
          (Default|UpdatePlotGUI (Variables|Default|GetMyPlot)))))))

(fn GrowWarmupTick
  (params (DeltaTime :type Float%20%28single-precision%29))
  (LocalVariables|SettmpRemainingTime DeltaTime)
  (Utilities|FlowControl|Sequence
    (:then_0
      (if (<= (Variables|Default|GetMaxGrowthWarmup) 0.0)
        (CallFunction|SetGrowState "NewEnumerator0")
        (elif (<= (Variables|Default|GetGrowthWarmupRate) 0.0)
          (LocalVariables|SettmpRemainingTime 0.0)
          (elif (>= (+ (Variables|Default|GetCurrentGrowthWarmup) (* DeltaTime (Variables|Default|GetGrowthWarmupRate))) (Variables|Default|GetMaxGrowthWarmup))
            (LocalVariables|SettmpRemainingTime (- (LocalVariables|GettmpRemainingTime) (/ (- (Variables|Default|GetMaxGrowthWarmup) (Variables|Default|GetCurrentGrowthWarmup)) (Variables|Default|GetGrowthWarmupRate))))
            (Variables|Default|SetCurrentGrowthWarmup 0.0)
            (CallFunction|SetGrowState "NewEnumerator0")
            (else
              (LocalVariables|SettmpRemainingTime 0.0)
              (Variables|Default|SetCurrentGrowthWarmup (+ (Variables|Default|GetCurrentGrowthWarmup) (* DeltaTime (Variables|Default|GetGrowthWarmupRate)))))))))
    (:then_1
      (return (LocalVariables|GettmpRemainingTime)))))

(fn CalculatedProductionRates
  (bind _growthrate (Utilities|GetCropGrowthRate))
  (if (Utilities|Enum|Equal(Enum) (Variables|Default|GetGrowState) "NewEnumerator0")
    (if (> (Utilities|GetCropGrowthRate) 0.0)
      (for _array_element (.Harvest%20Goods (CallFunction|CalculateHarvestAmount))
        (Utilities|Map|Add (LocalVariables|GetTmpRates) (.Name (Utilities|Struct|BreakGoodsQuantity _array_element)) (Utilities|Struct|MakeGoodsQuantity (.Name (Utilities|Struct|BreakGoodsQuantity _array_element)) (select (> _growthrate 0.0) (/ (.Quantity (Utilities|Struct|BreakGoodsQuantity _array_element)) (/ (.GrowthTime (Utilities|Struct|BreakCropType (Variables|Default|GetCrop%20Data))) _growthrate)) 0.0))))
      (return (LocalVariables|GetTmpRates))
      (else
        _)))
  (return (Utilities|Map|MakeMap)))

(fn DropSpirits
  (params (Spirits :type Array%20of%20Goods%20Quantity%20Structures))
  (for _array_element Spirits
    (if (Utilities|String|Contains (Utilities|String|ToString(Name) (.Name (Utilities|Struct|BreakGoodsQuantity _array_element))) " Spirit" true)
      (bind _returnvalue (Effects|SpawnEmitteratLocation "/Game/FungusFarm/Assets/Particles/SpiritFloat.SpiritFloat" (Transformation|GetWorldLocation (Variables|Default|GetSprinkleVolume))))
      (Effects|Components|ParticleSystem|SetFloatParameter _returnvalue "Count" (Math|Float|Clamp(Float) (.Quantity (Utilities|Struct|BreakGoodsQuantity _array_element)) 0.0 1e+02)))))

(fn CalculateSprinkleAmount
  (return (CallFunction|MultiplyInventory (Class|GoodsFunctionLibrary|EvaluateGoodsDrops (.SprinkleGoods (Utilities|Struct|BreakCropType (Variables|Default|GetCrop%20Data))) -1.0) (Variables|Default|GetSprinkleFactor) true)))

(fn GetGrowState
  (return (Variables|Default|GetGrowState)))

(fn UpdateCalculatedAttributes)

(fn GrowthTick
  (params (Delta%20Time :type Float%20%28single-precision%29))
  (bind _crop_data (Variables|Default|GetCrop%20Data))
  (bind _growthtime (Utilities|Struct|BreakCropType _crop_data))
  (bind _output_get (LocalVariables|SettmpStartingDeltaTime Delta%20Time))
  (LocalVariables|SettmpRemainingTime _output_get)
  (Utilities|IsValid (Variables|Default|GetMyPlot)
    (:Is%20Valid
      (Utilities|FlowControl|Sequence
        (:then_0
          (if (> (LocalVariables|GettmpRemainingTime) 0.0) :!label _label
            (switch Utilities|FlowControl|Switch|SwitchonCropGrowState (Variables|Default|GetGrowState)
              (:NewEnumerator1
                (bind _remaining_time (CallFunction|GrowWarmupTick (LocalVariables|GettmpRemainingTime)))
                (LocalVariables|SettmpRemainingTime _remaining_time)
                (goto _label))
              (:NewEnumerator0
                _)
              (:NewEnumerator3
                _)
              (:NewEnumerator2
                _))
            (bind _output_get_2 (LocalVariables|SettmpGrowthRate (Utilities|GetCropGrowthRate)))
            (if (> _output_get_2 0.0)
              (Utilities|FlowControl|Sequence
                (:then_0
                  (bind _returnvalue (Utilities|TimeRequiredtoGrowthComplete)
                    (:out
                      (bind _output_get_3 (LocalVariables|SettmpUsedTime (Math|Float|Clamp(Float) _returnvalue 0.0 (LocalVariables|GettmpRemainingTime))))
                      (CallFunction|InputsTick _output_get_3))))
                (:then_1
                  (if (Utilities|Enum|Equal(Enum) (Variables|Default|GetGrowState) "NewEnumerator0")
                    (if (>= (+ (* (LocalVariables|GettmpRemainingTime) (LocalVariables|GettmpGrowthRate)) (Variables|Default|GetCurrentGrowth)) _growthtime)
                      (Variables|Default|SetCurrentGrowth _growthtime)
                      (LocalVariables|SettmpRemainingTime (- (LocalVariables|GettmpRemainingTime) (LocalVariables|GettmpUsedTime)))
                      (CallFunction|SetGrowState "NewEnumerator4")
                      (else
                        (Variables|Default|SetCurrentGrowth (+ (* (LocalVariables|GettmpRemainingTime) (LocalVariables|GettmpGrowthRate)) (Variables|Default|GetCurrentGrowth)))
                        (LocalVariables|SettmpRemainingTime 0.0)
                        (CallFunction|UpdateGrowthGUI)
                        (Default|UpdatePlotGUI (Variables|Default|GetMyPlot)))))))
              (else
                (LocalVariables|SettmpRemainingTime 0.0)))))
        (:then_1
          (return (LocalVariables|GettmpRemainingTime)))))))

(fn CalculateHarvestAmount
  (bind _crop_data (Variables|Default|GetCrop%20Data))
  (bind (_name _displayname _thumbnail _thumbnailhardref _actorclass _plantingcost _harvestgoods _harvestgoodsbonus) (Utilities|Struct|BreakCropType _crop_data))
  (return (Class|GoodsFunctionLibrary|EvaluateGoodsDrops _harvestgoods -1.0) (Class|GoodsFunctionLibrary|EvaluateGoodsDrops _harvestgoodsbonus -1.0)))

(fn GetHarvestExperience
  (return (.HarvestExperience (Utilities|Struct|BreakCropType (Variables|Default|GetCrop%20Data)))))