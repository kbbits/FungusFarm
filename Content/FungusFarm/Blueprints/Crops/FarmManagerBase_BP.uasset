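; Farm manager for FungusFarm that tracks every crop plot in the level and drives crop growth, harvesting and replanting.
; A looping timer runs GrowTick, carrying leftover time through each crop's growth states and handling per-plot auto-harvest and auto-replant.
; Planting and replanting pay costs from the FF_GameState goods inventory.
; On game load it re-initializes equipment and plot references; it also sums production rates and supports pausing.
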(event Custom|DestroyCrop
  (params (Crop :type Crop%20Base%20BP%20Object%20Reference))
  (Actor|DestroyActor Crop))

(event Custom|ReplantPlot
  (params (Plot :type Crop%20Plot%20Base%20BP%20Object%20Reference))
  (CallFunction|DoReplantPlotifUnplanted Plot))

(event Custom|OnGameLoaded
  (params (SlotInfo :type Slot%20Info%20Object%20Reference))
  (Utilities|FlowControl|Sequence
    (:then_0
      ;[1 1 1] Init all Equipment
      (bind _outactors (Actor|GetAllActorsOfClass "/Game/FungusFarm/Blueprints/Equipment/Equipment_Base.Equipment_Base_C"))
      (for _array_element _outactors
        (Default|InitfromData _array_element)))
    (:then_1
      ;[1 1 1 1 16] Refresh Plot references and each Crop Plot's references. Plots will refresh their own equipped mods
      (CallFunction|RefreshPlotReferences)
      (for _array_element_2 (Variables|Default|GetPlots)
        (Default|RefreshReferences _array_element_2)))))

(event EventBeginPlay
  (Utilities|FlowControl|Sequence
    (:then_0
      (EventDispatchers|BindEventtoOnGameLoaded (Class|SaveManager|GetSaveManager) (delegate Custom|OnGameLoaded)))
    (:then_1
      (CallFunction|RefreshPlotReferences))
    (:then_2
      ;[1 1 1] Setup grow timer
      (bind _returnvalue (Utilities|Time|SetTimerbyFunctionName 0 "GrowTick" 0.2 true))
      (Variables|Default|SetGrowTimer _returnvalue))))

(event EventEndPlay
  (params (EndPlayReason :type EEndPlayReason%20Enum :default "Destroyed"))
  (Utilities|Time|ClearandInvalidateTimerbyHandle (Variables|Default|GetGrowTimer)))

(fn ConstructionScript)

(fn GrowTick
  (LocalVariables|SettmpDeltaTime (Class|KismetSystemLibrary|GetTimerElapsedTimeHandle (Variables|Default|GetGrowTimer)))
  (for _array_element (Variables|Default|GetPlots)
    (LocalVariables|SettmpCropRemainingTime (LocalVariables|GettmpDeltaTime))
    (Utilities|FlowControl|Sequence :!label _label
      (:then_0
        (Utilities|IsValid (Variables|/Game/FungusFarm/Blueprints/Equipment/CropPlots/CropPlotBase_BP.CropPlotBase_BP_C|GetMyCrop _array_element)
          (:Is%20Valid
            (bind _remaining_time (Default|GrowthTick (Variables|/Game/FungusFarm/Blueprints/Equipment/CropPlots/CropPlotBase_BP.CropPlotBase_BP_C|GetMyCrop _array_element) (LocalVariables|GettmpCropRemainingTime)))
            (LocalVariables|SettmpCropRemainingTime _remaining_time))))
      (:then_1
        (Utilities|IsValid (Variables|/Game/FungusFarm/Blueprints/Equipment/CropPlots/CropPlotBase_BP.CropPlotBase_BP_C|GetMyCrop _array_element)
          (:Is%20Valid
            (if (Utilities|Enum|Equal(Enum) (Default|GetGrowState (Variables|/Game/FungusFarm/Blueprints/Equipment/CropPlots/CropPlotBase_BP.CropPlotBase_BP_C|GetMyCrop _array_element)) "NewEnumerator4")
              (if (Variables|/Game/FungusFarm/Blueprints/Equipment/CropPlots/CropPlotBase_BP.CropPlotBase_BP_C|GetAutoHarvest _array_element)
                (Default|Harvest (Variables|/Game/FungusFarm/Blueprints/Equipment/CropPlots/CropPlotBase_BP.CropPlotBase_BP_C|GetMyCrop _array_element)))))))
      (:then_2
        (if (Variables|/Game/FungusFarm/Blueprints/Equipment/CropPlots/CropPlotBase_BP.CropPlotBase_BP_C|GetAutoReplant _array_element)
          (CallFunction|DoReplantPlotifUnplanted _array_element)))
      (:then_3
        (Utilities|IsValid (Variables|/Game/FungusFarm/Blueprints/Equipment/CropPlots/CropPlotBase_BP.CropPlotBase_BP_C|GetMyCrop _array_element)
          (:Is%20Valid
            (switch Utilities|FlowControl|Switch|SwitchonCropGrowState (Default|GetGrowState (Variables|/Game/FungusFarm/Blueprints/Equipment/CropPlots/CropPlotBase_BP.CropPlotBase_BP_C|GetMyCrop _array_element))
              (:NewEnumerator1
                _)
              (:NewEnumerator0
                _))
            (if (> (LocalVariables|GettmpCropRemainingTime) 0.0)
              (goto _label))))))))

(fn PlantCropinPlot
  (params (Crop%20Data :type Crop%20Type%20Structure) (Plot :type Crop%20Plot%20Base%20BP%20Object%20Reference))
  (Utilities|FlowControl|Sequence
    (:then_0
      (bind _asff_game_state (Utilities|Casting|CastToFF_GameState (Game|GetGameState)))
      (bind _successful (Default|RemoveGoodsInventoryBatch _asff_game_state (.PlantingCost (Utilities|Struct|BreakCropType Crop%20Data))))
      (LocalVariables|SetpaidPlanted? _successful))
    (:then_1
      (Utilities|IsValid (Variables|/Game/FungusFarm/Blueprints/Equipment/CropPlots/CropPlotBase_BP.CropPlotBase_BP_C|GetMyCrop Plot)
        (:Is%20Valid
          (CallFunction|RemoveCropfromPlot Plot))))
    (:then_2
      (Default|SetCrop Plot (LocalVariables|GetpaidPlanted?) Crop%20Data))))

(fn RemoveCropfromPlot
  (params (Plot :type Crop%20Plot%20Base%20BP%20Object%20Reference))
  (Utilities|IsValid (Variables|/Game/FungusFarm/Blueprints/Equipment/CropPlots/CropPlotBase_BP.CropPlotBase_BP_C|GetMyCrop Plot)
    (:Is%20Valid
      (CallFunction|DestroyCrop (Variables|/Game/FungusFarm/Blueprints/Equipment/CropPlots/CropPlotBase_BP.CropPlotBase_BP_C|GetMyCrop Plot))
      (Variables|/Game/FungusFarm/Blueprints/Equipment/CropPlots/CropPlotBase_BP.CropPlotBase_BP_C|SetMyCrop Plot 0)
      (Variables|/Game/FungusFarm/Blueprints/Equipment/CropPlots/CropPlotBase_BP.CropPlotBase_BP_C|SetSelectedCropData Plot ""))))

(fn CalculatedProductionRates
  (for _array_element (Variables|Default|GetPlots)
    (Utilities|IsValid (Variables|/Game/FungusFarm/Blueprints/Equipment/CropPlots/CropPlotBase_BP.CropPlotBase_BP_C|GetMyCrop _array_element)
      (:Is%20Valid
        (bind _rates (Default|CalculatedProductionRates (Variables|/Game/FungusFarm/Blueprints/Equipment/CropPlots/CropPlotBase_BP.CropPlotBase_BP_C|GetMyCrop _array_element)))
        (bind _total_inventory (CallFunction|SumInventories (LocalVariables|GettmpRates) _rates))
        (LocalVariables|SettmpRates _total_inventory))))
  (return (LocalVariables|GettmpRates)))

(fn Pause
  (Utilities|Time|PauseTimerbyHandle (Variables|Default|GetGrowTimer)))

(fn Unpause
  (if (Class|KismetSystemLibrary|IsTimerPausedHandle (Variables|Default|GetGrowTimer))
    (Utilities|Time|UnpauseTimerbyHandle (Variables|Default|GetGrowTimer))))

(fn AddPlot
  (params (Plot :type Crop%20Plot%20Base%20BP%20Object%20Reference))
  (Utilities|Array|AddUnique (Variables|Default|GetPlots) Plot))

(fn DoReplantPlotifUnplanted
  (params (Plot :type Crop%20Plot%20Base%20BP%20Object%20Reference))
  (bind _mycrop (Variables|/Game/FungusFarm/Blueprints/Equipment/CropPlots/CropPlotBase_BP.CropPlotBase_BP_C|GetMyCrop Plot))
  (bind _selectedcropdata (Variables|/Game/FungusFarm/Blueprints/Equipment/CropPlots/CropPlotBase_BP.CropPlotBase_BP_C|GetSelectedCropData Plot))
  (bind _mycrop_2 (Variables|/Game/FungusFarm/Blueprints/Equipment/CropPlots/CropPlotBase_BP.CropPlotBase_BP_C|GetMyCrop Plot))
  (bind (_name _displayname _thumbnail _thumbnailhardref _actorclass _plantingcost) (Utilities|Struct|BreakCropType _selectedcropdata))
  (if (Utilities|Name|NotEqual(Name) _name "None")
    (Utilities|IsValid _mycrop_2
      (:Is%20Valid
        (if (Utilities|Enum|Equal(Enum) (Default|GetGrowState _mycrop_2) "NewEnumerator5")
          (bind _asff_game_state (Utilities|Casting|CastToFF_GameState (Game|GetGameState) :!label _label))
          (bind _successful (Default|RemoveGoodsInventoryBatch _asff_game_state _plantingcost))
          (Utilities|IsValid _mycrop
            (:Is%20Valid
              (if _successful
                (Default|SetGrowState _mycrop "NewEnumerator1")))
            (:Is%20Not%20Valid
              (Default|SetCrop Plot _successful (Variables|/Game/FungusFarm/Blueprints/Equipment/CropPlots/CropPlotBase_BP.CropPlotBase_BP_C|GetSelectedCropData Plot))))))
      (:Is%20Not%20Valid
        (goto _label)))))

(fn RefreshPlotReferences
  ;[1 1 1] Find all plots
  (Variables|Default|SetPlots (Utilities|Array|MakeArray))
  (bind _outactors (Actor|GetAllActorsOfClass "/Game/FungusFarm/Blueprints/Equipment/CropPlots/CropPlotBase_BP.CropPlotBase_BP_C"))
  (for _array_element _outactors
    (CallFunction|AddPlot _array_element)))

(fn RemovePlot
  (params (Plot :type Crop%20Plot%20Base%20BP%20Object%20Reference))
  (Utilities|Array|RemoveItem (Variables|Default|GetPlots) Plot))

(fn FillTestVar
  (bind _asff_game_state (Utilities|Casting|CastToFF_GameState (Game|GetGameState)))
  (bind _unlocked_crops (Default|GetAllUnlockedCropData _asff_game_state))
  (bind _output_get (LocalVariables|SettmpColor (Utilities|Struct|MakeLinearColor (Math|Random|RandomFloat) (Math|Random|RandomFloat) (Math|Random|RandomFloat) 1.0)))
  (Development|PrintString (Utilities|String|Append "Added: " (Utilities|String|ToString(Name) (.Name (Utilities|Struct|BreakCropType (Utilities|Array|Get(acopy) _unlocked_crops))))) true true _output_get)
  (Utilities|Array|Add (Variables|Default|GetTestStructVar) (LocalVariables|GettmpColor))
  (Utilities|Array|Add (Variables|Default|GetCrafting%20Slots%20Test%20Var) (Utilities|Struct|MakeCraftingSlot (.Name (Utilities|Struct|BreakCropType (Utilities|Array|Get(acopy) _unlocked_crops))) (Math|Float|Truncate (.GrowthTime (Utilities|Struct|BreakCropType (Utilities|Array|Get(acopy) _unlocked_crops)))))))

(fn InspectTestVar
  (bind _tmpdebugstrings (LocalVariables|GettmpDebugStrings))
  (Utilities|FlowControl|Sequence
    (:then_0
      (Development|PrintString "Items in CraftingSlot TestVar" true true "(R=0.000000,G=0.660000,B=1.000000,A=1.000000)" 5.0)
      (for (_array_element _array_index) (Variables|Default|GetCrafting%20Slots%20Test%20Var)
        (Utilities|Array|Clear (LocalVariables|GettmpDebugStrings))
        (Utilities|Array|Add _tmpdebugstrings (Utilities|String|ToString(Name) (.Name (Utilities|Struct|BreakCraftingSlot _array_element))))
        (Utilities|Array|Add _tmpdebugstrings (Utilities|String|Append ": " (Utilities|String|ToString(Integer) (.Value (Utilities|Struct|BreakCraftingSlot _array_element)))))
        (Development|PrintString (Utilities|String|JoinStringArray (LocalVariables|GettmpDebugStrings) " 
") true true (Utilities|Array|Get(acopy) (Variables|Default|GetTestStructVar) _array_index) 5.0)))))