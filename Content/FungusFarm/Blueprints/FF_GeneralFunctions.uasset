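; General function set for FungusFarm that does math on goods inventories held as item arrays or type-keyed maps.
; It sums two inventories, merges arrays by type, and scales quantities with optional truncation, keeping only positive results.
; Array sums collapse duplicates through a summed map, then convert back to an array.
; Drop evaluation sums randomly selected goods; partial chances pass when the roll is at or above PercentChance, so higher values drop less often.
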(fn SumInventories
  (params (InventoryA :type Map%20of%20GoodsTypes%20Enums%20to%20Structs :default "NewEnumerator0") (InventoryB :type Map%20of%20GoodsTypes%20Enums%20to%20Structs :default "NewEnumerator0"))
  (Utilities|FlowControl|Sequence
    (:then_0
      (bind _keys (Utilities|Map|Keys InventoryA))
      (bind _output_get (LocalVariables|SettmpAllKeys _keys))
      (bind _keys_2 (Utilities|Map|Keys InventoryB))
      (Utilities|Array|AppendArray _output_get _keys_2)
      (for _array_element (LocalVariables|GettmpAllKeys)
        (Utilities|Array|AddUnique (LocalVariables|GettmpUniqueKeys) _array_element)))
    (:then_1
      (for _array_element_2 (LocalVariables|GettmpUniqueKeys)
        (Utilities|Map|Add (LocalVariables|GettmpInventory) _array_element_2 (Utilities|Struct|MakeGoodsInventoryItem_Struct _array_element_2 (+ (.Quantity (Utilities|Struct|BreakGoodsInventoryItem_Struct (.Value (Utilities|Map|Find InventoryA _array_element_2)))) (.Quantity (Utilities|Struct|BreakGoodsInventoryItem_Struct (.Value (Utilities|Map|Find InventoryB _array_element_2))))))))
      (return (LocalVariables|GettmpInventory)))))

(fn MultiplyInventory
  (params (Goods :type Array%20of%20Goods%20Inventory%20Item%20Struct%20Structures) (Multiplier :type Float%20%28single-precision%29) (TruncateAmounts :type Boolean))
  (for _array_element Goods
    (if (> (select TruncateAmounts (Math|Conversions|ToFloat(Integer) (Math|Float|Truncate (* (.Quantity (Utilities|Struct|BreakGoodsInventoryItem_Struct _array_element)) Multiplier))) (* (.Quantity (Utilities|Struct|BreakGoodsInventoryItem_Struct _array_element)) Multiplier)) 0.0)
      (Utilities|Array|Add (LocalVariables|GetTmpTotalInventory) (Utilities|Struct|MakeGoodsInventoryItem_Struct (.Type (Utilities|Struct|BreakGoodsInventoryItem_Struct _array_element)) (select TruncateAmounts (Math|Conversions|ToFloat(Integer) (Math|Float|Truncate (* (.Quantity (Utilities|Struct|BreakGoodsInventoryItem_Struct _array_element)) Multiplier))) (* (.Quantity (Utilities|Struct|BreakGoodsInventoryItem_Struct _array_element)) Multiplier))))))
  (return (LocalVariables|GetTmpTotalInventory)))

(fn EvaluateGoodsDrop
  (params (Drops :type Array%20of%20Goods%20Drop%20Chance%20Struct%20Structures))
  (Utilities|FlowControl|Sequence
    (:then_0
      ;[1 1 1] Fill tmp Array with drops
      (LocalVariables|SettmpTotalDroppedGoods (Utilities|Array|MakeArray))
      (for _array_element Drops
        (if (and (> (.percent_chance (Utilities|Struct|BreakGoodsDropChance_Struct _array_element)) 0.0) (or (>= (.percent_chance (Utilities|Struct|BreakGoodsDropChance_Struct _array_element)) 1.0) (>= (Math|Random|RandomFloatinRange 0.0 1.0) (.percent_chance (Utilities|Struct|BreakGoodsDropChance_Struct _array_element)))))
          (Utilities|Array|AppendArray (LocalVariables|GettmpTotalDroppedGoods) (.goods (Utilities|Struct|BreakGoodsDropChance_Struct _array_element))))))
    (:then_1
      (bind _summed_goods (CallFunction|SumGoodsArray (LocalVariables|GettmpTotalDroppedGoods)))
      (return _summed_goods))))

(fn SumGoodsArrays
  (params (Goods%20A :type Array%20of%20Goods%20Inventory%20Item%20Struct%20Structures) (Goods%20B :type Array%20of%20Goods%20Inventory%20Item%20Struct%20Structures))
  (Utilities|FlowControl|Sequence
    (:then_0
      (Utilities|Array|Clear (LocalVariables|GettmpTotalGoods)))
    (:then_1
      (Utilities|Array|AppendArray (LocalVariables|GettmpTotalGoods) Goods%20A)
      (Utilities|Array|AppendArray (LocalVariables|GettmpTotalGoods) Goods%20B))
    (:then_2
      (bind _goods_map (CallFunction|GoodsArraytoSummedMap (LocalVariables|GettmpTotalGoods)))
      (bind _goods_array (CallFunction|GoodsMaptoArray _goods_map))
      (return _goods_array))))

(fn GoodsArraytoSummedMap
  (params (Goods :type Array%20of%20Goods%20Inventory%20Item%20Struct%20Structures))
  (Utilities|FlowControl|Sequence
    (:then_0
      (LocalVariables|SettmpGoodsMap (Utilities|Map|MakeMap)))
    (:then_1
      (for _array_element Goods
        (Utilities|Map|Add (LocalVariables|GettmpGoodsMap) (.Type (Utilities|Struct|BreakGoodsInventoryItem_Struct _array_element)) (Utilities|Struct|MakeGoodsInventoryItem_Struct (.Type (Utilities|Struct|BreakGoodsInventoryItem_Struct _array_element)) (+ (select (.ReturnValue (Utilities|Map|Find (LocalVariables|GettmpGoodsMap) (.Type (Utilities|Struct|BreakGoodsInventoryItem_Struct _array_element)))) (.Quantity (Utilities|Struct|BreakGoodsInventoryItem_Struct (.Value (Utilities|Map|Find (LocalVariables|GettmpGoodsMap) (.Type (Utilities|Struct|BreakGoodsInventoryItem_Struct _array_element)))))) 0.0) (.Quantity (Utilities|Struct|BreakGoodsInventoryItem_Struct _array_element)))))))
    (:then_2
      (return (LocalVariables|GettmpGoodsMap)))))

(fn GoodsMaptoArray
  (params (Goods%20Map :type Map%20of%20GoodsTypes%20Enums%20to%20Structs :default "NewEnumerator0"))
  (Utilities|FlowControl|Sequence
    (:then_0
      (LocalVariables|SettmpGoodsArray (Utilities|Array|MakeArray)))
    (:then_1
      (bind _keys (Utilities|Map|Keys Goods%20Map))
      (for _array_element _keys
        (Utilities|Array|Add (LocalVariables|GettmpGoodsArray) (.Value (Utilities|Map|Find Goods%20Map _array_element)))))
    (:then_2
      (return (LocalVariables|GettmpGoodsArray)))))

(fn SumGoodsArray
  (params (Goods%20to%20Sum :type Array%20of%20Goods%20Inventory%20Item%20Struct%20Structures))
  (bind _goods_map (CallFunction|GoodsArraytoSummedMap Goods%20to%20Sum))
  (bind _goods_array (CallFunction|GoodsMaptoArray _goods_map))
  (return _goods_array))